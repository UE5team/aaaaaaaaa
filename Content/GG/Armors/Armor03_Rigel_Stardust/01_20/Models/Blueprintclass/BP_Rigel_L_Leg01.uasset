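; Left leg armor part Blueprint for Rigel Stardust that manages the leg's Niagara thruster and brake effects.
; The construction script attaches two leg effects to skeletal mesh sockets.
; Boost overrides call the parent, then stretch those effects along Z or restore that scale to normal.
; Setting brake adds two new Niagara components on brake sockets, while resetting only detaches them without destroying them.
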(fn `Reset Boost Effect`
  (`parent.Reset Boost Effect`)
  (`self.Reset Boust Efect Scale` (`self.L_Leg_Effect02`))
  (`self.Reset Boust Efect Scale` (`self.L_Leg_Effect01`)))

(fn `Reset Boust Efect Scale`
  (params (`ターゲット` :type "SceneComponent Object Reference"))
  (bind (_relativescale3d_x _relativescale3d_y) (`KismetMathLibrary.BreakVector` (`SceneComponent.RelativeScale3D` `ターゲット`)))
  (`SceneComponent.SetRelativeScale3D` `ターゲット` (`KismetMathLibrary.MakeVector` _relativescale3d_x _relativescale3d_y 1.0)))

(fn `Reset Brake Effect`
  (bind _l_brake_effect01 (`self.L_Brake_Effect01`))
  (bind _l_brake_effect02 (`self.L_Brake_Effect02`))
  (`|ExecutionSequence`
    (:`then_0`
      (`/Engine/EditorBlueprintResources/StandardMacros.IsValid` _l_brake_effect01
        (:`Is Valid`
          (`SceneComponent.K2_DetachFromComponent` _l_brake_effect01 "KeepRelative" "KeepRelative" "KeepRelative" true))))
    (:`then_1`
      (`/Engine/EditorBlueprintResources/StandardMacros.IsValid` _l_brake_effect02
        (:`Is Valid`
          (`SceneComponent.K2_DetachFromComponent` _l_brake_effect02 "KeepRelative" "KeepRelative" "KeepRelative" true))))))

(fn `Set Boost Effect`
  (`parent.Set Boost Effect`)
  (`self.Set Boust Efect Scale` (`self.L_Leg_Effect02`))
  (`self.Set Boust Efect Scale` (`self.L_Leg_Effect01`)))

(fn `Set Boust Efect Scale`
  (params (`ターゲット` :type "SceneComponent Object Reference"))
  (bind (_relativescale3d_x _relativescale3d_y) (`KismetMathLibrary.BreakVector` (`SceneComponent.RelativeScale3D` `ターゲット`)))
  (`SceneComponent.SetRelativeScale3D` `ターゲット` (`KismetMathLibrary.MakeVector` _relativescale3d_x _relativescale3d_y 2.383601)))

(fn `Set Brake Effect`
  (`|ExecutionSequence`
    (:`then_0`
      (bind _returnvalue (`AddComponent|NODE_AddNiagaraComponent-9`))
      (bind _output_get (set `self.L_Brake_Effect01` _returnvalue))
      (`SceneComponent.K2_AttachToComponent` _output_get (`self.SkeletalMeshComponent`) "L_Brake_Effect01" "KeepRelative" "KeepRelative" "KeepRelative" true))
    (:`then_1`
      (bind _returnvalue_2 (`AddComponent|NODE_AddNiagaraComponent-8`))
      (bind _output_get_2 (set `self.L_Brake_Effect02` _returnvalue_2))
      (`SceneComponent.K2_AttachToComponent` _output_get_2 (`self.SkeletalMeshComponent`) "L_Brake_Effect02" "KeepRelative" "KeepRelative" "KeepRelative" true))))

(fn `UserConstructionScript`
  (`|ExecutionSequence`
    (:`then_0`
      (bind _returnvalue (`AddComponent|NODE_AddNiagaraComponent-1`))
      (bind _output_get (set `self.L_Leg_Effect02` _returnvalue))
      (`SceneComponent.K2_AttachToComponent` _output_get (`self.SkeletalMeshComponent`) "L_Leg_Effect02" "KeepRelative" "KeepRelative" "KeepRelative" true))
    (:`then_1`
      (bind _returnvalue_2 (`AddComponent|NODE_AddNiagaraComponent-0`))
      (bind _output_get_2 (set `self.L_Leg_Effect01` _returnvalue_2))
      (`SceneComponent.K2_AttachToComponent` _output_get_2 (`self.SkeletalMeshComponent`) "L_Leg_Effect01" "KeepRelative" "KeepRelative" "KeepRelative" true))))