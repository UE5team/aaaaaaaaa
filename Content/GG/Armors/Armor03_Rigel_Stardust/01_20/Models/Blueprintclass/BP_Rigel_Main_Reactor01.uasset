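; Main reactor Blueprint for the Rigel armor, supplying its thruster effects and passing its boost, fly and brake start montages to SetAnimMontage at BeginPlay.
; The construction script attaches Niagara components to the left and right main thruster and sub-wing smoke sockets.
; Set and Reset Boost Effect call their parent versions, then stretch or restore the main thrusters' Z scale.
; Tick prints the right thruster's Z scale as debug output.
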(event `self.ReceiveBeginPlay`
  (`self.SetAnimMontage` "/Game/Animation/Montage/Armors/Rigel_StarDust/AM_RigelBoost_Start01.AM_RigelBoost_Start01" "/Game/Animation/Montage/Armors/Rigel_StarDust/AM_Rigel_Fly_Start01.AM_Rigel_Fly_Start01" "/Game/Animation/Montage/Armors/Rigel_StarDust/AM_RigelBrake_Start01.AM_RigelBrake_Start01"))

(event `self.ReceiveTick`
  (params (DeltaSeconds :type "Float (single-precision)"))
  (bind (_relativescale3d_x _relativescale3d_y _relativescale3d_z) (`KismetMathLibrary.BreakVector` (`SceneComponent.RelativeScale3D` (`self.R_Main_Thruster01`))))
  (`KismetSystemLibrary.PrintString` (`KismetStringLibrary.Conv_DoubleToString` _relativescale3d_z)))

(fn `Reset Boost Effect`
  (`parent.Reset Boost Effect`)
  (`self.Reset Thruster Boust Efect Scale` (`self.R_Main_Thruster01`))
  (`self.Reset Thruster Boust Efect Scale` (`self.L_Main_Thruster01`)))

(fn `Reset Thruster Boust Efect Scale`
  (params (`ターゲット` :type "SceneComponent Object Reference"))
  (bind (_relativescale3d_x _relativescale3d_y) (`KismetMathLibrary.BreakVector` (`SceneComponent.RelativeScale3D` `ターゲット`)))
  (`SceneComponent.SetRelativeScale3D` `ターゲット` (`KismetMathLibrary.MakeVector` _relativescale3d_x _relativescale3d_y 1.0)))

(fn `Set Boost Effect`
  (`parent.Set Boost Effect`)
  (`self.Set Thruster Boust Efect Scale` (`self.R_Main_Thruster01`))
  (`self.Set Thruster Boust Efect Scale` (`self.L_Main_Thruster01`)))

(fn `Set Thruster Boust Efect Scale`
  (params (`ターゲット` :type "SceneComponent Object Reference"))
  (bind (_relativescale3d_x _relativescale3d_y) (`KismetMathLibrary.BreakVector` (`SceneComponent.RelativeScale3D` `ターゲット`)))
  (`SceneComponent.SetRelativeScale3D` `ターゲット` (`KismetMathLibrary.MakeVector` _relativescale3d_x _relativescale3d_y 2.777778)))

(fn `UserConstructionScript`
  (`|ExecutionSequence`
    (:`then_0`
      (bind _returnvalue (`AddComponent|NODE_AddNiagaraComponent-1`))
      (bind _output_get (set `self.R_Main_Thruster01` _returnvalue))
      (`SceneComponent.K2_AttachToComponent` _output_get (`self.SkeletalMeshComponent`) "R_Main_Thruster01" "KeepRelative" "KeepRelative" "KeepRelative" true))
    (:`then_1`
      (bind _returnvalue_2 (`AddComponent|NODE_AddNiagaraComponent-0`))
      (bind _output_get_2 (set `self.L_Main_Thruster01` _returnvalue_2))
      (`SceneComponent.K2_AttachToComponent` _output_get_2 (`self.SkeletalMeshComponent`) "L_Main_Thruster01" "KeepRelative" "KeepRelative" "KeepRelative" true))
    (:`then_2`
      (bind _returnvalue_3 (`AddComponent|NODE_AddNiagaraComponent-2`))
      (`SceneComponent.K2_AttachToComponent` _returnvalue_3 (`self.SkeletalMeshComponent`) "L_Sub_Wing01_Smoke01" "KeepRelative" "KeepRelative" "KeepRelative" true))
    (:`then_3`
      (bind _returnvalue_4 (`AddComponent|NODE_AddNiagaraComponent-3`))
      (`SceneComponent.K2_AttachToComponent` _returnvalue_4 (`self.SkeletalMeshComponent`) "R_Sub_Wing01_Smoke01" "KeepRelative" "KeepRelative" "KeepRelative" true))))