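; Lux mount Blueprint that assembles armor and equipment parts onto a skeletal mesh, with no active gameplay logic.
; The construction script adds static mesh components and attaches them to named sockets for the cap, both arms, hips and legs, and a rifle.
; The thruster socket receives a child actor component instead of a static mesh.
; All attachments keep relative transforms, and the event graph holds only disabled placeholder events.
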(fn `UserConstructionScript`
  (`|ExecutionSequence`
    (:`then_0`
      (bind _returnvalue (`AddComponent|NODE_AddStaticMeshComponent-6`))
      (`SceneComponent.K2_AttachToComponent` _returnvalue (`self.SkeletalMeshComponent`) "Lux_Cap" "KeepRelative" "KeepRelative" "KeepRelative" true))
    (:`then_1`
      (bind _returnvalue_2 (`AddComponent|NODE_AddChildActorComponent-0`))
      (`SceneComponent.K2_AttachToComponent` _returnvalue_2 (`self.SkeletalMeshComponent`) "Lux_Thruster" "KeepRelative" "KeepRelative" "KeepRelative" true))
    (:`then_2`
      (bind _returnvalue_3 (`AddComponent|NODE_AddStaticMeshComponent-2`))
      (`SceneComponent.K2_AttachToComponent` _returnvalue_3 (`self.SkeletalMeshComponent`) "L_Lux_Arm" "KeepRelative" "KeepRelative" "KeepRelative" true))
    (:`then_3`
      (bind _returnvalue_4 (`AddComponent|NODE_AddStaticMeshComponent-3`))
      (`SceneComponent.K2_AttachToComponent` _returnvalue_4 (`self.SkeletalMeshComponent`) "R_Lux_Arm" "KeepRelative" "KeepRelative" "KeepRelative" true))
    (:`then_4`
      (bind _returnvalue_5 (`AddComponent|NODE_AddStaticMeshComponent-0`))
      (`SceneComponent.K2_AttachToComponent` _returnvalue_5 (`self.SkeletalMeshComponent`) "R_Lux_Hip" "KeepRelative" "KeepRelative" "KeepRelative" true))
    (:`then_5`
      (bind _returnvalue_6 (`AddComponent|NODE_AddStaticMeshComponent-1`))
      (`SceneComponent.K2_AttachToComponent` _returnvalue_6 (`self.SkeletalMeshComponent`) "L_Lux_Hip" "KeepRelative" "KeepRelative" "KeepRelative" true))
    (:`then_6`
      (bind _returnvalue_7 (`AddComponent|NODE_AddStaticMeshComponent-5`))
      (`SceneComponent.K2_AttachToComponent` _returnvalue_7 (`self.SkeletalMeshComponent`) "R_Lux_leg" "KeepRelative" "KeepRelative" "KeepRelative" true))
    (:`then_7`
      (bind _returnvalue_8 (`AddComponent|NODE_AddStaticMeshComponent-4`))
      (`SceneComponent.K2_AttachToComponent` _returnvalue_8 (`self.SkeletalMeshComponent`) "L_Lux_leg" "KeepRelative" "KeepRelative" "KeepRelative" true))
    (:`then_8`
      (bind _returnvalue_9 (`AddComponent|NODE_AddStaticMeshComponent-7`))
      (`SceneComponent.K2_AttachToComponent` _returnvalue_9 (`self.SkeletalMeshComponent`) "Rifle01" "KeepRelative" "KeepRelative" "KeepRelative" true))))