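; BP_Endent_Mount_Farem is an armor mount Blueprint for the Endent in the Farem set, assembled from separate mesh parts.
; Its construction script adds cap, left leg and right leg static meshes plus a skeletal thruster mesh.
; Each part attaches to its named socket on the main skeletal mesh component with relative transforms.
; The event graph holds only disabled default events, so it has no runtime logic.
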(fn `UserConstructionScript`
  (`|ExecutionSequence`
    (:`then_0`
      (bind _returnvalue (`AddComponent|NODE_AddStaticMeshComponent-2`))
      (`SceneComponent.K2_AttachToComponent` _returnvalue (`self.SkeletalMeshComponent`) "Endent_Cap" "KeepRelative" "KeepRelative" "KeepRelative" true))
    (:`then_1`
      (bind _returnvalue_2 (`AddComponent|NODE_AddSkeletalMeshComponent-0`))
      (`SceneComponent.K2_AttachToComponent` _returnvalue_2 (`self.SkeletalMeshComponent`) "Endent_Thruster" "KeepRelative" "KeepRelative" "KeepRelative" true))
    (:`then_2`
      (bind _returnvalue_3 (`AddComponent|NODE_AddStaticMeshComponent-0`))
      (`SceneComponent.K2_AttachToComponent` _returnvalue_3 (`self.SkeletalMeshComponent`) "L_Endent_leg" "KeepRelative" "KeepRelative" "KeepRelative" true))
    (:`then_3`
      (bind _returnvalue_4 (`AddComponent|NODE_AddStaticMeshComponent-1`))
      (`SceneComponent.K2_AttachToComponent` _returnvalue_4 (`self.SkeletalMeshComponent`) "R_Endent_leg" "KeepRelative" "KeepRelative" "KeepRelative" true))))