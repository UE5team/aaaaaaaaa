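; Mount Blueprint that assembles the Rigel armor set for Siori by attaching its pieces to a skeletal mesh.
; The Construction Script adds static mesh, skeletal mesh and child actor components, each attached to a named socket with relative transforms.
; Pieces include cap, muffler, thruster, side parts, hips, legs, shoes, spikes and a rifle, with thruster and legs as child actors.
; The event graph holds no gameplay logic.
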(fn `UserConstructionScript`
  (`|ExecutionSequence`
    (:`then_0`
      (bind _returnvalue (`AddComponent|NODE_AddStaticMeshComponent-7`))
      (`SceneComponent.K2_AttachToComponent` _returnvalue (`self.SkeletalMeshComponent`) "Rigel_Cap" "KeepRelative" "KeepRelative" "KeepRelative" true))
    (:`then_1`
      (bind _returnvalue_2 (`AddComponent|NODE_AddSkeletalMeshComponent-5`))
      (`SceneComponent.K2_AttachToComponent` _returnvalue_2 (`self.SkeletalMeshComponent`) "Rigel_Muffler" "KeepRelative" "KeepRelative" "KeepRelative" true))
    (:`then_2`
      (bind _returnvalue_3 (`AddComponent|NODE_AddChildActorComponent-0`))
      (`SceneComponent.K2_AttachToComponent` _returnvalue_3 (`self.SkeletalMeshComponent`) "Rigel_Thruster" "KeepRelative" "KeepRelative" "KeepRelative" true))
    (:`then_3`
      (bind _returnvalue_4 (`AddComponent|NODE_AddStaticMeshComponent-11`))
      (`SceneComponent.K2_AttachToComponent` _returnvalue_4 (`self.SkeletalMeshComponent`) "R_Rigel_Parts01" "KeepRelative" "KeepRelative" "KeepRelative" true))
    (:`then_4`
      (bind _returnvalue_5 (`AddComponent|NODE_AddStaticMeshComponent-12`))
      (`SceneComponent.K2_AttachToComponent` _returnvalue_5 (`self.SkeletalMeshComponent`) "R_Rigel_Parts02" "KeepRelative" "KeepRelative" "KeepRelative" true))
    (:`then_5`
      (bind _returnvalue_6 (`AddComponent|NODE_AddStaticMeshComponent-8`))
      (`SceneComponent.K2_AttachToComponent` _returnvalue_6 (`self.SkeletalMeshComponent`) "L_Rigel_Parts01" "KeepRelative" "KeepRelative" "KeepRelative" true))
    (:`then_6`
      (bind _returnvalue_7 (`AddComponent|NODE_AddStaticMeshComponent-9`))
      (`SceneComponent.K2_AttachToComponent` _returnvalue_7 (`self.SkeletalMeshComponent`) "L_Rigel_Parts02" "KeepRelative" "KeepRelative" "KeepRelative" true))
    (:`then_7`
      (bind _returnvalue_8 (`AddComponent|NODE_AddSkeletalMeshComponent-1`))
      (`SceneComponent.K2_AttachToComponent` _returnvalue_8 (`self.SkeletalMeshComponent`) "L_Rigel_Hip" "KeepRelative" "KeepRelative" "KeepRelative" true))
    (:`then_8`
      (bind _returnvalue_9 (`AddComponent|NODE_AddSkeletalMeshComponent-6`))
      (`SceneComponent.K2_AttachToComponent` _returnvalue_9 (`self.SkeletalMeshComponent`) "R_Rigel_Hip" "KeepRelative" "KeepRelative" "KeepRelative" true))
    (:`then_9`
      (bind _returnvalue_10 (`AddComponent|NODE_AddChildActorComponent-1`))
      (`SceneComponent.K2_AttachToComponent` _returnvalue_10 (`self.SkeletalMeshComponent`) "L_Rigel_Leg" "KeepRelative" "KeepRelative" "KeepRelative" true))
    (:`then_10`
      (bind _returnvalue_11 (`AddComponent|NODE_AddChildActorComponent-2`))
      (`SceneComponent.K2_AttachToComponent` _returnvalue_11 (`self.SkeletalMeshComponent`) "R_Rigel_Leg" "KeepRelative" "KeepRelative" "KeepRelative" true))
    (:`then_11`
      (bind _returnvalue_12 (`AddComponent|NODE_AddStaticMeshComponent-10`))
      (`SceneComponent.K2_AttachToComponent` _returnvalue_12 (`self.SkeletalMeshComponent`) "L_Rigel_Shoes" "KeepRelative" "KeepRelative" "KeepRelative" true))
    (:`then_12`
      (bind _returnvalue_13 (`AddComponent|NODE_AddStaticMeshComponent-13`))
      (`SceneComponent.K2_AttachToComponent` _returnvalue_13 (`self.SkeletalMeshComponent`) "R_Rigel_Shoes" "KeepRelative" "KeepRelative" "KeepRelative" true))
    (:`then_13`
      (bind _returnvalue_14 (`AddComponent|NODE_AddSkeletalMeshComponent-3`))
      (`SceneComponent.K2_AttachToComponent` _returnvalue_14 (`self.SkeletalMeshComponent`) "L_Rigel_Spike" "KeepRelative" "KeepRelative" "KeepRelative" true))
    (:`then_14`
      (bind _returnvalue_15 (`AddComponent|NODE_AddSkeletalMeshComponent-8`))
      (`SceneComponent.K2_AttachToComponent` _returnvalue_15 (`self.SkeletalMeshComponent`) "R_Rigel_Spike" "KeepRelative" "KeepRelative" "KeepRelative" true))
    (:`then_15`
      ;[1 1 1] Rifle
      (bind _returnvalue_16 (`AddComponent|NODE_AddStaticMeshComponent-14`))
      (`SceneComponent.K2_AttachToComponent` _returnvalue_16 (`self.SkeletalMeshComponent`) "Rifle01" "KeepRelative" "KeepRelative" "KeepRelative" true))))