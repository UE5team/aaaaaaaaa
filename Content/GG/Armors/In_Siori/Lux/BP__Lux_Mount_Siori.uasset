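; Mount Blueprint for the Lux armor of Siori, assembling armor parts on a skeletal mesh.
; Its construction script adds a skeletal mesh component and attaches it to the Lux_Thruster socket with relative transforms.
; Similar static mesh attachments for hip, arm, cap and leg sockets are present but disconnected, so only the thruster part is built by this script.
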(fn `UserConstructionScript`
  (bind _returnvalue (`AddComponent|NODE_AddSkeletalMeshComponent-0`))
  (`SceneComponent.K2_AttachToComponent` _returnvalue (`self.SkeletalMeshComponent`) "Lux_Thruster" "KeepRelative" "KeepRelative" "KeepRelative" true))