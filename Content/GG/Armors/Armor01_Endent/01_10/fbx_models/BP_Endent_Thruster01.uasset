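; Thruster Blueprint for the Endent armor that dresses its skeletal mesh with left and right exhaust and wing effects.
; The Construction Script adds Niagara components at the main effect sockets for normal and boost thrust, static meshes at the wing sockets, and separate Niagara components at the boost-only sockets.
; All are attached by socket name with relative transforms; the event graph is empty, so no effect switching happens here.
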(fn `UserConstructionScript`
  (`|ExecutionSequence`
    (:`then_0`
      ;[1 1 1] 通常エフェクト/ブースト
      (bind _returnvalue (`AddComponent|NODE_AddNiagaraComponent-0`))
      (`SceneComponent.K2_AttachToComponent` _returnvalue (`self.SkeletalMeshComponent`) "L_Effect01" "KeepRelative" "KeepRelative" "KeepRelative" true))
    (:`then_1`
      (bind _returnvalue_2 (`AddComponent|NODE_AddNiagaraComponent-1`))
      (`SceneComponent.K2_AttachToComponent` _returnvalue_2 (`self.SkeletalMeshComponent`) "L_Effect02" "KeepRelative" "KeepRelative" "KeepRelative" true))
    (:`then_2`
      (bind _returnvalue_3 (`AddComponent|NODE_AddNiagaraComponent-2`))
      (`SceneComponent.K2_AttachToComponent` _returnvalue_3 (`self.SkeletalMeshComponent`) "R_Effect01" "KeepRelative" "KeepRelative" "KeepRelative" true))
    (:`then_3`
      (bind _returnvalue_4 (`AddComponent|NODE_AddNiagaraComponent-3`))
      (`SceneComponent.K2_AttachToComponent` _returnvalue_4 (`self.SkeletalMeshComponent`) "R_Effect02" "KeepRelative" "KeepRelative" "KeepRelative" true))
    (:`then_4`
      (bind _returnvalue_5 (`AddComponent|NODE_AddStaticMeshComponent-5`))
      (`SceneComponent.K2_AttachToComponent` _returnvalue_5 (`self.SkeletalMeshComponent`) "L_Wing_Effect01" "KeepRelative" "KeepRelative" "KeepRelative" true))
    (:`then_5`
      (bind _returnvalue_6 (`AddComponent|NODE_AddStaticMeshComponent-6`))
      (`SceneComponent.K2_AttachToComponent` _returnvalue_6 (`self.SkeletalMeshComponent`) "L_Wing_Effect02" "KeepRelative" "KeepRelative" "KeepRelative" true))
    (:`then_6`
      (bind _returnvalue_7 (`AddComponent|NODE_AddStaticMeshComponent-8`))
      (`SceneComponent.K2_AttachToComponent` _returnvalue_7 (`self.SkeletalMeshComponent`) "R_Wing_Effect01" "KeepRelative" "KeepRelative" "KeepRelative" true))
    (:`then_7`
      (bind _returnvalue_8 (`AddComponent|NODE_AddStaticMeshComponent-7`))
      (`SceneComponent.K2_AttachToComponent` _returnvalue_8 (`self.SkeletalMeshComponent`) "R_Wing_Effect02" "KeepRelative" "KeepRelative" "KeepRelative" true))
    (:`then_8`
      ;[1 1 1] ブーストの時にのみ出るエフェクト
      (bind _returnvalue_9 (`AddComponent|NODE_AddNiagaraComponent-4`))
      (`SceneComponent.K2_AttachToComponent` _returnvalue_9 (`self.SkeletalMeshComponent`) "L_Boost_Effect01" "KeepRelative" "KeepRelative" "KeepRelative" true))
    (:`then_9`
      (bind _returnvalue_10 (`AddComponent|NODE_AddNiagaraComponent-5`))
      (`SceneComponent.K2_AttachToComponent` _returnvalue_10 (`self.SkeletalMeshComponent`) "R_Boost_Effect01" "KeepRelative" "KeepRelative" "KeepRelative" true))))