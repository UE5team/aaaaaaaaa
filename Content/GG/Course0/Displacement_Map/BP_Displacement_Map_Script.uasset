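; Geometry Script Blueprint that builds a displaced dynamic mesh from a source static mesh and a displacement texture.
; Unless Frozen, its event copies SourceMesh into the target mesh, applies PN tessellation, displaces it from DisplacementMap, then recomputes normals.
; As wired, processing follows the copy's Failure output, and the Magnitube variable is truncated into the displacement UV layer.
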(event `CustomEvent`
  (params (TargetMesh :type "DynamicMesh Object Reference"))
  (if (not (`self.Frozen`))
    (`self.SourceMesh`
      (:`then`
        (bind _returnvalue (`GeometryScriptLibrary_StaticMeshFunctions.CopyMeshFromStaticMesh` (`self.SourceMesh`) TargetMesh (struct) (struct) null)
          (:`Failure`
            (`GeometryScriptLibrary_MeshSubdivideFunctions.ApplyPNTessellation` _returnvalue (struct) (`self.Tessellation Level`) null)
            (`self.SourceMesh`
              (:`then`
                (bind _returnvalue_2 (`GeometryScriptLibrary_MeshDeformFunctions.ApplyDisplaceFromTextureMap` null (`self.Displacement_Map`) (struct) (struct) (`KismetMathLibrary.FTrunc` (`self.Magnitube`)) null))
                (`GeometryScriptLibrary_MeshNormalsFunctions.RecomputeNormals` _returnvalue_2 (struct) null))
              (:`else`)))))
      (:`else`))))

(fn `UserConstructionScript`)