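; Countdown board Blueprint with a text render component, built to count down and then show a GO text.
; The construction script sets the initial text from ConstTextValue.
; A Delay-based loop writes CountNum each second, decrements it and shows TextGO once it is no longer positive.
; That loop is disconnected: BeginPlay only runs a one-second Delay, so the countdown never executes.
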(event `self.ReceiveBeginPlay`
  (`KismetSystemLibrary.Delay` 1.0))

(fn `UserConstructionScript`
  (`TextRenderComponent.K2_SetText` (`self.TextRender`) (`self.ConstTextValue`)))