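; Race course spline actor that tracks the player's progress, lap count and wrong-way driving.
; Tick projects the player onto the spline for percent progress, treating jumps over half the course as lap changes and notifying the goal tape on forward laps.
; A yaw comparison against the spline shows the reverse-run widget after a short delay.
; The construction script can shift the start by cycling spline points; reverse-distance measurement is never called.
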(event `self.ReceiveBeginPlay`
  ;[1 1 1] biginPlay
  (bind _asbp_player (cast `/Game/Blueprint/Player/BP_Player` (`GameplayStatics.GetPlayerPawn` 0)))
  (set `self.BP Player` _asbp_player)
  (set `self.Max Spline Length` (`SplineComponent.GetSplineLength` (`self.CourseSpline`))))

(event `self.ReceiveTick`
  (params (DeltaSeconds :type "Float (single-precision)"))
  (bind _bp_goaltape (`self.BP_Goaltape`))
  (`|ExecutionSequence`
    (:`then_0`
      (`self.ToReverse` DeltaSeconds))
    (:`then_1`)
    (:`then_2`
      (bind _bp_player (`self.BP Player`)
        (:`then`
          (bind _returnvalue (* (/ (`SplineComponent.GetDistanceAlongSplineAtSplineInputKey` (`self.CourseSpline`) (`SplineComponent.FindInputKeyClosestToWorldLocation` (`self.CourseSpline`) (`SplineComponent.FindLocationClosestToWorldLocation` (`self.CourseSpline`) (`self.K2_GetActorLocation` _bp_player) "World"))) (`self.Max Spline Length`)) 100.0))
          (set `self.Course Percent` (`KismetMathLibrary.FFloor` _returnvalue))
          (bind _output_get (set `self.CurrentProgress` _returnvalue))
          (bind _output_get_2 (set `self.ProgressDiff` (- _output_get (`self.PreviousProgress`))))
          (if (> (`KismetMathLibrary.Abs` _output_get_2) 50.0)
            (if (< (`self.PreviousProgress`) (`self.CurrentProgress`))
              (set `self.PreviousProgress` (`self.CurrentProgress`))
              (set `self.Number of laps` (- (`self.Number of laps`) 1))
              (else
                (set `self.PreviousProgress` (`self.CurrentProgress`))
                (set `self.Number of laps` (+ (`self.Number of laps`) 1))
                (`/Engine/EditorBlueprintResources/StandardMacros.IsValid` _bp_goaltape
                  (:`Is Valid`
                    _)
                  (:`Is Not Valid`
                    (bind _returnvalue_2 (`GameplayStatics.GetActorOfClass` "/Game/Blueprint/Maps/Goal_tape_Blueprint.Goal_tape_Blueprint_C"))
                    (set `self.BP_Goaltape` _returnvalue_2)))
                (`/Game/Blueprint/Maps/Goal_tape_Blueprint.Goal` _bp_goaltape (`self.Number of laps`))))
            (elif (< (`self.ProgressDiff`) 0.0)
              (set `self.is to reverse` true)
              (set `self.PreviousProgress` (`self.CurrentProgress`))
              (else
                (set `self.is to reverse` false)
                (set `self.PreviousProgress` (`self.CurrentProgress`))))))
        (:`else`)))))

(fn `Get Course Progress`
  (returns (`Number of laps` :type Integer) (`Course Percent` :type Integer))
  (return (`self.Number of laps`) (`self.Course Percent`)))

(fn `Set Course Progress`
  (params (`Number of laps` :type "Integer (by ref)") (`Course Percent` :type "Integer (by ref)"))
  (`|VariableSetRef` `Number of laps` (`self.Number of laps`))
  (`|VariableSetRef` `Course Percent` (`self.Course Percent`))
  (return))

(fn `ToReverse`
  (params (InputPin :type "Float (single-precision)"))
  (bind _bp_player (`self.BP Player`))
  (bind (_returnvalue_roll _returnvalue_pitch _returnvalue_yaw) (`KismetMathLibrary.BreakRotator` (`self.K2_GetActorRotation` _bp_player)))
  (`self.BP Player`
    (:`then`
      (if (< (`KismetMathLibrary.Abs` (`KismetMathLibrary.NormalizeAxis` (- (.yaw (.rotation (`SplineComponent.FindTransformClosestToWorldLocation` (`self.CourseSpline`) (`self.K2_GetActorLocation` _bp_player) "World" false))) _returnvalue_yaw))) 130.0)
        (set `self.is to reverse` false)
        (set `self.Elapsed time` 0.0)
        (bind _returnvalue (`/Game/Blueprint/System/FL_MyLibrary.getWidgetCreator`))
        (`Widget.SetVisibility` (`/Game/Blueprint/System/BP_WidgetCreater.getUI Reverse Run` _returnvalue) "Hidden")
        (else
          (bind _output_get (set `self.Elapsed time` (+ (`self.Elapsed time`) InputPin)))
          (if (> _output_get 1.0)
            (set `self.is to reverse` true)
            (bind _returnvalue_2 (`/Game/Blueprint/System/FL_MyLibrary.getWidgetCreator`))
            (bind _ui_reverse_run (`/Game/Blueprint/System/BP_WidgetCreater.getUI Reverse Run` _returnvalue_2))
            (`/Engine/EditorBlueprintResources/StandardMacros.IsValid` _ui_reverse_run
              (:`Is Valid`
                (`Widget.SetVisibility` _ui_reverse_run "Visible"))
              (:`Is Not Valid`
                (`UserWidget.AddToViewport` _ui_reverse_run 0)))
            (else
              (set `self.is to reverse` false)
              (bind _returnvalue_3 (`/Game/Blueprint/System/FL_MyLibrary.getWidgetCreator`))
              (`Widget.SetVisibility` (`/Game/Blueprint/System/BP_WidgetCreater.getUI Reverse Run` _returnvalue_3) "Hidden"))))))
    (:`else`)))

(fn `UserConstructionScript`
  (locals (`Set point num` :type Integer))
  (bind _coursespline (`self.CourseSpline`))
  (bind _rotationstartpointnum (`self.RotationStartPointNum`))
  (bind _splinepoints (`self.SplinePoints`))
  (bind _set_point_num (`local.Set point num`))
  (bind _returnvalue (`KismetArrayLibrary.Array_Length` _splinepoints))
  (bind _returnvalue_2 (`SplineComponent.GetNumberOfSplinePoints` (`self.CourseSpline`)))
  (bind (_output_inputkey _output_position _output_arrivetangent _output_leavetangent _output_rotation _output_scale _output_type) (break `SplinePoint` (`|GetArrayItem` _splinepoints _set_point_num)))
  (if (not (> (`KismetMathLibrary.Abs_Int` (`self.RotationStartPointNum`)) (`SplineComponent.GetNumberOfSplinePoints` (`self.CourseSpline`))))
    (if (not (`self.ResetStartPoint`))
      (if (!= (`self.RotationStartPointNum`) 0)
        (if (not (> (`self.RotationStartPointNum`) 0))
          (set `self.RotationStartPointNum` (+ (`SplineComponent.GetNumberOfSplinePoints` (`self.CourseSpline`)) (`self.RotationStartPointNum`))))
        (`|ExecutionSequence` :!label _label
          (:`then_0`
            (`KismetArrayLibrary.Array_Resize` (`self.SplinePoints`) _returnvalue_2)
            (for _index (range _returnvalue_2)
              (bind (_returnvalue_location _returnvalue_rotation _returnvalue_scale) (`KismetMathLibrary.BreakTransform` (`SplineComponent.GetTransformAtSplinePoint` _coursespline _index "World" true)))
              (`KismetArrayLibrary.Array_Set` (`self.SplinePoints`) _index (make `SplinePoint` (`SplineComponent.GetDistanceAlongSplineAtSplinePoint` _coursespline _index) _returnvalue_location (`SplineComponent.GetArriveTangentAtSplinePoint` _coursespline _index "World") (`SplineComponent.GetLeaveTangentAtSplinePoint` _coursespline _index "World") _returnvalue_rotation _returnvalue_scale (`SplineComponent.GetSplinePointType` _coursespline _index)))))
          (:`then_1`
            (for _index_2 (range _returnvalue)
              (bind _returnvalue_3 (+ _index_2 _rotationstartpointnum))
              (if (> _returnvalue _returnvalue_3)
                (set `local.Set point num` _returnvalue_3)
                (else
                  (set `local.Set point num` (+ (- _index_2 _returnvalue) _rotationstartpointnum))))
              (`KismetSystemLibrary.PrintString` (`KismetStringLibrary.Conv_IntToString` _set_point_num))
              (`SplineComponent.SetLocationAtSplinePoint` (`self.CourseSpline`) _index_2 _output_position "World" true)
              (`SplineComponent.SetRotationAtSplinePoint` (`self.CourseSpline`) _index_2 _output_rotation "World" true)
              (`SplineComponent.SetTangentsAtSplinePoint` (`self.CourseSpline`) _index_2 _output_arrivetangent _output_leavetangent "World" true)
              (`SplineComponent.SetSplinePointType` (`self.CourseSpline`) _index_2 _output_type true)
              (`SplineComponent.SetScaleAtSplinePoint` (`self.CourseSpline`) _index_2 _output_scale true)))))
      (else
        (set `self.RotationStartPointNum` 0 :!label _label_2)
        (set `self.ResetStartPoint` false)
        (goto _label)))
    (else
      (goto _label_2))))