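; BP_Enemy is a turret-like enemy that tracks the player within range and periodically fires BP_Enemy_Bullet projectiles.
; Tick checks player distance, smoothly yaws the whole actor using EnemyTop's rotation, and pauses or resumes a looping launch timer created through DoOnce.
; Bullets spawn at EnemyTop's location.
; Damage reduces Life, and at zero the enemy drops a diagonal row of BP_Enemy_Points pickups before destroying itself.
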(event `self.ReceiveBeginPlay`
  (bind _asgi_defolut (cast `/Game/Blueprint/Maps/GI_Defolut` (`GameplayStatics.GetGameInstance`)))
  (set `self.GI_Defolut` _asgi_defolut))

(event `self.ReceiveTick`
  (params (DeltaSeconds :type "Float (single-precision)"))
  (bind _returnvalue (`GameplayStatics.GetPlayerCharacter` 0))
  (bind _enemy_top (`self.enemy top`))
  (bind _returnvalue_2 (`KismetMathLibrary.VSize` (- (`self.K2_GetActorLocation`) (`self.K2_GetActorLocation` _returnvalue))))
  (bind (_returnvalue_roll _returnvalue_pitch _returnvalue_yaw) (`KismetMathLibrary.BreakRotator` (`KismetMathLibrary.RInterpTo` (`SceneComponent.K2_GetComponentRotation` _enemy_top) (`KismetMathLibrary.Conv_VectorToRotator` (- (`SceneComponent.K2_GetComponentLocation` _enemy_top) (`self.K2_GetActorLocation` (`GameplayStatics.GetPlayerCharacter` 0)))) (`GameplayStatics.GetWorldDeltaSeconds`) 5.0)))
  ;[1 1 1] 敵の射程範囲の計算
  (`/Engine/EditorBlueprintResources/StandardMacros.IsValid` _returnvalue
    (:`Is Valid`
      ;[1 1 1] 弾のクールタイム
      (if (and (<= _returnvalue_2 30000.0) (>= _returnvalue_2 0.0))
        ;[1 1 1] 砲身がPlayerを狙って追尾する
        (`KismetSystemLibrary.K2_UnPauseTimerHandle` (`self.Launch Timer`))
        (`self.K2_SetActorRotation` (`KismetMathLibrary.MakeRotator` 0.0 0.0 _returnvalue_yaw))
        (`/Engine/EditorBlueprintResources/StandardMacros.DoOnce` false
          (:`Completed`
            ;[1 1 1] 弾が出るイベントの発生
            (bind _returnvalue_3 (`KismetSystemLibrary.K2_SetTimerDelegate` (`|CreateDelegate` :!event `LaunchBall`) 3.0 true))
            (set `self.Launch Timer` _returnvalue_3)))
        (else
          (`KismetSystemLibrary.K2_PauseTimerHandle` (`self.Launch Timer`)))))))

(event `LaunchBall`
  (bind _returnvalue_location (`KismetMathLibrary.BreakTransform` (`SceneComponent.K2_GetComponentToWorld` (`self.enemy top`))))
  ;[1 1 1] 弾の生成場所
  (`|SpawnActorFromClass` "/Game/Blueprint/Enemy/BP_Enemy_Bullet.BP_Enemy_Bullet_C" (`KismetMathLibrary.MakeTransform` _returnvalue_location) "Undefined" "OverrideRootScale" null 1 (0.0 0.0 0.0) null))

(event `self.ReceiveAnyDamage`
  (params (Damage :type "Float (single-precision)") (DamageType :type "DamageType Object Reference") (InstigatedBy :type "Controller Object Reference") (DamageCauser :type "Actor Object Reference"))
  (bind _output_get (set `self.Life` (- (`self.Life`) Damage)))
  (if (<= _output_get 0.0)
    ;[1 1 1] ポイントをスポーンする
    (for _index (range 1 6)
      (`|SpawnActorFromClass` "/Game/Blueprint/point/BP_Enemy_Points.BP_Enemy_Points_C" (`KismetMathLibrary.MakeTransform` (+ (* _index (20.0 20.0 0.0)) (`self.K2_GetActorLocation`)) (struct) (0.1 0.1 0.1)) "Undefined" "OverrideRootScale" null null))
    (`self.K2_DestroyActor`)))

(fn `UserConstructionScript`)