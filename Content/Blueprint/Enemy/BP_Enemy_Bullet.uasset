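; Enemy bullet actor that flies toward the player's position at spawn and destroys itself after a short delay.
; BeginPlay stores the normalized direction to the player, and Tick applies it times Speed as a local-space offset, without sweep or delta-time scaling.
; A PlayerDamage event, not called within this Blueprint, passes half the player's ConstMaxHP to TakeDamage on BP_InGame_GameMode.
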(event `self.ReceiveBeginPlay`
  (set `self.Dilection` (`KismetMathLibrary.Normal` (- (`self.K2_GetActorLocation` (`GameplayStatics.GetPlayerCharacter` 0)) (`self.K2_GetActorLocation` self))))
  ;[1 1 1] 弾が出てから5秒後に消滅する
  (`KismetSystemLibrary.Delay` 5.0)
  (`self.K2_DestroyActor`))

(event `self.ReceiveTick`
  (params (DeltaSeconds :type "Float (single-precision)"))
  ;[1 1 1] 弾の移動する動き
  (`self.K2_AddActorLocalOffset` (* (`self.Dilection`) (`self.speed`))))

(event `Player Damage`
  ;[1 1 1] PlayerにDamageを与える
  (bind _returnvalue (`GameplayStatics.GetActorOfClass` "/Game/Blueprint/Maps/BP_InGame_GameMode.BP_InGame_GameMode_C"))
  (`/Game/Blueprint/Maps/BP_InGame_GameMode.Take Damage` _returnvalue (/ (`/Game/Blueprint/Player/BP_Player.Const MaxHP` (`self.Get BP_Player`)) 2.0)))

(fn `Get BP_Player`
  (returns (BP_Player :type "/Game/Blueprint/Player/BP_Player Object Reference"))
  (bind _returnvalue (`GameplayStatics.GetActorOfClass` "/Game/Blueprint/Player/BP_Player.BP_Player_C"))
  (return _returnvalue))

(fn `UserConstructionScript`)