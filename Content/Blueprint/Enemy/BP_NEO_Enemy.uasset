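; Propeller-driven enemy that rides the BP_TM_Spline matching its EnemyIndex, yawing and rolling toward the player.
; Tick spins three propellers, updates spline movement and runs a range-and-cooldown attack check calling LaunchBall, which is empty here.
; Lethal damage conditionally removes it from the player's SMG target array, spawns point pickups and destroys it.
; Events swap the lock-on marker's material between default, locked and attack-locked states.
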(event `self.ReceiveBeginPlay`
  (bind _bp_tm_spline (`self.Get BP_TM_Spline`))
  (bind _transform (`/Game/Blueprint/Enemy/BP_TM_Spline.Spline Transform` _bp_tm_spline (`/Game/Blueprint/Enemy/BP_TM_Spline.Distance` _bp_tm_spline) (`/Game/Blueprint/Enemy/BP_TM_Spline.Speed` _bp_tm_spline)))
  (`SceneComponent.K2_SetWorldTransform` (`self.StaticMesh`) (`KismetMathLibrary.MakeTransform` (.location _transform) (`self.Set Player to Enemy Dist`) (.scale _transform)) false false))

(event `self.ReceiveActorBeginOverlap`
  (params (OtherActor :type "Actor Object Reference")))

(event `self.ReceiveTick`
  (params (DeltaSeconds :type "Float (single-precision)"))
  (bind _bp_tm_spline (`self.Get BP_TM_Spline`))
  (bind (_return_rotation_roll _return_rotation_pitch _return_rotation_yaw) (`KismetMathLibrary.BreakRotator` (`self.Set Player to Enemy Dist`)))
  (bind _enemy_size (`self.Enemy Size`))
  (`|ExecutionSequence`
    (:`then_0`
      (`self.Move_Puropera`)
      (`self.Move_Puropera1`)
      (`self.Move_Puropera2`))
    (:`then_1`
      (`self.Attack_Buki`))
    (:`then_2`
      (bind _transform (`/Game/Blueprint/Enemy/BP_TM_Spline.Spline Transform` _bp_tm_spline (`/Game/Blueprint/Enemy/BP_TM_Spline.Distance` _bp_tm_spline) (* (`/Game/Blueprint/Enemy/BP_TM_Spline.Speed` _bp_tm_spline) (`GameplayStatics.GetWorldDeltaSeconds`))))
      (`SceneComponent.K2_SetWorldTransform` (`self.StaticMeshComponent`) (`KismetMathLibrary.MakeTransform` (.location _transform) (struct) _enemy_size) false false)
      (`SceneComponent.K2_SetWorldTransform` (`self.StaticMesh`) (`KismetMathLibrary.MakeTransform` (.location _transform) (`KismetMathLibrary.MakeRotator` _return_rotation_roll 0.0 _return_rotation_yaw) _enemy_size) false false))))

(event `LaunchBall`
  ;[1 1 1] 弾の生成場所
)

(event `self.ReceiveAnyDamage`
  (params (Damage :type "Float (single-precision)") (DamageType :type "DamageType Object Reference") (InstigatedBy :type "Controller Object Reference") (DamageCauser :type "Actor Object Reference"))
  (bind _output_get (set `self.Life` (- (`self.Life`) Damage)))
  (if (<= _output_get 0.0)
    (`self.Remove_Enemy_Array`)
    ;[1 1 1] ポイントをスポーンする
    (for _index (range 1 6)
      (`|SpawnActorFromClass` "/Game/Blueprint/point/BP_Enemy_Points.BP_Enemy_Points_C" (`KismetMathLibrary.MakeTransform` (+ (* _index (20.0 20.0 0.0)) (`self.K2_GetActorLocation`)) (struct) (0.1 0.1 0.1)) "Undefined" "OverrideRootScale" null null))
    (`self.K2_DestroyActor`)))

(event `Set_Defolut_Color`
  (if (not (== (`PrimitiveComponent.GetMaterial` (`self.RockOnMark`) 0) "/Game/Blueprint/Enemy/M_DefolutColor.M_DefolutColor"))
    (`PrimitiveComponent.SetMaterial` (`self.RockOnMark`) 0 "/Game/Blueprint/Enemy/M_DefolutColor.M_DefolutColor")))

(event `Set_RockOn_Color`
  (if (not (and (== (`PrimitiveComponent.GetMaterial` (`self.RockOnMark`) 0) "/Game/Blueprint/Enemy/M_RockOnColor.M_RockOnColor") (not (`self.NowAttackRockOn`))))
    (`PrimitiveComponent.SetMaterial` (`self.RockOnMark`) 0 "/Game/Blueprint/Enemy/M_RockOnColor.M_RockOnColor")))

(event `Set_Attack_RockOn_Color`
  (if (not (== (`PrimitiveComponent.GetMaterial` (`self.RockOnMark`) 0) "/Game/Blueprint/Enemy/M_AttckRockOnColor.M_AttckRockOnColor"))
    (`PrimitiveComponent.SetMaterial` (`self.RockOnMark`) 0 "/Game/Blueprint/Enemy/M_AttckRockOnColor.M_AttckRockOnColor")
    (set `self.NowAttackRockOn` true)))

(event `self.StaticMesh.OnComponentBeginOverlap`
  (params (OverlappedComponent :type "PrimitiveComponent Object Reference") (OtherActor :type "Actor Object Reference") (OtherComp :type "PrimitiveComponent Object Reference") (OtherBodyIndex :type Integer) (bFromSweep :type Boolean) (SweepResult :type "HitResult Structure (by ref)"))
  (`KismetSystemLibrary.PrintString` (`KismetSystemLibrary.GetDisplayName` OtherComp)))

(event `self.puropera1.OnComponentBeginOverlap`
  (params (OverlappedComponent :type "PrimitiveComponent Object Reference") (OtherActor :type "Actor Object Reference") (OtherComp :type "PrimitiveComponent Object Reference") (OtherBodyIndex :type Integer) (bFromSweep :type Boolean) (SweepResult :type "HitResult Structure (by ref)"))
  (`KismetSystemLibrary.PrintString` (`KismetSystemLibrary.GetDisplayName` OtherComp)))

(fn `Attack_Buki`
  (bind _returnvalue (`GameplayStatics.GetPlayerCharacter` 0))
  (bind _returnvalue_2 (`KismetMathLibrary.VSize` (- (`self.K2_GetActorLocation`) (`self.K2_GetActorLocation` _returnvalue))))
  ;[1 1 1] 敵の射程範囲の計算
  (`/Engine/EditorBlueprintResources/StandardMacros.IsValid` _returnvalue
    (:`Is Valid`
      (if (and (<= _returnvalue_2 30000.0) (>= _returnvalue_2 0.0) (`self.BulletFire`))
        (set `self.BulletFire` false)
        (set `self.BulletFire_Count` 3.0)
        (`self.LaunchBall`)
        (else
          (bind _output_get (set `self.BulletFire_Count` (- (`self.BulletFire_Count`) (`GameplayStatics.GetWorldDeltaSeconds`))))
          (if (< _output_get 0.0)
            (set `self.BulletFire` true)))))))

(fn `Get BP_TM_Spline`
  (returns (BP_TM_Spline :type "/Game/Blueprint/Enemy/BP_TM_Spline Object Reference"))
  (bind _outactors (`GameplayStatics.GetAllActorsOfClass` "/Game/Blueprint/Enemy/BP_TM_Spline.BP_TM_Spline_C"))
  (for _array_element _outactors
    (if (== (`/Game/Blueprint/Enemy/BP_TM_Spline.Index` _array_element) (`self.EnemyIndex`))
      (return _array_element))))

(fn `Get_BP_Player`
  (returns (BP_Player :type "/Game/Blueprint/Player/BP_Player Object Reference"))
  (bind _returnvalue (`GameplayStatics.GetActorOfClass` "/Game/Blueprint/Player/BP_Player.BP_Player_C"))
  (return _returnvalue))

(fn `Move_Puropera`
  (bind _output_get (set `self.Puropera_Rotation` (`KismetMathLibrary.ComposeRotators` (`SceneComponent.GetSocketRotation` (`self.puropera`) "None") (struct :`Yaw` 25.0))))
  (`SceneComponent.K2_SetRelativeRotation` (`self.puropera`) _output_get false false))

(fn `Move_Puropera1`
  (bind _output_get (set `self.Puropera1_Rotation` (`KismetMathLibrary.ComposeRotators` (`SceneComponent.GetSocketRotation` (`self.puropera1`) "None") (struct :`Yaw` 25.0))))
  (`SceneComponent.K2_SetRelativeRotation` (`self.puropera1`) _output_get false false))

(fn `Move_Puropera2`
  (bind _output_get (set `self.Puropera2_Rotation` (`KismetMathLibrary.ComposeRotators` (`SceneComponent.GetSocketRotation` (`self.puropera2`) "None") (struct :`Yaw` 25.0))))
  (`SceneComponent.K2_SetRelativeRotation` (`self.puropera2`) _output_get false false))

(fn `Remove_Enemy_Array`
  (switch `int` (`self.Enemy_Kill_Weapon_Num`)
    (:`3`
      (`KismetArrayLibrary.Array_RemoveItem` (`/Game/Blueprint/Player/BP_Player.SMG_Enemy_Pos` (`self.Get_BP_Player`)) (`self.K2_GetActorLocation`))
      (`/Engine/EditorBlueprintResources/StandardMacros.DecrementInt` (`/Game/Blueprint/Player/BP_Player.Set_SMG_Enemy_Array_Num` (`self.Get_BP_Player`))))))

(fn `Set Player to Enemy Dist`
  (returns (`Return Rotation` :type "Rotator Structure"))
  (bind (_returnvalue_roll _returnvalue_pitch _returnvalue_yaw) (`KismetMathLibrary.BreakRotator` (`KismetMathLibrary.ComposeRotators` (`KismetMathLibrary.FindLookAtRotation` (`self.K2_GetActorLocation`) (`self.K2_GetActorLocation` (`self.Get_BP_Player`))) (struct :`Yaw` -90.0))))
  (return (`KismetMathLibrary.MakeRotator` _returnvalue_roll _returnvalue_pitch _returnvalue_yaw)))

(fn `UserConstructionScript`)