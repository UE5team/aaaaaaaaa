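; Player bullet actor that flies toward a TargetLocation and deals fixed damage to actors tagged Enemy on overlap, then destroys itself.
; Size, applied at BeginPlay, and speed come from the "PL" row of DT_Bullet_Prameters, despite the getter's Enemy name.
; Tick re-reads the row, offsets without sweep or delta-time scaling, so speed is frame-rate dependent, and prints the movement vector.
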(event `self.ReceiveBeginPlay`
  (`SceneComponent.SetWorldScale3D` (`self.Bullet`) (`.Bullet Size` (`self.Get DT_Enemy_Prameters`))))

(event `self.ReceiveTick`
  (params (DeltaSeconds :type "Float (single-precision)"))
  (bind _returnvalue (* (`self.Get DT_Enemy_Prameters`) (`KismetMathLibrary.Normal` (- (`self.TargetLocation`) (`self.K2_GetActorLocation`)))))
  (`self.K2_AddActorWorldOffset` _returnvalue)
  (`KismetSystemLibrary.PrintString` (`KismetStringLibrary.Conv_VectorToString` _returnvalue)))

(event `self.Bullet.OnComponentBeginOverlap`
  (params (OverlappedComponent :type "PrimitiveComponent Object Reference") (OtherActor :type "Actor Object Reference") (OtherComp :type "PrimitiveComponent Object Reference") (OtherBodyIndex :type Integer) (bFromSweep :type Boolean) (SweepResult :type "HitResult Structure (by ref)"))
  (if (`self.ActorHasTag` OtherActor "Enemy")
    (`GameplayStatics.ApplyDamage` OtherActor 20.0)
    (`self.K2_DestroyActor`)))

(fn `Get DT_Enemy_Prameters`
  (returns (`Bullet Speed` :type "Float (double-precision)") (`Bullet Size` :type "Vector Structure"))
  (bind _returnvalue (`|GetDataTableRow` "/Game/PL/DT_Bullet_Prameters.DT_Bullet_Prameters" "PL")
    (:`then`
      (return (break `/Game/PL/ST_Bullet_Prameters` _returnvalue) (`.BulletSize_5_35D0CE7745E9D238FBE821AE43F18FEB` (break `/Game/PL/ST_Bullet_Prameters` _returnvalue))))))

(fn `UserConstructionScript`)