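; Character Blueprint for weapon selection that applies the chosen weapon through two select-weapon components.
; The SetWeapon event reads the widget index from BP_SelectGameMode, found via GetActorOfClass, and branches on it.
; Index 1 switches Weapon0 and sets its socket on the first component, while index 2 only switches Weapon1 on the second.
; An unconnected GetGMCharacterSelection lookup never runs.
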(event `SetWeapon`
  (bind _bp_selectweapon0component (`self.BP_SelectWeapon0Component`))
  (bind _weapon0 (`self.Weapon0`))
  (bind _returnvalue (`GameplayStatics.GetActorOfClass` "/Game/Blueprint/Select/BP_SelectGameMode.BP_SelectGameMode_C"))
  (bind _widget_index (`/Game/Blueprint/Select/BP_SelectGameMode.Get Widget Index` _returnvalue))
  (switch `int` _widget_index
    (:`1`
      (`/Game/Blueprint/CharacterSelection/Weapon/BP_SelectWeapon0Component.switchingWeapon` _bp_selectweapon0component _weapon0)
      (`/Game/Blueprint/CharacterSelection/Weapon/BP_SelectWeapon0Component.SetWeaponSocket` _bp_selectweapon0component _weapon0))
    (:`2`
      (`/Game/Blueprint/CharacterSelection/Weapon/BP_SelectWeapon1Component.switchingWeapon` (`self.BP_SelectWeapon1Component`) (`self.Weapon1`)))))

(fn `UserConstructionScript`)