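; BP_Thruster is a player thruster actor that plays boost, fly and brake animation montages on its skeletal mesh, forward or reversed.
; Montages are supplied through SetAnimMontage, and each play event runs SetUpMontage to derive mesh, rate and start position.
; If the montage is playing, the event calls SetABPConditionVariable with the direction and montage type.
; That function and the boost effect functions are empty here, and the construction script's validity checks have no effect.
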(event `PlayMontageBoost`
  (params (ReversePlay :type Boolean))
  (bind (_return_montage _return_playrate _return_startingposition _return_animationmeshcomponent) (`/Game/Blueprint/System/FL_MyLibrary.Set Up Montage` (`self.BoostMontage`) ReversePlay (`self.SkeletalMeshComponent`)))
  (`|PlayMontage` _return_animationmeshcomponent _return_montage _return_playrate _return_startingposition
    (:`then`
      (if (`/Game/Blueprint/System/FL_MyLibrary.IsPlayingAnimMontage` (`self.SkeletalMeshComponent`))
        (`self.SetABP ConditionVariable` ReversePlay "NewEnumerator1")))))

(event `PlayMontageFly`
  (params (ReversePlay :type Boolean))
  (bind (_return_montage _return_playrate _return_startingposition _return_animationmeshcomponent) (`/Game/Blueprint/System/FL_MyLibrary.Set Up Montage` (`self.FlyMontage`) ReversePlay (`self.SkeletalMeshComponent`)))
  (`|PlayMontage` _return_animationmeshcomponent _return_montage _return_playrate _return_startingposition
    (:`then`
      (if (`/Game/Blueprint/System/FL_MyLibrary.IsPlayingAnimMontage` (`self.SkeletalMeshComponent`))
        (`self.SetABP ConditionVariable` ReversePlay)))))

(event `PlayMontageBack`
  (params (ReversePlay :type Boolean))
  (bind (_return_montage _return_playrate _return_startingposition _return_animationmeshcomponent) (`/Game/Blueprint/System/FL_MyLibrary.Set Up Montage` (`self.BrakeMontage`) ReversePlay (`self.SkeletalMeshComponent`)))
  (`|PlayMontage` _return_animationmeshcomponent _return_montage _return_playrate _return_startingposition
    (:`then`
      (if (`/Game/Blueprint/System/FL_MyLibrary.IsPlayingAnimMontage` (`self.SkeletalMeshComponent`))
        (`self.SetABP ConditionVariable` ReversePlay "NewEnumerator2")))))

(fn `Reset Boost Effect`)

(fn `Set Boost Effect`)

(fn `SetABP ConditionVariable`
  (params (ReversePlay :type Boolean) (NextMontage :type "/Game/Animation/Montage/Armors/E_MontageState Enum" :default "NewEnumerator0")))

(fn `SetAnimMontage`
  (params (BoostMontage :type "AnimMontage Object Reference") (FlyMontage :type "AnimMontage Object Reference") (BackMontage :type "AnimMontage Object Reference"))
  (`|ExecutionSequence`
    (:`then_0`
      (set `self.BoostMontage` BoostMontage))
    (:`then_1`
      (set `self.FlyMontage` FlyMontage))
    (:`then_2`
      (set `self.BrakeMontage` BackMontage))))

(fn `UserConstructionScript`
  (`/Engine/EditorBlueprintResources/StandardMacros.IsValid` (`self.BoostMontage`)
    (:`Is Valid`
      (`/Engine/EditorBlueprintResources/StandardMacros.IsValid` (`self.BoostMontage`)
        (:`Is Valid`
          (`/Engine/EditorBlueprintResources/StandardMacros.IsValid` (`self.BoostMontage`)))))))