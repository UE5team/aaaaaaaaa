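; Player drift component that adds sharper turning and recharges the boost gauge while drifting.
; Holding IA_Drift locks the direction from initial side input, then adds yaw from the gap between drift and normal max rotation.
; Releasing the button or that direction ends the drift.
; Tick refills BP_Player's boost amount while drifting, not boosting and below max, with a charge sound gated by DoOnce.
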(event `self.ReceiveBeginPlay`
  (bind _bp_player (`self.BP Player`))
  (bind _asbp_player (cast `/Game/Blueprint/Player/BP_Player` (`self.GetOwner`)))
  (set `self.BP Player` _asbp_player)
  (`KismetSystemLibrary.Delay` 0.1)
  (set `self.AddRotate` (- (`/Game/Blueprint/Player/BP_Player.Const Max Drift Rotate` _bp_player) (`/Game/Blueprint/Player/BP_Player.ConstMaxRotate` _bp_player))))

(event `self.ReceiveTick`
  (params (DeltaSeconds :type "Float (single-precision)"))
  (bind _bp_player (`self.BP Player`))
  (bind _bp_player_2 (`self.BP Player`))
  ;[1 1 1] ブーストゲージの変数に足すようにする
  (if (and (not (`/Game/Blueprint/Player/AC_Boost.IsBoost` (`/Game/Blueprint/Player/BP_Player.AC_Boost` (`self.BP Player`)))) (`self.IsDrift`) (< (`/Game/Blueprint/Player/BP_Player.Boost amount` _bp_player_2) (`/Game/Blueprint/Player/BP_Player.Const Max Boost amount` _bp_player_2)))
    (`|ExecutionSequence`
      (:`then_0`
        (`/Engine/EditorBlueprintResources/StandardMacros.DoOnce` false :!label _label
          (:`Completed`
            (`self.CreateDriftSound`)
            (`self.PlayDriftSound`))))
      (:`then_1`
        (set `self.Stop Sound` true)
        (set `/Game/Blueprint/Player/BP_Player.Boost amount` (+ (`/Game/Blueprint/Player/BP_Player.Boost amount` _bp_player) (`/Game/Blueprint/Player/BP_Player.Const Recover Boost amount` _bp_player)) _bp_player)))
    (elif (`self.Stop Sound`)
      (`self.StopDriftSound`)
      (set `self.Stop Sound` false)
      (goto _label :!via `Reset`))))

(event `EnhancedInput|/Game/Input/Player/IA_Drift`
  (params (ActionValue :type Boolean) (ElapsedSeconds :type "Float (double-precision)") (TriggeredSeconds :type "Float (double-precision)") (InputAction :type "InputAction Object Reference" :default "/Game/Input/Player/IA_Drift.IA_Drift"))
  (:`Triggered`
    (`|ExecutionSequence`
      (:`then_0`
        (`/Engine/EditorBlueprintResources/StandardMacros.DoOnce` false :!label _label_2
          (:`Completed`
            (if (< (`self.UnderDeadZone`) (`/Game/Blueprint/Player/BP_Player.SideMoveValueX` (`self.BP Player`)))
              (set `self.IsPlayerVecRight` true)
              (set `self.IsDrift` true :!label _label_3)
              (elif (< (`/Game/Blueprint/Player/BP_Player.SideMoveValueX` (`self.BP Player`)) (* (`self.UnderDeadZone`) -1.0))
                (set `self.IsPlayerVecLeft` true)
                (goto _label_3))))))
      (:`then_1`
        (if (`self.IsDrift`)
          (if (`self.IsPlayerVecRight`)
            (if (< (`self.UnderDeadZone`) (`/Game/Blueprint/Player/BP_Player.SideMoveValueX` (`self.BP Player`)))
              (`Actor.K2_AddActorLocalRotation` (`self.BP Player`) (`KismetMathLibrary.MakeRotator` 0.0 0.0 (`self.AddRotate`)) true false)
              (else
                (set `self.IsDrift` false)
                (set `self.IsPlayerVecRight` false)))
            (elif (`self.IsPlayerVecLeft`)
              (if (< (`/Game/Blueprint/Player/BP_Player.SideMoveValueX` (`self.BP Player`)) (* (`self.UnderDeadZone`) -1.0))
                (`Actor.K2_AddActorLocalRotation` (`self.BP Player`) (`KismetMathLibrary.MakeRotator` 0.0 0.0 (* (`self.AddRotate`) -1.0)) true false)
                (else
                  (set `self.IsDrift` false)
                  (set `self.IsPlayerVecLeft` false)))))))))
  (:`Completed`
    (set `self.IsDrift` false)
    (set `self.IsPlayerVecRight` false)
    (set `self.IsPlayerVecLeft` false)
    (goto _label_2 :!via `Reset`)))

(fn `CreateDriftSound`
  (bind _returnvalue (`GameplayStatics.CreateSound2D` "/Game/Sound/aihara/ブーストゲージチャージ音_Cue.ブーストゲージチャージ音_Cue" 1.0 1.0 0.0 null))
  (set `self.DriftSound` _returnvalue))

(fn `PlayDriftSound`
  (`AudioComponent.Play` (`self.DriftSound`) 0.0))

(fn `StopDriftSound`
  (`AudioComponent.Stop` (`self.DriftSound`)))