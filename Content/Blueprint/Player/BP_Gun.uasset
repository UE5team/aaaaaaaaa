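; BP_Gun is a gun actor that fires bursts of BP_BUllet projectiles toward a supplied target location.
; The construction script fills the remaining bullet count from the "PL" row of DT_Bullet_Prameters.
; Fire loops over the burst count, spawning bullets at the Arrow's transform and decrementing ammo, though its empty-ammo check does nothing.
; A helper returns the first BP_Player found; the event graph has no active logic.
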(fn `Fire`
  (params (TargetLocation :type "Vector Structure"))
  (bind _remainingbulletnum (`self.RemainingBulletNum`))
  (for _ (range (+ (`self.5 point Burst`) 1))
    (`|SpawnActorFromClass` "/Game/Blueprint/Player/BP_BUllet.BP_BUllet_C" (`SceneComponent.K2_GetComponentToWorld` (`self.Arrow`)) "Undefined" "MultiplyWithRoot" null TargetLocation null)
    (`/Engine/EditorBlueprintResources/StandardMacros.DecrementInt` _remainingbulletnum
      (:`  `
        (if (<= _remainingbulletnum 0)
          _)))))

(fn `Get BP_Player`
  (returns (BP_Player :type "/Game/Blueprint/Player/BP_Player Object Reference"))
  (bind _outactors (`GameplayStatics.GetAllActorsOfClass` "/Game/Blueprint/Player/BP_Player.BP_Player_C"))
  (return (`|GetArrayItem` _outactors)))

(fn `Get DT_Bullet_Prameters`
  (returns (`Bullet Speed` :type "Float (double-precision)") (`Bullet Size` :type "Vector Structure") (`Max Bullet Num` :type Integer))
  (bind _returnvalue (`|GetDataTableRow` "/Game/PL/DT_Bullet_Prameters.DT_Bullet_Prameters" "PL")
    (:`then`
      (return (break `/Game/PL/ST_Bullet_Prameters` _returnvalue) (`.BulletSize_5_35D0CE7745E9D238FBE821AE43F18FEB` (break `/Game/PL/ST_Bullet_Prameters` _returnvalue)) (`.MaxBulletNum_9_6DB1A31D448BFFD4FD7B43B3D4D55D2F` (break `/Game/PL/ST_Bullet_Prameters` _returnvalue))))))

(fn `UserConstructionScript`
  (set `self.RemainingBulletNum` (`.Max Bullet Num` (`self.Get DT_Bullet_Prameters`))))