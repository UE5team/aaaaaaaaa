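; Actor component for BP_Player that highlights BP_NEO_Enemy actors as lock-on candidates.
; Every Tick it scans all enemies through a DoOnce it immediately resets, setting lock-on or default color by distance and controller-facing dot product.
; The dot product is compared against ±60 as if degrees, so only distance effectively filters.
; An unconnected screen-bounds visibility test with debug prints never runs.
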(event `self.ReceiveBeginPlay`
  (bind _asbp_player (cast `/Game/Blueprint/Player/BP_Player` (`self.GetOwner`)))
  (set `self.BP Player` _asbp_player))

(event `self.ReceiveTick`
  (params (DeltaSeconds :type "Float (single-precision)"))
  (`self.CheckEnemyDistance`))

(event `CheckEnemyDistance`
  (bind _returnvalue (`GameplayStatics.GetPlayerController` 0))
  (`/Engine/EditorBlueprintResources/StandardMacros.DoOnce` false :!label _label
    (:`Completed`
      (bind _outactors (`GameplayStatics.GetAllActorsOfClass` "/Game/Blueprint/Enemy/BP_NEO_Enemy.BP_NEO_Enemy_C"))
      (for (_array_element _array_index) _outactors
        (bind _returnvalue_2 (`KismetMathLibrary.Dot_VectorVector` (`SceneComponent.GetForwardVector` (`Actor.RootComponent` _returnvalue)) (`KismetMathLibrary.GetForwardVector` (`KismetMathLibrary.FindLookAtRotation` (`Actor.K2_GetActorLocation` _returnvalue) (`Actor.K2_GetActorLocation` _array_element)))))
        (if (and (< (`KismetMathLibrary.Abs` (`Actor.GetDistanceTo` (`self.BP Player`) (`|GetArrayItem` _outactors _array_index))) 50000.0) (>= _returnvalue_2 -60.0) (< _returnvalue_2 60.0))
          (bind _output (`|GetArrayItem` _outactors _array_index))
          (`/Game/Blueprint/Enemy/BP_NEO_Enemy.Set_RockOn_Color` _output)
          (else
            (`/Game/Blueprint/Enemy/BP_NEO_Enemy.Set_Defolut_Color` _output))))
      (`self.Reset`))))

(event `Reset`
  (goto _label :!via `Reset`))