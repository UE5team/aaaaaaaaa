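; Player component that handles braking and reversing through the IA_BackMove input.
; While held, it swaps the character's braking friction and max walk speed, restoring defaults on release and exposing the brake state.
; A velocity-versus-forward dot product lets backward movement input apply only when the player is not moving forward.
; Older brake logic and the only call to the off-course (dirt) speed interpolation sit in disconnected nodes.
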(event `self.ReceiveBeginPlay`
  (bind _asbp_player (cast `/Game/Blueprint/Player/BP_Player` (`self.GetOwner`)))
  (set `self.BP Player` _asbp_player))

(event `EnhancedInput|/Game/Input/Player/IA_BackMove`
  (params (ActionValue :type "Float (double-precision)") (ElapsedSeconds :type "Float (double-precision)") (TriggeredSeconds :type "Float (double-precision)") (InputAction :type "InputAction Object Reference" :default "/Game/Input/Player/IA_BackMove.IA_BackMove"))
  (bind _bp_player (`self.BP Player`))
  (bind _bp_player_2 (`self.BP Player`))
  (bind (_returnvalue_roll _returnvalue_pitch _returnvalue_yaw) (`KismetMathLibrary.BreakRotator` (`Actor.K2_GetActorRotation` _bp_player)))
  (bind _charactermovement (`Character.CharacterMovement` _bp_player_2))
  (:`Triggered`
    (if (not (`self.getNowMoveState`))
      (`Pawn.AddMovementInput` _bp_player (`KismetMathLibrary.GetForwardVector` (`KismetMathLibrary.MakeRotator` 0.0 0.0 _returnvalue_yaw)) (* ActionValue -1.0) false)))
  (:`Started`
    (set `self._is_input_brake` true)
    (set `CharacterMovementComponent.BrakingFriction` (`self.Brake time Braking Friction`) _charactermovement)
    (set `CharacterMovementComponent.MaxWalkSpeed` 3000.0 _charactermovement))
  (:`Completed`
    (set `self._is_input_brake` false)
    (set `CharacterMovementComponent.BrakingFriction` (`self.Default Player Braking Friction`) _charactermovement)
    (set `CharacterMovementComponent.MaxWalkSpeed` (`/Game/Blueprint/Player/BP_Player.DefaultMax Walk Speed` _bp_player_2) _charactermovement)))

(fn `getIsInputBrake`
  (returns (`return value` :type Boolean))
  (return (`self._is_input_brake`)))

(fn `getNowMoveState`
  (returns (value :type Boolean))
  (bind _bp_player (`self.BP Player`))
  (return (> (`KismetMathLibrary.Dot_VectorVector` (`KismetMathLibrary.Normal` (`MovementComponent.Velocity` (`Character.CharacterMovement` _bp_player))) (`SceneComponent.GetForwardVector` (`Actor.RootComponent` _bp_player))) 0.0)))

(fn `SetCourceOutWalkSpeed`
  (bind (`_st_ingameparameters_ダート最高速度` `_st_ingameparameters_ダート速度減少スピード`) (break `/Game/PL/ST_InGameParameters` (make `/Game/PL/ST_InGameParameters` 5000.0)))
  (bind _bp_player (`self.BP Player`)
    (:`then`
      (`/Engine/EditorBlueprintResources/StandardMacros.IsValid` _bp_player
        (:`Is Valid`
          (set `CharacterMovementComponent.MaxWalkSpeed` (`KismetMathLibrary.FInterpTo` (`CharacterMovementComponent.MaxWalkSpeed` (`Character.CharacterMovement` (`self.BP Player`))) `_st_ingameparameters_ダート最高速度` (`GameplayStatics.GetWorldDeltaSeconds`) `_st_ingameparameters_ダート速度減少スピード`) (`Character.CharacterMovement` _bp_player)))))
    (:`else`)))