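; BP_ResultPlayer is a player mech, apparently for the result screen, with armor and two weapons chosen in the game instance.
; BeginPlay attaches armor components and equipped minigun, missiles, sniper or SMG to mesh sockets.
; IA_WeaponFire routes press, hold and release to the slot selected by ChangeWeapon.
; Range overlaps store enemy positions per weapon, and bullet hits trigger timed invincibility; movement and status setup are left unwired.
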(event `self.ReceiveBeginPlay`
  (`|ExecutionSequence`
    (:`then_0`
      (`self.Set_GI_Defult`))
    (:`then_1`
      (`self.Set_Player_Gaisou`)
      (`self.Set_Weapon1`)
      (`self.Set_Weapon2`))))

(event `resetCameraRotation`
  (bind _camera (`self.Camera`))
  (bind _returnvalue (`SceneComponent.GetRelativeTransform` (`self.Camera`)))
  (if (> (.roll (.rotation _returnvalue)) 0.0)
    (`SceneComponent.K2_SetRelativeRotation` _camera (`KismetMathLibrary.MakeRotator` (+ (.roll (.rotation _returnvalue)) (* (`self.addCameraRotation`) -1.0))) true false :!label _label)
    (`KismetSystemLibrary.Delay` 0.01)
    (if (> (.roll (.rotation _returnvalue)) 0.0)
      (goto _label))
    (else
      ;[1 1 1] カメラの回転制御
      (`SceneComponent.K2_SetRelativeRotation` _camera (`KismetMathLibrary.MakeRotator` (+ (.roll (.rotation _returnvalue)) (`self.addCameraRotation`))) true false :!label _label_2)
      (`KismetSystemLibrary.Delay` 0.01)
      (if (< (.roll (.rotation _returnvalue)) 0.0)
        (goto _label_2)))))

(event `Invincible`
  ;[1 1 1] 無敵時間に入れて3秒後終了
  (set `self.IsHitCoolTime` true)
  (`KismetSystemLibrary.Delay` (`self.HitCoolTime`))
  (set `self.IsHitCoolTime` false))

(event `self.CapsuleComponent.OnComponentBeginOverlap`
  (params (OverlappedComponent :type "PrimitiveComponent Object Reference") (OtherActor :type "Actor Object Reference") (OtherComp :type "PrimitiveComponent Object Reference") (OtherBodyIndex :type Integer) (bFromSweep :type Boolean) (SweepResult :type "HitResult Structure (by ref)"))
  ;[1 1 1] 無敵時間に入っているかを確認
  (if (not (`self.IsHitCoolTime`))
    (bind _asbp_enemy_bullet (cast `/Game/Blueprint/Enemy/BP_Enemy_Bullet` OtherActor))
    (`/Game/Blueprint/Enemy/BP_Enemy_Bullet.Player Damage` _asbp_enemy_bullet)
    (`self.Invincible`)))

(event `RepairingInvincible`
  ;[1 1 1] リペア明けの無敵時間十秒後に終了
  (set `self.IsHitCoolTime` true)
  (`KismetSystemLibrary.Delay` (`self.RepairingCoolTime`))
  (set `self.IsHitCoolTime` false))

(event `self.SMG_Range.OnComponentBeginOverlap`
  (params (OverlappedComponent :type "PrimitiveComponent Object Reference") (OtherActor :type "Actor Object Reference") (OtherComp :type "PrimitiveComponent Object Reference") (OtherBodyIndex :type Integer) (bFromSweep :type Boolean) (SweepResult :type "HitResult Structure (by ref)"))
  (`self.Set_SMG_Enemy_Array` OtherActor))

(event `self.Missile_Range.OnComponentBeginOverlap`
  (params (OverlappedComponent :type "PrimitiveComponent Object Reference") (OtherActor :type "Actor Object Reference") (OtherComp :type "PrimitiveComponent Object Reference") (OtherBodyIndex :type Integer) (bFromSweep :type Boolean) (SweepResult :type "HitResult Structure (by ref)"))
  ;[1 1 1] コリジョンにあった敵の座標を配列に代入するところ
  (`self.Set_Missile_Enemy_Array` OtherActor))

(event `self.SMG_Range.OnComponentEndOverlap`
  (params (OverlappedComponent :type "PrimitiveComponent Object Reference") (OtherActor :type "Actor Object Reference") (OtherComp :type "PrimitiveComponent Object Reference") (OtherBodyIndex :type Integer))
  (`self.Remove_SMG_Enemy_Array` OtherActor))

(event `self.Missile_Range.OnComponentEndOverlap`
  (params (OverlappedComponent :type "PrimitiveComponent Object Reference") (OtherActor :type "Actor Object Reference") (OtherComp :type "PrimitiveComponent Object Reference") (OtherBodyIndex :type Integer))
  (`self.Remove_Missile_Enemy_Array` OtherActor))

(event `self.SR_Range.OnComponentBeginOverlap`
  (params (OverlappedComponent :type "PrimitiveComponent Object Reference") (OtherActor :type "Actor Object Reference") (OtherComp :type "PrimitiveComponent Object Reference") (OtherBodyIndex :type Integer) (bFromSweep :type Boolean) (SweepResult :type "HitResult Structure (by ref)"))
  (`self.Set_SR_Enemy_Array` OtherActor))

(event `self.SR_Range.OnComponentEndOverlap`
  (params (OverlappedComponent :type "PrimitiveComponent Object Reference") (OtherActor :type "Actor Object Reference") (OtherComp :type "PrimitiveComponent Object Reference") (OtherBodyIndex :type Integer))
  (`self.Remove_SR_Enemy_Array` OtherActor))

(event `EnhancedInput|/Game/Input/Player/IA_WeaponFire`
  (params (ActionValue :type "Vector2D Structure") (ElapsedSeconds :type "Float (double-precision)") (TriggeredSeconds :type "Float (double-precision)") (InputAction :type "InputAction Object Reference" :default "/Game/Input/Player/IA_WeaponFire.IA_WeaponFire"))
  (:`Triggered`
    (if (`self.Change_Weapon`)
      (`self.Fire_Trigger_Weapon1`)
      (else
        (`self.Fire_Trigger_Weapon2`))))
  (:`Started`
    (if (`self.Change_Weapon`)
      (`self.Fire_Started_Weapon1`)
      (else
        (`self.Fire_Started_Weapon2`)))
    (`|PlayMontage` (`self.Mesh`) "/Game/NewPlayer/Mon_Minigun.Mon_Minigun"))
  (:`Completed`
    (if (`self.Change_Weapon`)
      (`self.Fire_End_Weapon1`)
      (else
        (`self.Fire_End_Weapon2`)))))

(fn `DestroyRepairingParticle`
  (`ActorComponent.K2_DestroyComponent` (`self.ReparingParticle`)))

(fn `Fire_End_Weapon1`
  (switch `int` (`|GetArrayItem` (`/Game/Blueprint/Maps/GI_Defolut.Equip Focus Index Array` (`self.GI_Defolut`)))
    (:`0`
      (`/Game/Blueprint/Weapon/NEO_MineGun2.Fire_End_MineGun` (`self.NEO_MineGun`)))
    (:`1`
      _)
    (:`2`
      _)
    (:`3`
      (`/Game/Blueprint/Weapon/SMC_SMG.FireEnd_SMG` (`self.SMG`))))
  (return))

(fn `Fire_End_Weapon2`
  (switch `int` (`|GetArrayItem` (`/Game/Blueprint/Maps/GI_Defolut.Equip Focus Index Array` (`self.GI_Defolut`)))
    (:`0`
      (`/Game/Blueprint/Weapon/NEO_MineGun2.Fire_End_MineGun` (`self.NEO_MineGun`)))
    (:`1`
      _)
    (:`2`
      _)
    (:`3`
      (`/Game/Blueprint/Weapon/SMC_SMG.FireEnd_SMG` (`self.SMG`))))
  (return))

(fn `Fire_Started_Weapon1`
  (switch `int` (`|GetArrayItem` (`/Game/Blueprint/Maps/GI_Defolut.Equip Focus Index Array` (`self.GI_Defolut`)))
    (:`0`
      _)
    (:`1`
      (`/Game/Blueprint/Weapon/NEO_Missile_R2.Fire Started Missile` (`self.NEO_Missile_R`)))
    (:`2`
      (`/Game/Blueprint/Weapon/SMC_SR.Fire_Started_SR` (`self.SR`)))
    (:`3`
      _))
  (return))

(fn `Fire_Started_Weapon2`
  (switch `int` (`|GetArrayItem` (`/Game/Blueprint/Maps/GI_Defolut.Equip Focus Index Array` (`self.GI_Defolut`)) 1)
    (:`0`
      _)
    (:`1`
      (`/Game/Blueprint/Weapon/NEO_Missile_R2.Fire Started Missile` (`self.NEO_Missile_R`)))
    (:`2`
      (`/Game/Blueprint/Weapon/SMC_SR.Fire_Started_SR` (`self.SR`)))
    (:`3`
      _))
  (return))

(fn `Fire_Trigger_Weapon1`
  (switch `int` (`|GetArrayItem` (`/Game/Blueprint/Maps/GI_Defolut.Equip Focus Index Array` (`self.GI_Defolut`)))
    (:`0`
      (`/Game/Blueprint/Weapon/NEO_MineGun2.Fire_Trigger_MineGun` (`self.NEO_MineGun`)))
    (:`1`
      _)
    (:`2`
      _)
    (:`3`
      (`/Game/Blueprint/Weapon/SMC_SMG.Fire_SMG` (`self.SMG`))))
  (return))

(fn `Fire_Trigger_Weapon2`
  (switch `int` (`|GetArrayItem` (`/Game/Blueprint/Maps/GI_Defolut.Equip Focus Index Array` (`self.GI_Defolut`)) 1)
    (:`0`
      (`/Game/Blueprint/Weapon/NEO_MineGun2.Fire_Trigger_MineGun` (`self.NEO_MineGun`)))
    (:`1`
      _)
    (:`2`
      _)
    (:`3`
      (`/Game/Blueprint/Weapon/SMC_SMG.Fire_SMG` (`self.SMG`))))
  (return))

(fn `Missile Exist2の初期化`
  (set `self.Missile2_exist` true))

(fn `Missile Exist3の初期化`
  (set `self.Missile3_exist` true))

(fn `Missile Exist４の初期化`
  (set `self.Missile4_exist` true))

(fn `Missile_Exist１の初期化`
  (set `self.Missile1_exist` true))

(fn `Remove_Missile_Enemy_Array`
  (params (`Other Actor` :type "Actor Object Reference"))
  (if (`self.ActorHasTag` `Other Actor` "Enemy")
    (bind _asbp_neo_enemy (cast `/Game/Blueprint/Enemy/BP_NEO_Enemy` `Other Actor`))
    (`KismetArrayLibrary.Array_RemoveItem` (`self.Enemy_Position`) (`self.K2_GetActorLocation` _asbp_neo_enemy))
    (bind _result (`/Engine/EditorBlueprintResources/StandardMacros.DecrementInt` (`self.SetEnemy Missile Index`)))))

(fn `Remove_SMG_Enemy_Array`
  (params (`Other Actor` :type "Actor Object Reference"))
  (if (`self.ActorHasTag` `Other Actor` "Enemy")
    (bind _asbp_neo_enemy (cast `/Game/Blueprint/Enemy/BP_NEO_Enemy` `Other Actor`))
    (`KismetArrayLibrary.Array_RemoveItem` (`self.SR_Enemy_pos`) (`self.K2_GetActorLocation` _asbp_neo_enemy))))

(fn `Remove_SR_Enemy_Array`
  (params (`Other Actor` :type "Actor Object Reference"))
  (if (`self.ActorHasTag` `Other Actor` "Enemy")
    (bind _asbp_neo_enemy (cast `/Game/Blueprint/Enemy/BP_NEO_Enemy` `Other Actor`))
    (`KismetArrayLibrary.Array_RemoveItem` (`self.SR_Enemy_pos`) (`self.K2_GetActorLocation` _asbp_neo_enemy))))

(fn `Set_GI_Defult`
  (bind _gi_default (`/Game/Blueprint/System/FL_MyLibrary.Get GI_Default`))
  (set `self.GI_Defolut` _gi_default))

(fn `Set_Missile_Enemy_Array`
  (params (`Other Actor` :type "Actor Object Reference"))
  (bind _enemy_position (`self.Enemy_Position`))
  (if (`self.ActorHasTag` `Other Actor` "Enemy")
    (bind _asbp_neo_enemy (cast `/Game/Blueprint/Enemy/BP_NEO_Enemy` `Other Actor`))
    (bind _result (`/Engine/EditorBlueprintResources/StandardMacros.IncrementInt` (`self.SetEnemy Missile Index`))
      (:`  `
        (`KismetArrayLibrary.Array_Insert` _enemy_position (`self.K2_GetActorLocation` _asbp_neo_enemy))
        (if (>= _result 4)
          (`KismetArrayLibrary.Array_Remove` _enemy_position 4))))))

(fn `Set_Player_Gaisou`
  (bind _mesh (`self.Mesh`))
  (bind _mesh_2 (`self.Mesh`))
  (bind _mesh_3 (`self.Mesh`))
  (bind _mesh_4 (`self.Mesh`))
  (bind _mesh_5 (`self.Mesh`))
  (bind _mesh_6 (`self.Mesh`))
  (bind _mesh_7 (`self.Mesh`))
  (`|ExecutionSequence`
    (:`then_0`
      (bind _returnvalue (`AddComponent|NODE_AddStaticMeshComponent-12`))
      (`SceneComponent.K2_AttachToComponent` _returnvalue _mesh_2 "Armar_Back" "KeepRelative" "KeepRelative" "KeepRelative" true)
      (bind _returnvalue_2 (`AddComponent|NODE_AddStaticMeshComponent-13`))
      (`SceneComponent.K2_AttachToComponent` _returnvalue_2 _mesh_2 "Armar" "KeepRelative" "KeepRelative" "KeepRelative" true))
    (:`then_1`
      (bind _returnvalue_3 (`AddComponent|NODE_AddStaticMeshComponent-45`))
      (`SceneComponent.K2_AttachToComponent` _returnvalue_3 _mesh_4 "Armar_L" "KeepRelative" "KeepRelative" "KeepRelative" true)
      (bind _returnvalue_4 (`AddComponent|NODE_AddStaticMeshComponent-16`))
      (`SceneComponent.K2_AttachToComponent` _returnvalue_4 _mesh_4 "Armar_L_Thruster" "KeepRelative" "KeepRelative" "KeepRelative" true)
      (bind _returnvalue_5 (`AddComponent|NODE_AddStaticMeshComponent-17`))
      (`SceneComponent.K2_AttachToComponent` _returnvalue_5 _mesh_4 "Armar_L_Roket" "KeepRelative" "KeepRelative" "KeepRelative" true))
    (:`then_2`
      (bind _returnvalue_6 (`AddComponent|NODE_AddStaticMeshComponent-27`))
      (`SceneComponent.K2_AttachToComponent` _returnvalue_6 _mesh "Armar_R" "KeepRelative" "KeepRelative" "KeepRelative" true)
      (bind _returnvalue_7 (`AddComponent|NODE_AddStaticMeshComponent-28`))
      (`SceneComponent.K2_AttachToComponent` _returnvalue_7 _mesh "Armar_R_Thruster" "KeepRelative" "KeepRelative" "KeepRelative" true)
      (bind _returnvalue_8 (`AddComponent|NODE_AddStaticMeshComponent-29`))
      (`SceneComponent.K2_AttachToComponent` _returnvalue_8 _mesh "Armar_R_Roket" "KeepRelative" "KeepRelative" "KeepRelative" true))
    (:`then_3`
      (bind _returnvalue_9 (`AddComponent|NODE_AddStaticMeshComponent-21`))
      (`SceneComponent.K2_AttachToComponent` _returnvalue_9 _mesh_6 "Buki01_L_Arm01" "KeepRelative" "KeepRelative" "KeepRelative" true)
      (bind _returnvalue_10 (`AddComponent|NODE_AddStaticMeshComponent-22`))
      (`SceneComponent.K2_AttachToComponent` _returnvalue_10 _mesh_6 "Buki01_L_Arm02" "KeepRelative" "KeepRelative" "KeepRelative" true)
      (bind _returnvalue_11 (`AddComponent|NODE_AddStaticMeshComponent-23`))
      (`SceneComponent.K2_AttachToComponent` _returnvalue_11 _mesh_6 "Buki01_L_Arm_03" "KeepRelative" "KeepRelative" "KeepRelative" true))
    (:`then_4`
      (bind _returnvalue_12 (`AddComponent|NODE_AddStaticMeshComponent-33`))
      (`SceneComponent.K2_AttachToComponent` _returnvalue_12 _mesh_3 "Buki01_R_Arm1" "KeepRelative" "KeepRelative" "KeepRelative" true)
      (bind _returnvalue_13 (`AddComponent|NODE_AddStaticMeshComponent-34`))
      (`SceneComponent.K2_AttachToComponent` _returnvalue_13 _mesh_3 "Buki01_R_Arm02" "KeepRelative" "KeepRelative" "KeepRelative" true)
      (bind _returnvalue_14 (`AddComponent|NODE_AddStaticMeshComponent-35`))
      (`SceneComponent.K2_AttachToComponent` _returnvalue_14 _mesh_3 "Buki01_R_Arm_03" "KeepRelative" "KeepRelative" "KeepRelative" true))
    (:`then_5`
      (bind _returnvalue_15 (`AddComponent|NODE_AddStaticMeshComponent-39`))
      (`SceneComponent.K2_AttachToComponent` _returnvalue_15 _mesh_7 "Buki03_Arm01" "KeepRelative" "KeepRelative" "KeepRelative" true)
      (bind _returnvalue_16 (`AddComponent|NODE_AddStaticMeshComponent-40`))
      (`SceneComponent.K2_AttachToComponent` _returnvalue_16 _mesh_7 "Buki03_Arm02" "KeepRelative" "KeepRelative" "KeepRelative" true))
    (:`then_6`
      (bind _returnvalue_17 (`AddComponent|NODE_AddStaticMeshComponent-43`))
      (`SceneComponent.K2_AttachToComponent` _returnvalue_17 _mesh_5 "Buki04_Arm01" "KeepRelative" "KeepRelative" "KeepRelative" true)
      (bind _returnvalue_18 (`AddComponent|NODE_AddStaticMeshComponent-44`))
      (`SceneComponent.K2_AttachToComponent` _returnvalue_18 _mesh_5 "Buki04_Arm02" "KeepRelative" "KeepRelative" "KeepRelative" true))))

(fn `Set_SMG_Enemy_Array`
  (params (`Other Actor` :type "Actor Object Reference"))
  (if (`self.ActorHasTag` `Other Actor` "Enemy")
    (bind _asbp_neo_enemy (cast `/Game/Blueprint/Enemy/BP_NEO_Enemy` `Other Actor`))
    (bind _result (`/Engine/EditorBlueprintResources/StandardMacros.IncrementInt` (`self.Set_SMG_Enemy_Array_Num`))
      (:`  `
        (`KismetArrayLibrary.Array_Insert` (`self.SMG_Enemy_Pos`) (`self.K2_GetActorLocation` _asbp_neo_enemy) _result)))))

(fn `Set_SR_Enemy_Array`
  (params (`Other Actor` :type "Actor Object Reference"))
  (if (`self.ActorHasTag` `Other Actor` "Enemy")
    (bind _asbp_neo_enemy (cast `/Game/Blueprint/Enemy/BP_NEO_Enemy` `Other Actor`))
    (`/Engine/EditorBlueprintResources/StandardMacros.IncrementInt` (`self.set_enemy_SR_Index`)
      (:`  `
        (`KismetArrayLibrary.Array_Insert` (`self.SR_Enemy_pos`) (`self.K2_GetActorLocation` _asbp_neo_enemy))))))

(fn `Set_Weapon1`
  (switch `int` (`|GetArrayItem` (`/Game/Blueprint/Maps/GI_Defolut.Equip Focus Index Array` (`self.GI_Defolut`)))
    (:`0`
      (bind _returnvalue (`AddComponent|NODE_AddNEO_MineGun2-0`))
      (bind _output_get (set `self.NEO_MineGun` _returnvalue))
      (`SceneComponent.K2_AttachToComponent` _output_get (`self.Mesh`) "Buki02_02" "SnapToTarget" "SnapToTarget" "SnapToTarget" true))
    (:`1`
      (bind _returnvalue_2 (`AddComponent|NODE_AddNEO_Missile_L2-2`))
      (bind _output_get_2 (set `self.NEO_Missile_L` _returnvalue_2))
      (`SceneComponent.K2_AttachToComponent` _output_get_2 (`self.Mesh`) "Missile_Pod_L" "SnapToTarget" "SnapToTarget" "SnapToTarget" true)
      (bind _returnvalue_3 (`AddComponent|NODE_AddNEO_Missile_R2-1`))
      (bind _output_get_3 (set `self.NEO_Missile_R` _returnvalue_3))
      (`SceneComponent.K2_AttachToComponent` _output_get_3 (`self.Mesh`) "Missile_Pod_R" "SnapToTarget" "SnapToTarget" "SnapToTarget" true))
    (:`2`
      (bind _returnvalue_4 (`AddComponent|NODE_AddSMC_SR-2`))
      (bind _output_get_4 (set `self.SR` _returnvalue_4))
      (`SceneComponent.K2_AttachToComponent` _output_get_4 (`self.Mesh`) "BUki04" "SnapToTarget" "SnapToTarget" "SnapToTarget" true))
    (:`3`
      (bind _returnvalue_5 (`AddComponent|NODE_AddSMC_SMG-2`))
      (bind _output_get_5 (set `self.SMG` _returnvalue_5))
      (`SceneComponent.K2_AttachToComponent` _output_get_5 (`self.Mesh`) "Buki03" "SnapToTarget" "SnapToTarget" "SnapToTarget" true))))

(fn `Set_Weapon2`
  (switch `int` (`|GetArrayItem` (`/Game/Blueprint/Maps/GI_Defolut.Equip Focus Index Array` (`self.GI_Defolut`)) 1)
    (:`0`
      (bind _returnvalue (`AddComponent|NODE_AddNEO_MineGun2-1`))
      (bind _output_get (set `self.NEO_MineGun` _returnvalue))
      (`SceneComponent.K2_AttachToComponent` _output_get (`self.Mesh`) "Weapon02" "SnapToTarget" "SnapToTarget" "SnapToTarget" true))
    (:`1`
      (`AddComponent|NODE_AddNEO_Missile_L2-1`))
    (:`2`
      (bind _returnvalue_2 (`AddComponent|NODE_AddSMC_SR-3`))
      (bind _output_get_2 (set `self.SR` _returnvalue_2))
      (`SceneComponent.K2_AttachToComponent` _output_get_2 (`self.Mesh`) "Weapon04" "SnapToTarget" "SnapToTarget" "SnapToTarget" true))
    (:`3`
      (bind _returnvalue_3 (`AddComponent|NODE_AddSMC_SMG-3`))
      (bind _output_get_3 (set `self.SMG` _returnvalue_3))
      (`SceneComponent.K2_AttachToComponent` _output_get_3 (`self.Mesh`) "Weapon03" "SnapToTarget" "SnapToTarget" "SnapToTarget" true))))

(fn `SetRepairingParticle`
  (bind (_returnvalue_location _returnvalue_rotation) (`KismetMathLibrary.BreakTransform` (`SceneComponent.GetRelativeTransform` (`self.CapsuleComponent`))))
  (bind _returnvalue (`AddComponent|NODE_AddParticleSystemComponent-2` :`RelativeTransform` (`KismetMathLibrary.MakeTransform` _returnvalue_location _returnvalue_rotation)))
  (set `self.ReparingParticle` _returnvalue))

(fn `Setup Status`
  (bind _gi_default (`/Game/Blueprint/System/FL_MyLibrary.Get GI_Default`))
  (bind (_speed _acceleration _turbo _weight) (`/Game/Blueprint/Maps/GI_Defolut.GetTotalStatus` _gi_default))
  (set `self.speed` _speed)
  (set `self.acceleration` _acceleration)
  (set `self.turbo` _turbo)
  (set `self.weight` _weight))

(fn `UserConstructionScript`)