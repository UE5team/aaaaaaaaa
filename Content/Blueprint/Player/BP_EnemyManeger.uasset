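; BP_EnemyManeger spawns and clears the game's BP_NEO_Enemy actors.
; SpawnEnemy places one scaled-up enemy at each BP_TM_Spline, writing the same array index to both so they pair up, and increments EnemyCount on the GI_Defolut game instance.
; ResetEnemy destroys every BP_NEO_Enemy in the world but leaves EnemyCount and the spline indices untouched.
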(fn `Get GI_Defolut`
  (returns (`GI Defolut` :type "/Game/Blueprint/Maps/GI_Defolut Object Reference"))
  (bind _asgi_defolut (cast `/Game/Blueprint/Maps/GI_Defolut` (`GameplayStatics.GetGameInstance`)))
  (return _asgi_defolut))

(fn `Reset Enemy`
  (bind _outactors (`GameplayStatics.GetAllActorsOfClass` "/Game/Blueprint/Enemy/BP_NEO_Enemy.BP_NEO_Enemy_C"))
  (for _array_element _outactors
    (`self.K2_DestroyActor` _array_element)))

(fn `Spawn Enemy`
  (bind _outactors (`GameplayStatics.GetAllActorsOfClass` "/Game/Blueprint/Enemy/BP_TM_Spline.BP_TM_Spline_C"))
  (for (_array_element _array_index) _outactors
    (set `/Game/Blueprint/Enemy/BP_TM_Spline.Index` _array_index _array_element)
    (`/Engine/EditorBlueprintResources/StandardMacros.IncrementInt` (`/Game/Blueprint/Maps/GI_Defolut.EnemyCount` (`self.Get GI_Defolut`))
      (:`  `
        (bind _returnvalue_location (`KismetMathLibrary.BreakTransform` (`self.GetTransform` _array_element)))
        (bind _returnvalue (`|SpawnActorFromClass` "/Game/Blueprint/Enemy/BP_NEO_Enemy.BP_NEO_Enemy_C" (`KismetMathLibrary.MakeTransform` _returnvalue_location (struct) (5.0 5.0 5.0)) "Undefined" "OverrideRootScale" null null))
        (set `/Game/Blueprint/Enemy/BP_NEO_Enemy.EnemyIndex` _array_index _returnvalue)))))

(fn `UserConstructionScript`)