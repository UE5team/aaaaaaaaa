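; Player component that runs the racer's boost while the boost input is held.
; Boost starts with enough gauge and the accelerator pressed, raising max speed and turning on boost fire, then drains by an amount derived at BeginPlay from turbo stats.
; On release or empty gauge, it stops the fire and has the invisible floor actor restore walk speed unless off course.
; Tick drives post-process speed lines during boost or high velocity.
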(event `self.ReceiveBeginPlay`
  (bind ((`ターボステータスの１に相当する増加量_54_F997BB6D4A8D0E267ABB99BA33D841F0` `_ターボステータスの１に相当する増加量`) (`ブーストゲージ消費量中央値_66_F75A7DCE42BD31ABD8819C9FA3171928` `_ブーストゲージ消費量中央値`)) (break `/Game/PL/ST_PlayerParameters` (make `/Game/PL/ST_PlayerParameters`)))
  (`self.Get Floor_Invisble`)
  (bind _gi_default (`/Game/Blueprint/System/FL_MyLibrary.Get GI_Default`))
  (set `self.BoostDecreasedValue` (- (+ (* (`/Game/Blueprint/Player/BP_Player.TOTAL_EQUIP_STATUS_CENTER_VALUE` (`self.Get Player`)) `_ターボステータスの１に相当する増加量`) `_ブーストゲージ消費量中央値`) (* `_ターボステータスの１に相当する増加量` (`/Game/Blueprint/Maps/GI_Defolut.GetTotalTurboMagnification` _gi_default)))))

(event `EnhancedInput|/Game/Input/Player/IA_Boost`
  (params (ActionValue :type Boolean) (ElapsedSeconds :type "Float (double-precision)") (TriggeredSeconds :type "Float (double-precision)") (InputAction :type "InputAction Object Reference" :default "/Game/Input/Player/IA_Boost.IA_Boost"))
  (bind _asbp_player (`self.Get Player`))
  (bind _boost_amount (`/Game/Blueprint/Player/BP_Player.Boost amount` _asbp_player))
  (:`Triggered`
    ;[1 1 1] たまっているブーストゲージから決まった値分ブーストゲージから引く
    (if (`self.IsBoost`)
      (if (> _boost_amount 0.0)
        (set `/Game/Blueprint/Player/BP_Player.Boost amount` (- _boost_amount (`self.BoostDecreasedValue`)) _asbp_player)
        (else
          (set `self.IsBoost` false)))
      (else
        (`self.End Boost` :!label _label)
        (`/Game/Blueprint/Player/BP_Player.OffBoustFire` (`self.Get Player`)))))
  (:`Started`
    (if (and (> (`/Game/Blueprint/Player/BP_Player.Boost amount` _asbp_player) 1.0) (`/Game/Blueprint/Player/BP_Player.OnAccelerator` _asbp_player))
      (set `self.IsBoost` true)
      (`self.Set_Boost_Speed`)
      (`/Game/Blueprint/Player/BP_Player.OnBoustFire` (`self.Get Player`))))
  (:`Completed`
    (goto _label)))

(event `self.ReceiveTick`
  (params (DeltaSeconds :type "Float (single-precision)"))
  (if (or (> (`KismetMathLibrary.FTrunc` (`KismetMathLibrary.VSize` (`Actor.GetVelocity` (`self.Get Player`)))) 22000) (`self.IsBoost`))
    (`KismetMaterialLibrary.SetScalarParameterValue` "/Game/Animation/SpeedLine/MPC_PostProcess.MPC_PostProcess" "SpeedLineOpacity" (`self.Parameter Value`))
    (if (>= (`self.Parameter Value`) 1.0)
      (set `self.Parameter Value` 1.0)
      (else
        (set `self.Parameter Value` (`KismetMathLibrary.FInterpTo` (`self.Parameter Value`) 1.0 DeltaSeconds 2.5))))
    (else
      (`KismetMaterialLibrary.SetScalarParameterValue` "/Game/Animation/SpeedLine/MPC_PostProcess.MPC_PostProcess" "SpeedLineOpacity"))))

(fn `End Boost`
  (bind _asbp_player (`self.Get Player`))
  (set `self.IsBoost` false)
  (bind _floorinvisble (`self.FloorInvisble`)
    (:`then`
      (if (not (`/Game/Blueprint/Maps/Floor_invisble_Blueprint.isOffCource` _floorinvisble))
        (`/Game/Blueprint/Maps/Floor_invisble_Blueprint.Set Defult Walk Speed` (`self.FloorInvisble`))
        (set `CharacterMovementComponent.MaxAcceleration` (`/Game/Blueprint/Player/BP_Player.DefaultMaxAcceleration` _asbp_player) (`Character.CharacterMovement` _asbp_player))
        (`KismetMaterialLibrary.SetScalarParameterValue` "/Game/Animation/SpeedLine/MPC_PostProcess.MPC_PostProcess" "SpeedLineOpacity")))
    (:`else`)))

(fn `Get Floor_Invisble`
  (bind _returnvalue (`GameplayStatics.GetActorOfClass` "/Game/Blueprint/Maps/Floor_invisble_Blueprint.Floor_invisble_Blueprint_C"))
  (set `self.FloorInvisble` _returnvalue))

(fn `Get Player`
  (returns (`AsBP Player` :type "/Game/Blueprint/Player/BP_Player Object Reference"))
  (return (cast `/Game/Blueprint/Player/BP_Player` (`self.GetOwner`) :!pure true)))

(fn `Get WB HP and Boost`
  (returns (`WBP HPAnd Boost` :type "/Game/Blueprint/Maps/WBP_HPAndBoost Object Reference"))
  (bind _foundwidgets (`WidgetBlueprintLibrary.GetAllWidgetsOfClass` "/Game/Blueprint/Maps/BP_Ingame_UI.BP_Ingame_UI_C"))
  (return (`/Game/Blueprint/Maps/BP_Ingame_UI.WBP_HPAndBoost_0` (`|GetArrayItem` _foundwidgets))))

(fn `Set_Boost_Speed`
  (bind _asbp_player (`self.Get Player`))
  (bind _charactermovement (`Character.CharacterMovement` _asbp_player))
  (set `CharacterMovementComponent.MaxWalkSpeed` (`/Game/Blueprint/Player/BP_Player.ConstMaxBoostSpeed` _asbp_player) _charactermovement)
  (set `CharacterMovementComponent.MaxAcceleration` (`/Game/Blueprint/Player/BP_Player.DefaultMaxAcceleration` _asbp_player) _charactermovement))