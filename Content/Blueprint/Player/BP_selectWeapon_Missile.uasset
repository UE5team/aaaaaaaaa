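; Missile weapon mesh component for the character in weapon selection, showing missile models on that character's mesh.
; SetMissile casts the owner to BP_SelectWeaponCharacter and snaps the component to its CharactorMesh at the socket indexed from WeaponSocket.
; SwitchingWeapon swaps the static mesh from WeaponArray by index, and DetachMissile detaches the component.
; BeginPlay and Tick are unused.
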(fn `Detach_Missile`
  (`self.K2_DetachFromComponent` "KeepRelative"))

(fn `Set_Missile`
  (params (Weapon_Index :type Integer))
  (bind _asbp_select_weapon_character (cast `/Game/Blueprint/Player/BP_SelectWeaponCharacter` (`self.GetOwner`)))
  (`self.K2_AttachToComponent` (`/Game/Blueprint/Player/BP_SelectWeaponCharacter.CharactorMesh` _asbp_select_weapon_character) (`|GetArrayItem` (`self.Weapon_Socket`) Weapon_Index) "SnapToTarget" "SnapToTarget" "SnapToTarget"))

(fn `switchingWeapon`
  (params (WeaponNum :type Integer))
  (`self.SetStaticMesh` (`|GetArrayItem` (`self.WeaponArray`) WeaponNum)))