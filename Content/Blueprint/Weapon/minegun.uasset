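; Player minegun weapon that attaches to the character's "weapon3" socket and fires bursts of BP_Player_Minegun actors from its "fire" socket.
; Held input spawns shots after a short Delay until a shot cap or release stops the sound and starts a cooldown.
; Tick counts the cooldown down directly in the WB_CT widget.
; DoOnce gates limit the timer refill, firing sound and GI_Defolut weapon-point award to once per cycle.
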(event `self.ReceiveBeginPlay`
  (bind _asbp_player (cast `/Game/Blueprint/Player/BP_Player` (`self.GetOwner`)))
  (bind _output_get (set `self.First Person Character` _asbp_player))
  (`self.K2_AttachToComponent` (`Character.Mesh` _output_get) "weapon3" "KeepRelative" "KeepRelative" "KeepRelative"))

(event `self.ReceiveTick`
  (params (DeltaSeconds :type "Float (single-precision)"))
  (if (`self.MineGun_CT_Bool`)
    (`|ExecutionSequence`
      (:`then_0`
        (goto _label :!via `Reset`))
      (:`then_1`
        (bind _newparam (`self.GetWB_CT`))
        (bind _output_get (set `/Game/Blueprint/Player/WB_CT.MineGun_CT2` (- (`/Game/Blueprint/Player/WB_CT.MineGun_CT2` _newparam) (`GameplayStatics.GetWorldDeltaSeconds`)) _newparam))
        (if (< _output_get 0.0)
          (set `self.MineGun_CT_bool` false)
          (goto _label_2 :!via `Reset`))))
    (else
      (`/Engine/EditorBlueprintResources/StandardMacros.DoOnce` false :!label _label
        (:`Completed`
          (bind _newparam_2 (`self.GetWB_CT`))
          (bind _output_get_2 (set `/Game/Blueprint/Player/WB_CT.MineGun_CT2` (`self.MineGun_CT`) _newparam_2))
          (`KismetSystemLibrary.PrintString` (`KismetStringLibrary.Concat_StrStr` (`KismetStringLibrary.Conv_DoubleToString` _output_get_2) "秒")))))))

(event `EnhancedInput|/Game/Input/Player/IA_MineGun`
  (params (ActionValue :type Boolean) (ElapsedSeconds :type "Float (double-precision)") (TriggeredSeconds :type "Float (double-precision)") (InputAction :type "InputAction Object Reference" :default "/Game/Input/Player/IA_MineGun.IA_MineGun"))
  (:`Triggered`
    (set `self.Mine_Gun_Fire` true)
    (if (`self.Mine_Gun_Fire`)
      (if (not (`self.MineGun_CT_Bool`))
        (`|ExecutionSequence`
          (:`then_0`
            (`/Engine/EditorBlueprintResources/StandardMacros.DoOnce` false :!label _label_2
              (:`Completed`
                (bind _asgi_defolut (cast `/Game/Blueprint/Maps/GI_Defolut` (`GameplayStatics.GetGameInstance`)))
                (set `/Game/Blueprint/Maps/GI_Defolut.WeaponPoints` (+ (`/Game/Blueprint/Maps/GI_Defolut.WeaponPoints` _asgi_defolut) (`self.Weapon Point`)) _asgi_defolut)
                (bind _returnvalue (`GameplayStatics.CreateSound2D` "/Game/Sound/Weapon/MineGun/MineGun_Sound.MineGun_Sound" 1.5 1.0 0.0 null))
                (set `self.MineGunSE` _returnvalue)
                (`AudioComponent.Play` (`self.MineGunSE`) 0.0))))
          (:`then_1`
            (`KismetSystemLibrary.Delay` 0.2)
            (`self.MineGun`))))))
  (:`Completed`
    (set `self.Mine_Gun_Fire` false)))

(event `MineGun`
  (bind (_returnvalue_location _returnvalue_rotation) (`KismetMathLibrary.BreakTransform` (`self.GetSocketTransform` "fire")))
  (if (and (<= (`self.MineGun_Count`) 30) (`self.Mine_Gun_Fire`))
    (bind _result (`/Engine/EditorBlueprintResources/StandardMacros.IncrementInt` (`self.MineGun_Count`))
      (:`  `
        (bind _output_get (set `self.MineGun_Count` _result))
        (`KismetSystemLibrary.PrintString` (`KismetStringLibrary.Conv_IntToString` _output_get))
        (`|SpawnActorFromClass` "/Game/Blueprint/Weapon/BP_Player_Minegun.BP_Player_Minegun_C" (`KismetMathLibrary.MakeTransform` _returnvalue_location _returnvalue_rotation) "Undefined" "OverrideRootScale" null 500.0 null)))
    (else
      (`AudioComponent.Stop` (`self.MineGunSE`))
      (set `self.MineGun_Count` 0)
      (set `self.MineGun_CT_Bool` true))))

(fn `GetWB_CT`
  (returns (NewParam :type "/Game/Blueprint/Player/WB_CT Object Reference"))
  (bind _foundwidgets (`WidgetBlueprintLibrary.GetAllWidgetsOfClass` "/Game/Blueprint/Player/WB_CT.WB_CT_C"))
  (return (`|GetArrayItem` _foundwidgets)))