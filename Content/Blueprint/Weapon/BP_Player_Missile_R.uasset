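; BP_Player_Missile_R is a player missile that rises along a fixed diagonal, then flies in a straight line toward a stored enemy location.
; Tick counts rise frames, captures the direction once, moves by local offsets and self-destructs after a delay.
; GetEnemyLocation scans enemies for minimum distance every tick but never writes EnemyLocation.
; Ending sphere overlap with a BP_Enemy deals damage, plays an explosion sound and destroys the missile.
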(event `self.ReceiveBeginPlay`)

(event `self.ReceiveTick`
  (params (DeltaSeconds :type "Float (single-precision)"))
  (`self.GetEnemyLocation`)
  (if (>= (`self.Missile_Rise_Time`) 30.0)
    (if (`self.get_enemy_posision`)
      (`self.K2_AddActorLocalOffset` (* (`self.Missile_Vec`) (`self.move_speed`)))
      (`KismetSystemLibrary.Delay` 5.0)
      (`self.K2_DestroyActor`)
      (set `self.Missile_Rise_Time` 0.0)
      (else
        (set `self.Missile_Vec` (- (`self.Enemy_Location`) (`self.K2_GetActorLocation`)))
        (set `self.get_enemy_posision` true)))
    (else
      (`self.K2_AddActorLocalOffset` (* (-1.5 0.0 1.5) (`self.Rise_speed`)))
      (bind _result (`/Engine/EditorBlueprintResources/StandardMacros.IncrementFloat` (`self.Missile_Rise_Time`))
        (:`  `
          (set `self.Missile_Rise_Time` _result))))))

(event `self.Sphere.OnComponentEndOverlap`
  (params (OverlappedComponent :type "PrimitiveComponent Object Reference") (OtherActor :type "Actor Object Reference") (OtherComp :type "PrimitiveComponent Object Reference") (OtherBodyIndex :type Integer))
  (bind _asbp_enemy (cast `/Game/Blueprint/Enemy/BP_Enemy` OtherActor))
  (`GameplayStatics.ApplyDamage` _asbp_enemy 100.0)
  (`GameplayStatics.PlaySound2D` "/Game/Sound/Weapon/Missile/爆発3.爆発3" 2.0 1.0 0.0 null null)
  (`self.K2_DestroyActor`)
  (`KismetSystemLibrary.PrintString` "Destroy"))

(fn `GetEnemyLocation`
  (bind _outactors (`GameplayStatics.GetAllActorsOfClass` "/Game/Blueprint/Enemy/BP_Enemy.BP_Enemy_C"))
  (for _array_element _outactors
    (bind _returnvalue (`self.GetDistanceTo` _array_element self))
    (if (< _returnvalue (`self.Min_Distance`))
      (set `self.Min_Distance` _returnvalue)
      (`GameplayStatics.GetActorOfClass` "/Game/Blueprint/Weapon/BP_Player_Missile_L.BP_Player_Missile_L_C"))))

(fn `UserConstructionScript`)