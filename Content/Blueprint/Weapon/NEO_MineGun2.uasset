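; Minigun weapon component for BP_Player that attaches to the "weapon3" socket of the owner's mesh on BeginPlay.
; A DoOnce-gated trigger calls Fire, which loops over BulletMax with a short Delay in the body, spawning BP_Player_Minegun actors at the Buki02_Bullet socket.
; A second DoOnce limits creation of the 2D firing sound; loop completion stops it and re-arms the trigger.
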(event `self.ReceiveBeginPlay`
  (bind _asbp_player (cast `/Game/Blueprint/Player/BP_Player` (`self.GetOwner`)))
  (bind _output_get (set `self.First Person Character` _asbp_player))
  (`self.K2_AttachToComponent` (`Character.Mesh` _output_get) "weapon3" "KeepRelative" "KeepRelative" "KeepRelative"))

(event `self.ReceiveTick`
  (params (DeltaSeconds :type "Float (single-precision)")))

(event `Fire_Trigger_MineGun`
  (`/Engine/EditorBlueprintResources/StandardMacros.DoOnce` false :!label _label
    (:`Completed`
      (`self.Fire`)
      (`self.FireReset`))))

(event `StartReset`
  (goto _label :!via `Reset`))

(event `Fire`
  (bind (_returnvalue_location _returnvalue_rotation) (`KismetMathLibrary.BreakTransform` (`self.GetSocketTransform` "Buki02_Bullet")))
  (for _ (range (+ (`self.Bullet Max`) 1))
    (`KismetSystemLibrary.Delay` 0.2)
    (`|ExecutionSequence`
      (:`then_0`
        (`/Engine/EditorBlueprintResources/StandardMacros.DoOnce` false :!label _label_2
          (:`Completed`
            (bind _returnvalue (`GameplayStatics.CreateSound2D` "/Game/Sound/Weapon/MineGun/MineGun_Sound.MineGun_Sound" 1.5 1.0 0.0 null))
            (set `self.MineGunSE` _returnvalue)
            (`AudioComponent.Play` (`self.MineGunSE`) 0.0))))
      (:`then_1`
        (`|SpawnActorFromClass` "/Game/Blueprint/Weapon/BP_Player_Minegun.BP_Player_Minegun_C" (`KismetMathLibrary.MakeTransform` _returnvalue_location _returnvalue_rotation) "Undefined" "OverrideRootScale" null 50.0 null))))
  (`AudioComponent.Stop` (`self.MineGunSE`))
  (`self.StartReset`))

(event `FireReset`
  (goto _label_2 :!via `Reset`))

(fn `Fire_End_MineGun`
  (set `self.Mine_Gun_Fire` false))

(fn `Get_BP_Player`
  (returns (BP_Player :type "/Game/Blueprint/Player/BP_Player Object Reference"))
  (bind _returnvalue (`GameplayStatics.GetActorOfClass` "/Game/Blueprint/Player/BP_Player.BP_Player_C"))
  (return _returnvalue))

(fn `GetWB_CT`
  (returns (NewParam :type "/Game/Blueprint/Player/WB_CT Object Reference"))
  (bind _foundwidgets (`WidgetBlueprintLibrary.GetAllWidgetsOfClass` "/Game/Blueprint/Player/WB_CT.WB_CT_C"))
  (return (`|GetArrayItem` _foundwidgets)))