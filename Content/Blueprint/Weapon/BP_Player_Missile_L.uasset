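; Player-fired left missile that flies toward the first enemy position stored on BP_Player, captured once at BeginPlay rather than tracked live.
; Each Tick applies a normalised direction-to-target as a local offset, and a timer destroys it after five seconds.
; On sphere end-overlap (not begin), it damages NEO enemies or destroys enemy bullets, playing an explosion sound and destroying itself.
; Enemy-search functions are never called.
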(event `self.ReceiveBeginPlay`
  (`self.Get_BP_Player`)
  (set `self.Enemy_Pos` (`|GetArrayItem` (`/Game/Blueprint/Player/BP_Player.Enemy_Position` (`self.BP_Player`))))
  (`self.Get_NEO_Missile_L`))

(event `self.ReceiveTick`
  (params (DeltaSeconds :type "Float (single-precision)"))
  (`self.K2_AddActorLocalOffset` (* (`KismetMathLibrary.Normal` (- (`self.Enemy_Pos`) (`self.K2_GetActorLocation`))) (`self.move_speed`)))
  (`self.Life_count`))

(event `self.Sphere.OnComponentEndOverlap`
  (params (OverlappedComponent :type "PrimitiveComponent Object Reference") (OtherActor :type "Actor Object Reference") (OtherComp :type "PrimitiveComponent Object Reference") (OtherBodyIndex :type Integer))
  (`|ExecutionSequence`
    (:`then_0`
      (if (`self.ActorHasTag` OtherActor "Enemy")
        (bind _asbp_neo_enemy (cast `/Game/Blueprint/Enemy/BP_NEO_Enemy` OtherActor))
        (`GameplayStatics.ApplyDamage` _asbp_neo_enemy 100.0)
        (`GameplayStatics.PlaySound2D` "/Game/Sound/Weapon/Missile/爆発3.爆発3" 2.0 1.0 0.0 null null)
        (`self.K2_DestroyActor`)))
    (:`then_1`
      (if (`self.ActorHasTag` OtherActor "EnemyBullet")
        (`GameplayStatics.PlaySound2D` "/Game/Sound/Weapon/Missile/爆発3.爆発3" 2.0 1.0 0.0 null null)
        (`AudioComponent.Stop` (`/Game/Blueprint/Weapon/NEO_Missile_R.MissileSound` (`self.NEO_Missile_R`)))
        (`self.K2_DestroyActor` OtherActor)
        (`self.K2_DestroyActor`)))))

(fn `Get_BP_Player`
  (bind _returnvalue (`GameplayStatics.GetActorOfClass` "/Game/Blueprint/Player/BP_Player.BP_Player_C"))
  (set `self.BP_Player` _returnvalue))

(fn `Get_GI_Defolut`
  (returns (`AsGI Defolut` :type "/Game/Blueprint/Maps/GI_Defolut Object Reference"))
  (bind _asgi_defolut (cast `/Game/Blueprint/Maps/GI_Defolut` (`GameplayStatics.GetGameInstance`)))
  (return _asgi_defolut))

(fn `Get_NEO_Missile_L`
  (bind _returnvalue (`AddComponent|NODE_AddNEO_Missile_R-0`))
  (set `self.NEO_Missile_R` _returnvalue))

(fn `GetEnemyLocation`
  (`GameplayStatics.GetActorOfClass` "/Game/Blueprint/Player/BP_Player.BP_Player_C"))

(fn `GetNEOEnemyLocation`
  (bind _outactors (`GameplayStatics.GetAllActorsOfClass` "/Game/Blueprint/Enemy/BP_Enemy.BP_Enemy_C"))
  (for _array_element _outactors
    (bind _returnvalue (`self.GetDistanceTo` _array_element self))
    (if (< _returnvalue (`self.Min_Distance`))
      (set `self.Min_Distance` _returnvalue)
      (`GameplayStatics.GetActorOfClass` "BP_Player_Missile_L_C"))))

(fn `Life_count`
  (bind _output_get (set `self.Life_time` (+ (`self.Life_time`) (`GameplayStatics.GetWorldDeltaSeconds`))))
  (if (>= _output_get 5.0)
    (`self.K2_DestroyActor`)
    (set `self.Life_time` 0.0))
  (return))

(fn `UserConstructionScript`)