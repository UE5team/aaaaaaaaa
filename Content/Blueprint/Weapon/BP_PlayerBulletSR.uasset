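; BP_PlayerBulletSR is a player bullet that heads toward an enemy position and damages BP_NEO_Enemy actors.
; On BeginPlay it copies the first SREnemyPos entry from BP_Player as a fixed target.
; Each Tick it moves by a swept local offset along the normalized vector to that point, destroying itself after its lifetime.
; Fixed damage applies when its sphere's overlap with an enemy ends, without destroying the bullet.
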(event `self.ReceiveBeginPlay`
  (`self.Get_BP_Player`)
  (set `self.Enemy pos` (`|GetArrayItem` (`/Game/Blueprint/Player/BP_Player.SR_Enemy_pos` (`self.BP_Player`)))))

(event `self.ReceiveTick`
  (params (DeltaSeconds :type "Float (single-precision)"))
  (bind _existtime (`self.ExistTime`))
  (`|ExecutionSequence`
    (:`then_0`
      ;[1 1 1] プレイヤー前方に弾を移動
      (`self.K2_AddActorLocalOffset` (* (`KismetMathLibrary.Normal` (- (`self.Enemy pos`) (`self.K2_GetActorLocation`))) (`self.Speed`)) true))
    (:`then_1`
      (set `self.ExistTime` (+ DeltaSeconds _existtime)) ; 弾が出現している時間を計測
    )
    (:`then_2`
      ;[1 1 1] 寿命を迎えたら消す
      (if (< (`self.DestroyTIme`) _existtime)
        (`self.K2_DestroyActor`)))))

(event `self.Sphere.OnComponentEndOverlap`
  (params (OverlappedComponent :type "PrimitiveComponent Object Reference") (OtherActor :type "Actor Object Reference") (OtherComp :type "PrimitiveComponent Object Reference") (OtherBodyIndex :type Integer))
  (bind _asbp_neo_enemy (cast `/Game/Blueprint/Enemy/BP_NEO_Enemy` OtherActor))
  (`GameplayStatics.ApplyDamage` _asbp_neo_enemy 5.0))

(fn `Get_BP_Player`
  (bind _returnvalue (`GameplayStatics.GetActorOfClass` "/Game/Blueprint/Player/BP_Player.BP_Player_C"))
  (set `self.BP_Player` _returnvalue))

(fn `UserConstructionScript`)