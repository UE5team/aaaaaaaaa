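; BP_PlayerBulletSMG is the player's SMG bullet, which damages BP_Enemy actors it hits.
; On BeginPlay it derives a direction from the player-to-bullet positions, then each Tick sweeps away along it as a local offset, unscaled by delta time.
; A sphere overlap with an enemy applies damage and destroys the bullet, which also destroys itself once its accumulated lifetime passes a limit.
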(event `self.ReceiveBeginPlay`
  (set `self.MoveDirection` (`KismetMathLibrary.Normal` (- (`self.K2_GetActorLocation` (`GameplayStatics.GetPlayerCharacter` 0)) (`self.K2_GetActorLocation`))))
  (`KismetSystemLibrary.PrintString` "Bullet Begin"))

(event `self.ReceiveTick`
  (params (DeltaSeconds :type "Float (single-precision)"))
  (bind _existtime (`self.ExistTime`))
  (`|ExecutionSequence`
    (:`then_0`
      ;[1 1 1] 決められた方向に移動
      (`self.K2_AddActorLocalOffset` (* (`self.Speed`) (`self.MoveDirection`) -1.0) true))
    (:`then_1`
      (set `self.ExistTime` (+ DeltaSeconds _existtime)) ; 弾が出現している時間を計測
    )
    (:`then_2`
      ;[1 1 1] 寿命を迎えたら消す
      (if (< (`self.DestroyTIme`) _existtime)
        (`self.K2_DestroyActor`)))))

(event `self.Sphere.OnComponentBeginOverlap`
  (params (OverlappedComponent :type "PrimitiveComponent Object Reference") (OtherActor :type "Actor Object Reference") (OtherComp :type "PrimitiveComponent Object Reference") (OtherBodyIndex :type Integer) (bFromSweep :type Boolean) (SweepResult :type "HitResult Structure (by ref)"))
  (bind _asbp_enemy (cast `/Game/Blueprint/Enemy/BP_Enemy` OtherActor))
  (`GameplayStatics.ApplyDamage` _asbp_enemy 1.0)
  (`self.K2_DestroyActor`)
  (`KismetSystemLibrary.PrintString` "Destroy"))

(fn `UserConstructionScript`)