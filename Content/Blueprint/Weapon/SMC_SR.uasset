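; Sniper rifle component for the player that attaches to the Weapon2 mesh socket and adds its own input mapping on BeginPlay.
; IA_SR spawns a BP_PlayerBulletSR ahead of the owner when ready, plays the shot sound and adds its cost to GameInstance WeaponPoints.
; Firing sets SRCoolTime on PlayerState; Tick then plays the bolt-action sound once and counts down the timer stored in the WB_CT widget before re-arming.
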(event `self.ReceiveBeginPlay`
  (`|ExecutionSequence`
    (:`then_0`
      ;[1 1 1] プレイヤーのSKMのソケットにSMGのメッシュをアタッチ
      (bind _asbp_player (cast `/Game/Blueprint/Player/BP_Player` (`self.GetOwner`)))
      (bind _output_get (set `self.BP Player` _asbp_player))
      (`self.K2_AttachToComponent` (`Character.Mesh` _output_get) "Weapon2" "KeepRelative" "KeepRelative" "KeepRelative"))
    (:`then_1`
      ;[1 1 1] プレイヤーステートを参照できる変数を作成
      (bind _asbp_player_state (cast `/Game/Blueprint/Player/BP_PlayerState` (`GameplayStatics.GetPlayerState` 0)))
      (set `self.BP PlayerState` _asbp_player_state))
    (:`then_2`
      ;[1 1 1] インプットアクションを追加
      (bind _asplayer_controller (cast `PlayerController` (`Pawn.GetController` (`self.BP Player`))))
      (bind _returnvalue (pcsubsystem `EnhancedInputLocalPlayerSubsystem` _asplayer_controller))
      (`/Engine/EditorBlueprintResources/StandardMacros.IsValid` _returnvalue
        (:`Is Valid`
          (`EnhancedInputSubsystemInterface.AddMappingContext` _returnvalue "/Game/Input/Player/IMC_SR.IMC_SR" 1 (struct)))))
    (:`then_3`
      ;[1 1 1] ゲームインスタンスを参照できる変数を作成
      (bind _asgi_defolut (cast `/Game/Blueprint/Maps/GI_Defolut` (`GameplayStatics.GetGameInstance`)))
      (set `self.GI VariableRetention` _asgi_defolut))))

(event `EnhancedInput|/Game/Input/Player/IA_SR`
  (params (ActionValue :type Boolean) (ElapsedSeconds :type "Float (double-precision)") (TriggeredSeconds :type "Float (double-precision)") (InputAction :type "InputAction Object Reference" :default "/Game/Input/Player/IA_SR.IA_SR"))
  (bind _returnvalue (`self.GetOwner`))
  (bind _gi_variableretention (`self.GI VariableRetention`))
  ;[1 1 1] SR発射
  (:`Started`
    ;;[1 1 1] 弾が発射準備ができているかを判定
    (if (`self.IsFireSet`)
      (bind _returnvalue_2 (`GameplayStatics.CreateSound2D` "/Game/Sound/Weapon/SR/狙撃銃発射.狙撃銃発射" 3.0 1.0 0.0 null))
      (bind _output_get (set `self.SR_Sound` _returnvalue_2))
      (`AudioComponent.Play` _output_get 0.0)
      ;;[1 1 1] 弾を出す
      (`|SpawnActorFromClass` "/Game/Blueprint/Weapon/BP_PlayerBulletSR.BP_PlayerBulletSR_C" (`KismetMathLibrary.MakeTransform` (+ (`Actor.K2_GetActorLocation` _returnvalue) (* (`Actor.GetActorForwardVector` _returnvalue) (`self.BulletSpawnLocation`)))) "Undefined" "OverrideRootScale" null null) ; SMG
      (set `self.IsFireSet` false)
      (set `/Game/Blueprint/Player/BP_PlayerState.SR CoolTime` true (`self.BP PlayerState`))
      ;;[1 1 1] ポイント消費
      (set `/Game/Blueprint/Maps/GI_Defolut.WeaponPoints` (+ (`/Game/Blueprint/Maps/GI_Defolut.WeaponPoints` _gi_variableretention) (`self.WeaponConsumptionPoints`)) _gi_variableretention))))

(event `self.ReceiveTick`
  (params (DeltaSeconds :type "Float (single-precision)"))
  ;[1 1 1] クールタイム
  (if (`/Game/Blueprint/Player/BP_PlayerState.SR CoolTime` (`self.BP PlayerState`))
    (`|ExecutionSequence`
      (:`then_0`
        (`/Engine/EditorBlueprintResources/StandardMacros.DoOnce` false :!label _label
          (:`Completed`
            (bind _newparam (`self.GetWB_CT`))
            (set `/Game/Blueprint/Player/WB_CT.SR CoolTimeNow` (`self.MaxCoolTime`) _newparam)
            (bind _returnvalue (`GameplayStatics.CreateSound2D` "/Game/Sound/Weapon/SR/狙撃銃のボルトアクション.狙撃銃のボルトアクション" 1.0 1.0 0.0 null))
            (bind _output_get (set `self.SR_Relord_Sound` _returnvalue))
            (`AudioComponent.Play` _output_get 0.0))))
      (:`then_1`
        (bind _newparam_2 (`self.GetWB_CT`))
        (bind _output_get_2 (set `/Game/Blueprint/Player/WB_CT.SR CoolTimeNow` (- (`/Game/Blueprint/Player/WB_CT.SR CoolTimeNow` _newparam_2) (`GameplayStatics.GetWorldDeltaSeconds`)) _newparam_2))
        (if (<= _output_get_2 0.0)
          (set `/Game/Blueprint/Player/BP_PlayerState.SR CoolTime` false (`self.BP PlayerState`))
          (set `self.IsFireSet` true))))
    (else
      (goto _label :!via `Reset`))))

(fn `GetWB_CT`
  (returns (NewParam :type "/Game/Blueprint/Player/WB_CT Object Reference"))
  (bind _foundwidgets (`WidgetBlueprintLibrary.GetAllWidgetsOfClass` "/Game/Blueprint/Player/WB_CT.WB_CT_C"))
  (return (`|GetArrayItem` _foundwidgets)))