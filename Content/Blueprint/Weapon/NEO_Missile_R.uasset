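; Missile weapon Blueprint that fires a left and right player missile pair from the MissileFire socket on IA_Missile input, with sound.
; Each pair targets the BP_Player enemy position at MissileIndex, which cycles through four slots and resets the player's missile-exist states on wrap.
; Each shot adds its consumption to WeaponPoints in GI_Defolut and starts a three-second cooldown.
; Tick counts the cooldown down directly on the WB_CT widget's MissileCT, then re-enables firing.
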(event `self.ReceiveBeginPlay`)

(event `EnhancedInput|/Game/Input/Player/IA_Missile`
  (params (ActionValue :type Boolean) (ElapsedSeconds :type "Float (double-precision)") (TriggeredSeconds :type "Float (double-precision)") (InputAction :type "InputAction Object Reference" :default "/Game/Input/Player/IA_Missile.IA_Missile"))
  (bind _returnvalue_location (`KismetMathLibrary.BreakTransform` (`self.GetSocketTransform` "MissileFire")))
  (bind _returnvalue_location_2 (`KismetMathLibrary.BreakTransform` (`self.GetSocketTransform` "MissileFire")))
  (:`Triggered`
    ;[1 1 1] ボタンを押したらMissile_LとMissile_RからMissileをスポーンさせる
    (if (not (`self.Missile CT Exist`))
      (bind _outactors (`GameplayStatics.GetAllActorsOfClass` "/Game/Blueprint/Player/BP_Player.BP_Player_C"))
      (bind _returnvalue (`GameplayStatics.CreateSound2D` "/Game/Sound/Weapon/Missile/Missile.Missile" 1.0 1.0 0.0 null))
      (bind _output_get (set `self.NewVar` _returnvalue))
      (`AudioComponent.Play` _output_get 0.0)
      (bind _output (`|GetArrayItem` _outactors))
      (bind _output_2 (`|GetArrayItem` (`/Game/Blueprint/Player/BP_Player.Enemy_Position` _output) (`/Game/Blueprint/Player/BP_Player.Missile Index` _output)))
      (`|SpawnActorFromClass` "/Game/Blueprint/Weapon/BP_Player_Missile_L.BP_Player_Missile_L_C" (`KismetMathLibrary.MakeTransform` _returnvalue_location_2 (struct) (0.5 0.5 0.5)) "Undefined" "OverrideRootScale" null 0.0 50.0 _output_2 null)
      (`|SpawnActorFromClass` "/Game/Blueprint/Weapon/BP_Player_Missile_R.BP_Player_Missile_R_C" (`KismetMathLibrary.MakeTransform` _returnvalue_location (struct) (0.5 0.5 0.5)) "Undefined" "OverrideRootScale" null 0.0 50.0 _output_2 null)
      ;[1 1 1] ポイント消費計算
      (bind _asgi_defolut (cast `/Game/Blueprint/Maps/GI_Defolut` (`GameplayStatics.GetGameInstance`)))
      (set `/Game/Blueprint/Maps/GI_Defolut.WeaponPoints` (+ (`/Game/Blueprint/Maps/GI_Defolut.WeaponPoints` _asgi_defolut) (`self.Weapon Point Consumption`)) _asgi_defolut)
      (bind _missile_index (`/Game/Blueprint/Player/BP_Player.Missile Index` _output))
      ;[1 1 1] 配列番号の切り替え
      (if (> _missile_index 2)
        (set `/Game/Blueprint/Player/BP_Player.Missile Index` 0 _output)
        ;[1 1 1] Enemyの座標を配列に入れる条件の初期化
        (bind _returnvalue_2 (`GameplayStatics.GetActorOfClass` "/Game/Blueprint/Player/BP_Player.BP_Player_C"))
        (`|ExecutionSequence`
          (:`then_0`
            (`/Game/Blueprint/Player/BP_Player.Missile_Exist１の初期化` _returnvalue_2))
          (:`then_1`
            (`/Game/Blueprint/Player/BP_Player.Missile Exist2の初期化` _returnvalue_2))
          (:`then_2`
            (`/Game/Blueprint/Player/BP_Player.Missile Exist3の初期化` _returnvalue_2))
          (:`then_3`
            (`/Game/Blueprint/Player/BP_Player.Missile Exist４の初期化` _returnvalue_2)
            ;[1 1 1] Missileのクールタイム
            (set `self.Missile CT Exist` true :!label _label)))
        (else
          (`/Engine/EditorBlueprintResources/StandardMacros.IncrementInt` _missile_index
            (:`  `
              (goto _label))))))))

(event `self.ReceiveTick`
  (params (DeltaSeconds :type "Float (single-precision)"))
  (if (`self.Missile CT Exist`)
    (`|ExecutionSequence`
      (:`then_0`
        (`/Engine/EditorBlueprintResources/StandardMacros.DoOnce` false :!label _label_2
          (:`Completed`
            (bind _wb_ct (`self.GetWB_CT`))
            (set `/Game/Blueprint/Player/WB_CT.Missile_CT` 3.0 _wb_ct))))
      (:`then_1`
        (bind _wb_ct_2 (`self.GetWB_CT`))
        (bind _output_get (set `/Game/Blueprint/Player/WB_CT.Missile_CT` (- (`/Game/Blueprint/Player/WB_CT.Missile_CT` _wb_ct_2) (`GameplayStatics.GetWorldDeltaSeconds`)) _wb_ct_2))
        (if (< _output_get 0.0)
          (set `self.Missile CT Exist` false)
          (goto _label_2 :!via `Reset`))))))

(fn `GetWB_CT`
  (returns (WB_CT :type "/Game/Blueprint/Player/WB_CT Object Reference"))
  (bind _foundwidgets (`WidgetBlueprintLibrary.GetAllWidgetsOfClass` "/Game/Blueprint/Player/WB_CT.WB_CT_C"))
  (return (`|GetArrayItem` _foundwidgets)))