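; SMG weapon mesh component that fires bullets at enemies flagged with an existing attack lock-on.
; Fire_SMG scans all BP_NEO_Enemy actors and spawns a burst from the SMG_Bullet socket for each flagged one, passing that enemy's position.
; A DoOnce limits the 2D firing sound to one play until ReSetSE resets it.
; Spawn-location helpers are unused by the firing path, and FireEnd_SMG is empty.
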(event `self.ReceiveBeginPlay`)

(event `ReSetSE`
  ;[1 1 1] SMG発射
  (goto _label :!via `Reset`))

(event `Fire_SMG`
  ;[1 1 1] SMG発射
  (bind _outactors (`GameplayStatics.GetAllActorsOfClass` "/Game/Blueprint/Enemy/BP_NEO_Enemy.BP_NEO_Enemy_C"))
  (for (_ _array_index) _outactors
    (bind _output (`|GetArrayItem` _outactors _array_index))
    (if (`/Game/Blueprint/Enemy/BP_NEO_Enemy.AttackRockOnExist` _output)
      (for _ (range 4)
        (`|SpawnActorFromClass` "/Game/Blueprint/Weapon/BP_PlayerBulletSMG.BP_PlayerBulletSMG_C" (`KismetMathLibrary.MakeTransform` (`self.GetSocketLocation` "SMG_Bullet")) "Undefined" "OverrideRootScale" null (`Actor.K2_GetActorLocation` _output) null)
        (`/Engine/EditorBlueprintResources/StandardMacros.DoOnce` false :!label _label
          (:`Completed`
            (bind _returnvalue (`GameplayStatics.CreateSound2D` "/Game/Sound/Weapon/SMG/サブマシンガン発射2.サブマシンガン発射2" 1.0 1.0 0.0 null))
            (bind _output_get (set `self.SMG_Sound` _returnvalue))
            (`AudioComponent.Play` _output_get 0.0)))))))

(event `self.ReceiveTick`
  (params (DeltaSeconds :type "Float (single-precision)")))

(fn `BasicSpawnLocation`
  (returns (ReturnValue :type "Vector Structure"))
  (bind _returnvalue (`self.GetOwner`))
  (return (+ (`Actor.K2_GetActorLocation` _returnvalue) (* (`Actor.GetActorForwardVector` _returnvalue) (`self.BulletSpawnLocation`)))))

(fn `FireEnd_SMG`)

(fn `GetWB_CT`
  (returns (NewParam :type "/Game/Blueprint/Player/WB_CT Object Reference"))
  (bind _foundwidgets (`WidgetBlueprintLibrary.GetAllWidgetsOfClass` "/Game/Blueprint/Player/WB_CT.WB_CT_C"))
  (return (`|GetArrayItem` _foundwidgets)))

(fn `RandomSpawnLocation`
  (params (A :type "Vector Structure"))
  (returns (ReturnValue :type "Vector Structure"))
  (return (+ A (* (`self.GetForwardVector`) (`KismetMathLibrary.DegCos` (`KismetMathLibrary.RandomFloatInRange` 0.0 180.0)) (`self.SMG Blur`)))))