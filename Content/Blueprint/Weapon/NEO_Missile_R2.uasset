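; NEO_Missile_R2 is a player missile weapon that fires left and right missile pairs when the player has stored enemy positions.
; FireTriggerMissile plays the sound, spawns missiles at two sockets outside cooldown, and adds the point cost to GI_Defolut's WeaponPoints.
; While the fired count is under four, it drops the first target and resets the DoOnce gates.
; When MissileCTExist is set, Tick runs the cooldown countdown stored in the WB_CT widget.
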(event `MineCT`
  (`/Engine/EditorBlueprintResources/StandardMacros.DoOnce` false :!label _label))

(event `ResetMineCT`
  (goto _label :!via `Reset`))

(event `Delay`
  (`KismetSystemLibrary.Delay` 0.2))

(event `PointCalculation`
  ;[1 1 1] ポイント計算
  (`/Engine/EditorBlueprintResources/StandardMacros.DoOnce` false :!label _label_2
    (:`Completed`
      (bind _asgi_defolut (cast `/Game/Blueprint/Maps/GI_Defolut` (`GameplayStatics.GetGameInstance`)))
      (set `/Game/Blueprint/Maps/GI_Defolut.WeaponPoints` (+ (`/Game/Blueprint/Maps/GI_Defolut.WeaponPoints` _asgi_defolut) (`self.Weapon Point Consumption`)) _asgi_defolut))))

(event `ResetPointCalculation`
  ;[1 1 1] ポイント計算
  (goto _label_2 :!via `Reset`))

(event `self.ReceiveBeginPlay`
  (`self.Get_BP_Player`))

(event `self.ReceiveTick`
  (params (DeltaSeconds :type "Float (single-precision)"))
  (if (`self.Missile CT Exist`)
    (`|ExecutionSequence`
      (:`then_0`
        (`/Engine/EditorBlueprintResources/StandardMacros.DoOnce` false :!label _label_3
          (:`Completed`
            (bind _wb_ct (`self.GetWB_CT`))
            (set `/Game/Blueprint/Player/WB_CT.Missile_CT` 3.0 _wb_ct))))
      (:`then_1`
        (bind _wb_ct_2 (`self.GetWB_CT`))
        (bind _output_get (set `/Game/Blueprint/Player/WB_CT.Missile_CT` (- (`/Game/Blueprint/Player/WB_CT.Missile_CT` _wb_ct_2) (`GameplayStatics.GetWorldDeltaSeconds`)) _wb_ct_2))
        (if (< _output_get 0.0)
          (set `self.Missile CT Exist` false)
          (goto _label_3 :!via `Reset`))))))

(fn `Fire_Trigger_Missile`
  (bind _returnvalue_location (`KismetMathLibrary.BreakTransform` (`self.GetSocketTransform` "Missile_R_Bullet")))
  (bind _returnvalue_location_2 (`KismetMathLibrary.BreakTransform` (`self.GetSocketTransform` "Missile_L_Bullet")))
  (if (`KismetArrayLibrary.Array_IsNotEmpty` (`/Game/Blueprint/Player/BP_Player.Enemy_Position` (`self.As BP Player`)))
    (`|ExecutionSequence`
      (:`then_0`
        (`self.MineCT`)
        ;[1 1 1] ボタンを押したらMissile_LとMissile_RからMissileをスポーンさせる
        (if (not (`self.Missile CT Exist`))
          (bind _returnvalue (`GameplayStatics.GetActorOfClass` "/Game/Blueprint/Player/BP_Player.BP_Player_C"))
          (bind _returnvalue_2 (`GameplayStatics.CreateSound2D` "/Game/Sound/Weapon/Missile/Missile.Missile" 1.0 1.0 0.0 null))
          (bind _output_get (set `self.MissileSound` _returnvalue_2))
          (`AudioComponent.Play` _output_get 0.0)
          (`/Engine/EditorBlueprintResources/StandardMacros.IncrementInt` (`self.Number of missiles fired`)
            (:`  `
              (`|SpawnActorFromClass` "/Game/Blueprint/Weapon/BP_Player_Missile_L.BP_Player_Missile_L_C" (`KismetMathLibrary.MakeTransform` _returnvalue_location_2 (struct) (0.5 0.5 0.5)) "Undefined" "OverrideRootScale" null 0.0 50.0 (0.0 0.0 0.0) null)
              (`|SpawnActorFromClass` "/Game/Blueprint/Weapon/BP_Player_Missile_R.BP_Player_Missile_R_C" (`KismetMathLibrary.MakeTransform` _returnvalue_location (struct) (0.5 0.5 0.5)) "Undefined" "OverrideRootScale" null 0.0 50.0 (0.0 0.0 0.0) null)))))
      (:`then_1`
        ;[1 1 1] ポイント消費計算
        (`self.PointCalculation`))
      (:`then_2`
        ;[1 1 1] 配列番号の切り替え
        (if (not (>= (`self.Number of missiles fired`) 4))
          (`self.Delay`)
          (`KismetArrayLibrary.Array_Remove` (`/Game/Blueprint/Player/BP_Player.Enemy_Position` (`self.As BP Player`)))
          (`self.ResetPointCalculation`)
          (`self.ResetMineCT`)
          (`/Engine/EditorBlueprintResources/StandardMacros.DecrementInt` (`/Game/Blueprint/Player/BP_Player.SetEnemy Missile Index` _returnvalue)))))))

(fn `Get_BP_Player`
  (bind _returnvalue (`GameplayStatics.GetActorOfClass` "/Game/Blueprint/Player/BP_Player.BP_Player_C"))
  (set `self.As BP Player` _returnvalue))

(fn `GetWB_CT`
  (returns (WB_CT :type "/Game/Blueprint/Player/WB_CT Object Reference"))
  (bind _foundwidgets (`WidgetBlueprintLibrary.GetAllWidgetsOfClass` "/Game/Blueprint/Player/WB_CT.WB_CT_C"))
  (return (`|GetArrayItem` _foundwidgets)))