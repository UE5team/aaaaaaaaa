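; BP_Player_Minegun is a player minigun projectile that damages enemies it passes through.
; Tick moves it by BulletVec times Speed in local space, unswept and not scaled by delta time, and a five-second Delay then destroys it.
; Sphere overlaps apply fixed damage to Enemy-tagged actors without destroying the projectile.
; Helper getters for BP_Player and GI_Defolut exist but drive no active logic.
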(event `self.ReceiveTick`
  (params (DeltaSeconds :type "Float (single-precision)"))
  (`self.K2_AddActorLocalOffset` (* (`self.Bullet_vec`) (`self.speed`)))
  (`KismetSystemLibrary.Delay` 5.0)
  (`self.K2_DestroyActor`))

(event `self.Sphere.OnComponentBeginOverlap`
  (params (OverlappedComponent :type "PrimitiveComponent Object Reference") (OtherActor :type "Actor Object Reference") (OtherComp :type "PrimitiveComponent Object Reference") (OtherBodyIndex :type Integer) (bFromSweep :type Boolean) (SweepResult :type "HitResult Structure (by ref)"))
  (if (`self.ActorHasTag` OtherActor "Enemy")
    (`GameplayStatics.ApplyDamage` OtherActor 100.0)))

(fn `Get_BP_Player`
  (returns (BP_Player :type "/Game/Blueprint/Player/BP_Player Object Reference"))
  (bind _returnvalue (`GameplayStatics.GetActorOfClass` "/Game/Blueprint/Player/BP_Player.BP_Player_C"))
  (return _returnvalue))

(fn `Get_GI_Defolut`
  (returns (`GI Defolut` :type "/Game/Blueprint/Maps/GI_Defolut Object Reference"))
  (bind _asgi_defolut (cast `/Game/Blueprint/Maps/GI_Defolut` (`GameplayStatics.GetGameInstance`)))
  (return _asgi_defolut))

(fn `UserConstructionScript`)