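; BP_Enemy_Points is a point pickup that homes in on BP_Player and awards enemy points on contact.
; Each tick it offsets itself along the normalized direction to the player, applied in local space, with speed compounding 5% per frame.
; Overlapping a "Player"-tagged actor calls AddEnemyPoint on BP_InGame_GameMode and destroys the pickup.
; It also self-destructs once the in-game UI's Timer reports IsGoal.
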(event `self.ReceiveBeginPlay`
  (bind _returnvalue (`GameplayStatics.GetActorOfClass` "/Game/Blueprint/Player/BP_Player.BP_Player_C"))
  (set `self.NewVar` _returnvalue)
  (bind _foundwidgets (`WidgetBlueprintLibrary.GetAllWidgetsOfClass` "/Game/Blueprint/Maps/WBP_Ingame_UI.WBP_Ingame_UI_C"))
  (set `self.Timer` (`/Game/Blueprint/Maps/WBP_Ingame_UI.timer` (`|GetArrayItem` _foundwidgets))))

(event `self.ReceiveTick`
  (params (DeltaSeconds :type "Float (single-precision)"))
  ;[1 1 1] 弾の移動する動き
  (bind _return_coordinate (`self.Get Coordinate`))
  (bind _return_point_speed (`self.Get Point Speed`))
  (`self.K2_AddActorLocalOffset` (* _return_coordinate _return_point_speed))
  (if (`/Game/Blueprint/Maps/timer.is goal` (`self.Timer`))
    (`self.K2_DestroyActor`)))

(event `self.ReceiveActorBeginOverlap`
  (params (OtherActor :type "Actor Object Reference"))
  (bind _is_goal (`/Game/Blueprint/Maps/timer.is goal` (`self.Timer`)))
  (if (and (not _is_goal) (`self.ActorHasTag` OtherActor "Player"))
    (`self.GetPoint`)
    (`self.K2_DestroyActor`)
    (elif _is_goal
      (`self.K2_DestroyActor`))))

(fn `CanBeObitained`
  (params (Pawn :type "Pawn Object Reference") (`Player Controller` :type "PlayerController Object Reference"))
  (returns (ReturnValue :type Boolean))
  (return (== (`self.GetLifeSpan` Pawn) 0.0)))

(fn `Get Coordinate`
  (returns (`Return Coordinate` :type "Vector Structure"))
  ;[1 1 1] Playerとのベクトルを出している
  (bind _newvar (`self.NewVar`)
    (:`then`
      (return (`KismetMathLibrary.Normal` (- (`self.K2_GetActorLocation` _newvar) (`self.K2_GetActorLocation` self)) 1e-05)))
    (:`else`)))

(fn `Get Point Speed`
  (returns (`Return Point Speed` :type "Float (double-precision)"))
  (bind _output_get (set `self.point speed` (* (`self.point speed`) 1.05)))
  (return _output_get))

(fn `GetPoint`
  ;[1 1 1] Pointを取得したらトータルポイントを追加する
  (bind _returnvalue (`GameplayStatics.GetActorOfClass` "/Game/Blueprint/Maps/BP_InGame_GameMode.BP_InGame_GameMode_C"))
  (bind _newpointnumber (`/Game/Blueprint/Maps/BP_InGame_GameMode.AddEnemyPoint` _returnvalue)))

(fn `UserConstructionScript`)