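; BP_point2 is a point pickup that flies toward the player and adds to the score on contact.
; BeginPlay captures the normalized direction to the player once, and Tick moves the actor along it as a local offset at PointSpeed, without homing or sweep.
; Overlapping an actor tagged Player calls GetPoint, which passes Number to GM_Point's AddPoint and prints the result, then destroys the pickup.
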(event `self.ReceiveBeginPlay`
  (set `self.Coordinate` (`KismetMathLibrary.Normal` (- (`self.K2_GetActorLocation` (`GameplayStatics.GetPlayerCharacter` 0)) (`self.K2_GetActorLocation` self)))))

(event `self.ReceiveTick`
  (params (DeltaSeconds :type "Float (single-precision)"))
  ;[1 1 1] 弾の移動する動き
  (`self.K2_AddActorLocalOffset` (* (`self.Coordinate`) (`self.point speed`))))

(event `self.ReceiveActorBeginOverlap`
  (params (OtherActor :type "Actor Object Reference"))
  (if (`self.ActorHasTag` OtherActor "Player")
    (`self.GetPoint`)
    (`self.K2_DestroyActor`)))

(fn `CanBeObitained`
  (params (Pawn :type "Pawn Object Reference") (`Player Controller` :type "PlayerController Object Reference"))
  (returns (ReturnValue :type Boolean))
  (return (== (`self.GetLifeSpan` Pawn) 0.0)))

(fn `GetPoint`
  ;[1 1 1] Pointを取得したらトータルポイントを追加する
  (bind _asgm_point (cast `/Game/Blueprint/point/GM_Point` (`GameplayStatics.GetGameMode`)))
  (bind _newpointnumber (`/Game/Blueprint/point/GM_Point.AddPoint` _asgm_point (`self.Number`)))
  (`KismetSystemLibrary.PrintString` (`KismetStringLibrary.Conv_IntToString` _newpointnumber)))

(fn `UserConstructionScript`)