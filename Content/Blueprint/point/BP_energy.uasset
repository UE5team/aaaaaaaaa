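; BP_energy is an energy pickup that turns into a point actor when the player collects it.
; On overlap with an actor tagged "Player", it calls GetPoint and then destroys itself.
; GetPoint spawns BP_point2 at the pickup's transform and plays a sound at its location.
; CanBeObitained is an empty stub, and BeginPlay, Tick and the construction script do nothing.
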(event `self.ReceiveActorBeginOverlap`
  (params (OtherActor :type "Actor Object Reference"))
  (if (`self.ActorHasTag` OtherActor "Player")
    (`self.GetPoint`)
    (`self.K2_DestroyActor`)))

(fn `CanBeObitained`
  (params (Pawn :type "Pawn Object Reference") (`Player Controller` :type "PlayerController Object Reference")))

(fn `GetPoint`
  ;[1 1 1] energyを取得したらPointを生成する
  (`|SpawnActorFromClass` "/Game/Blueprint/point/BP_point2.BP_point2_C" (`self.GetTransform`) "Undefined" "OverrideRootScale" null null)
  (`GameplayStatics.PlaySoundAtLocation` "/Game/Blueprint/point/決定ボタンを押す13.決定ボタンを押す13" (`self.K2_GetActorLocation`) (struct) 1.0 1.0 0.0 null null null null))

(fn `UserConstructionScript`)