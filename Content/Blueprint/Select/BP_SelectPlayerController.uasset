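; Player controller for the selection screen that turns Enhanced Input actions into character and weapon selection steps.
; BeginPlay hides the cursor, adds the selection mapping context and caches the BP_SelectWeaponCharacter.
; Increment and decrement, throttled by a short Delay, step BP_SelectHUD and update the decision index in BP_SelectGameMode.
; Decide and Back hide HUD visibility and move the game mode's widget index; Decide also sets the weapon, Back refocuses the widget.
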(event `self.ReceiveBeginPlay`
  (bind _returnvalue (`GameplayStatics.GetPlayerController` 0))
  (bind _returnvalue_2 (`GameplayStatics.GetPlayerController` 0))
  (bind _returnvalue_3 (pcsubsystem `EnhancedInputLocalPlayerSubsystem` _returnvalue))
  (`WidgetBlueprintLibrary.SetInputMode_GameAndUIEx` _returnvalue_2 null)
  (set `PlayerController.bShowMouseCursor` false _returnvalue_2)
  (bind _returnvalue_4 (`GameplayStatics.GetActorOfClass` "/Game/Blueprint/Player/BP_SelectWeaponCharacter.BP_SelectWeaponCharacter_C"))
  (set `self.SelectWeaponCharactor` _returnvalue_4)
  ;[1 1 1] コメント
  (`/Engine/EditorBlueprintResources/StandardMacros.IsValid` _returnvalue_3
    (:`Is Valid`
      (`EnhancedInputSubsystemInterface.AddMappingContext` _returnvalue_3 "/Game/Input/CharacterSelection/IMC_CharacterSelection.IMC_CharacterSelection" 0 (struct))
      (`self.EnableInput` _returnvalue))))

(event `EnhancedInput|/Game/Input/CharacterSelection/IA_Charactor_Decrement`
  (params (ActionValue :type Boolean) (ElapsedSeconds :type "Float (double-precision)") (TriggeredSeconds :type "Float (double-precision)") (InputAction :type "InputAction Object Reference" :default "/Game/Input/CharacterSelection/IA_Charactor_Decrement.IA_Charactor_Decrement"))
  (:`Triggered`
    ;[1 1 1] デクリメントを実行する
    (`KismetSystemLibrary.Delay` 0.3)
    (bind _returnvalue (`GameplayStatics.GetActorOfClass` "/Game/Blueprint/Select/BP_SelectHUD.BP_SelectHUD_C"))
    (`/Game/Blueprint/Select/BP_SelectHUD.Decrement` _returnvalue)
    (bind _returnvalue_2 (`GameplayStatics.GetActorOfClass` "/Game/Blueprint/Select/BP_SelectGameMode.BP_SelectGameMode_C"))
    (`/Game/Blueprint/Select/BP_SelectGameMode.Set Decision Index` _returnvalue_2)))

(event `EnhancedInput|/Game/Input/CharacterSelection/IA_Charactor_Increment`
  (params (ActionValue :type Boolean) (ElapsedSeconds :type "Float (double-precision)") (TriggeredSeconds :type "Float (double-precision)") (InputAction :type "InputAction Object Reference" :default "/Game/Input/CharacterSelection/IA_Charactor_Increment.IA_Charactor_Increment"))
  (:`Triggered`
    ;[1 1 1] インクリメントを実行する
    (`KismetSystemLibrary.Delay` 0.3)
    (bind _returnvalue (`GameplayStatics.GetActorOfClass` "/Game/Blueprint/Select/BP_SelectHUD.BP_SelectHUD_C"))
    (`/Game/Blueprint/Select/BP_SelectHUD.Increment` _returnvalue)
    (bind _returnvalue_2 (`GameplayStatics.GetActorOfClass` "/Game/Blueprint/Select/BP_SelectGameMode.BP_SelectGameMode_C"))
    (`/Game/Blueprint/Select/BP_SelectGameMode.Set Decision Index` _returnvalue_2)))

(event `EnhancedInput|/Game/Input/CharacterSelection/IA_Decide`
  (params (ActionValue :type Boolean) (ElapsedSeconds :type "Float (double-precision)") (TriggeredSeconds :type "Float (double-precision)") (InputAction :type "InputAction Object Reference" :default "/Game/Input/CharacterSelection/IA_Decide.IA_Decide"))
  (:`Started`
    ;[1 1 1] 決定を実行する
    (bind _returnvalue (`GameplayStatics.GetActorOfClass` "/Game/Blueprint/Select/BP_SelectHUD.BP_SelectHUD_C"))
    (`/Game/Blueprint/Select/BP_SelectHUD.Set Visility Hidden` _returnvalue)
    (bind _returnvalue_2 (`GameplayStatics.GetActorOfClass` "/Game/Blueprint/Select/BP_SelectGameMode.BP_SelectGameMode_C"))
    (`/Game/Blueprint/Select/BP_SelectGameMode.Set Decision Index` _returnvalue_2)
    (`/Game/Blueprint/Select/BP_SelectGameMode.Increment Widget Index` _returnvalue_2)
    (bind _selectweaponcharactor (`self.SelectWeaponCharactor`)
      (:`then`
        (`/Game/Blueprint/Player/BP_SelectWeaponCharacter.SetWeapon` _selectweaponcharactor)
        (`/Game/Blueprint/Select/BP_SelectGameMode.Set Decision Index` _returnvalue_2))
      (:`else`))))

(event `EnhancedInput|/Game/Input/CharacterSelection/IA_Back`
  (params (ActionValue :type Boolean) (ElapsedSeconds :type "Float (double-precision)") (TriggeredSeconds :type "Float (double-precision)") (InputAction :type "InputAction Object Reference" :default "/Game/Input/CharacterSelection/IA_Back.IA_Back"))
  (:`Started`
    ;[1 1 1] ウィジェットインデックスを減らす
    (bind _returnvalue (`GameplayStatics.GetActorOfClass` "/Game/Blueprint/Select/BP_SelectHUD.BP_SelectHUD_C"))
    (`/Game/Blueprint/Select/BP_SelectHUD.Set Visility Hidden` _returnvalue)
    (bind _returnvalue_2 (`GameplayStatics.GetActorOfClass` "/Game/Blueprint/Select/BP_SelectGameMode.BP_SelectGameMode_C"))
    (`/Game/Blueprint/Select/BP_SelectGameMode.Decrement Widget Index` _returnvalue_2)
    (`/Game/Blueprint/Select/BP_SelectHUD.Set Focus Widget` _returnvalue)))

(fn `UserConstructionScript`)