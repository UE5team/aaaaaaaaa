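; Game mode for the selection screen, holding the current step and focused choice for character, equipment and course.
; Focus steps wrap around data table row counts, and equipment changes also update a weapon on BP_SelectManager's preview character (Weapon1 on increment, Weapon0 on decrement).
; It switches between selection and per-course BGM, and saves character and equipment indices to the game instance.
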(event `self.ReceiveBeginPlay`
  (`self.CreateSelectionBGM`)
  (`self.PlaySelectionBGM`)
  (set `self.Focus Index Array` (`|MakeArray` 0 0 0)))

(event `Set Decision Index`
  (params (`widget Index` :type Integer) (`Focus Indx` :type "Integer (by ref)"))
  (`KismetArrayLibrary.Array_Set` (`self.Focus Index Array`) `widget Index` `Focus Indx` true))

(fn `Create Selection SE`
  (bind _returnvalue (`GameplayStatics.CreateSound2D` "/Game/Sound/Select/拳銃をチャッと構える.拳銃をチャッと構える" 1.0 1.0 0.0 null))
  (set `self.SE` _returnvalue))

(fn `CreateSelectionBGM`
  (bind _returnvalue (`GameplayStatics.CreateSound2D` "/Game/Sound/Select/parabox_ver2_0.parabox_ver2_0" 1.0 1.0 0.0 null))
  (set `self.Slelct BGM` _returnvalue))

(fn `Decrement Chatacter Focus Index`
  (params (InputPin :type Integer))
  (returns (`Focus Index` :type Integer))
  (bind _returnvalue (- (`|GetArrayItem` (`self.Focus Index Array`) InputPin) 1))
  (if (>= _returnvalue 0)
    (bind _output_get (set `self.Focus Index` _returnvalue))
    (`KismetArrayLibrary.Array_Set` (`self.Focus Index Array`) 0 _output_get true)
    (else
      (bind _outrownames (`DataTableFunctionLibrary.GetDataTableRowNames` "/Game/PL/DT_Character_Parameters.DT_Character_Parameters"))
      (bind _output_get_2 (set `self.Focus Index` (- (`KismetArrayLibrary.Array_Length` _outrownames) 1)))
      (`KismetArrayLibrary.Array_Set` (`self.Focus Index Array`) 0 _output_get_2 true)))
  (return (`self.Focus Index`)))

(fn `Decrement Cource Focus Index`
  (params (InputPin :type Integer))
  (returns (`Focus Index` :type Integer))
  (bind _returnvalue (- (`|GetArrayItem` (`self.Focus Index Array`) InputPin) 1))
  (if (>= _returnvalue 0)
    (bind _output_get (set `self.Focus Index` _returnvalue))
    (`KismetArrayLibrary.Array_Set` (`self.Focus Index Array`) InputPin _output_get true)
    (else
      (bind _outrownames (`DataTableFunctionLibrary.GetDataTableRowNames` "/Game/PL/DT_SelectCource.DT_SelectCource"))
      (bind _output_get_2 (set `self.Focus Index` (- (`KismetArrayLibrary.Array_Length` _outrownames) 1)))
      (`KismetArrayLibrary.Array_Set` (`self.Focus Index Array`) InputPin _output_get_2 true)))
  (return (`self.Focus Index`)))

(fn `Decrement Focus index`
  (params (Selection :type Integer))
  (returns (NewParam :type Integer))
  (switch `int` Selection
    (:`0`
      (bind _focus_index (`self.Decrement Chatacter Focus Index` Selection))
      (return _focus_index))
    (:`1`
      (bind _focus_index_2 (`self.Derement Equip Focus Index` Selection))
      (return _focus_index_2))
    (:`2`
      (bind _focus_index_3 (`self.Decrement Cource Focus Index` Selection))
      (return _focus_index_3))))

(fn `Decrement Widget Index`
  (returns (Output_Get :type Integer))
  (bind _returnvalue (- (`self.Select Index`) 1))
  (if (>= _returnvalue 0)
    (bind _output_get (set `self.Select Index` _returnvalue))
    (return _output_get)))

(fn `Derement Equip Focus Index`
  (params (InputPin :type Integer))
  (returns (`Focus Index` :type Integer))
  (bind _returnvalue (- (`self.Focus Index`) 1))
  (`|ExecutionSequence`
    (:`then_0`
      (set `self.Focus Index` (`|GetArrayItem` (`self.Focus Index Array`) InputPin))
      (if (>= _returnvalue 0)
        (set `self.Focus Index` _returnvalue)
        (else
          (bind _outrownames (`DataTableFunctionLibrary.GetDataTableRowNames` "/Game/PL/DT_PL_EquipParameters.DT_PL_EquipParameters"))
          (set `self.Focus Index` (- (`KismetArrayLibrary.Array_Length` _outrownames) 1))))
      (`KismetArrayLibrary.Array_Set` (`self.Focus Index Array`) InputPin (`self.Focus Index`) true))
    (:`then_1`
      (bind _outrownames_2 (`DataTableFunctionLibrary.GetDataTableRowNames` "/Game/PL/DT_Equip.DT_Equip"))
      (bind _returnvalue_2 (`|GetDataTableRow` "/Game/PL/DT_Equip.DT_Equip" (`|GetArrayItem` _outrownames_2 (`self.Focus Index`)))
        (:`then`
          (bind _returnvalue_3 (`GameplayStatics.GetActorOfClass` "/Game/Blueprint/Select/BP_SelectManager.BP_SelectManager_C"))
          (bind _selectweaponcharactor (`/Game/Blueprint/Select/BP_SelectManager.SelectWeaponCharactor` _returnvalue_3)
            (:`then`
              (set `/Game/Blueprint/Player/BP_SelectWeaponCharacter.Weapon0` (`.武器番号_34_E6FC3BA041887FEE2711BAB2DF3332FA` (break `/Game/Blueprint/CharacterSelection/Structures/ST_Equip` _returnvalue_2)) _selectweaponcharactor))
            (:`else`
              _))
          (return (`self.Focus Index`)))))))

(fn `Get Focus Index`
  (params (`Widget Index` :type Integer))
  (returns (`Focus Index` :type Integer))
  (return (`|GetArrayItem` (`self.Focus Index Array`) `Widget Index`)))

(fn `Get MaxWidget Index`
  (returns (`Max Widget Index` :type Integer))
  (return (`self.Max Select Index`)))

(fn `Get Widget Index`
  (returns (`Widget Index` :type Integer))
  (return (`self.Select Index`)))

(fn `GetMaxCharacterStatus`
  (returns (`Max Character Status` :type "Float (double-precision)"))
  (return (`self.Max Character Status`)))

(fn `GetMaxEquipStatus`
  (returns (`Max Equip Status` :type "Float (double-precision)"))
  (return (`self.Max Equip Status`)))

(fn `Increment Character Focus Index`
  (params (InputPin :type Integer))
  (returns (`Focus Index` :type Integer))
  (bind _returnvalue (+ (`|GetArrayItem` (`self.Focus Index Array`) InputPin) 1))
  (bind _outrownames (`DataTableFunctionLibrary.GetDataTableRowNames` "/Game/PL/DT_Character_Parameters.DT_Character_Parameters"))
  (if (< _returnvalue (`KismetArrayLibrary.Array_Length` _outrownames))
    (bind _output_get (set `self.Focus Index` _returnvalue))
    (`KismetArrayLibrary.Array_Set` (`self.Focus Index Array`) 0 _output_get true)
    (else
      (bind _output_get_2 (set `self.Focus Index` 0))
      (`KismetArrayLibrary.Array_Set` (`self.Focus Index Array`) 0 _output_get_2 true)))
  (return (`self.Focus Index`)))

(fn `Increment Cource Focus Index`
  (params (InputPin :type Integer))
  (returns (`Focus Index` :type Integer))
  (bind _returnvalue (+ (`|GetArrayItem` (`self.Focus Index Array`) InputPin) 1))
  (bind _outrownames (`DataTableFunctionLibrary.GetDataTableRowNames` "/Game/PL/DT_SelectCource.DT_SelectCource"))
  (if (< _returnvalue (`KismetArrayLibrary.Array_Length` _outrownames))
    (bind _output_get (set `self.Focus Index` _returnvalue))
    (`KismetArrayLibrary.Array_Set` (`self.Focus Index Array`) InputPin _output_get true)
    (else
      (bind _output_get_2 (set `self.Focus Index` 0))
      (`KismetArrayLibrary.Array_Set` (`self.Focus Index Array`) InputPin _output_get_2 true)))
  (return (`self.Focus Index`)))

(fn `Increment Equip Focus Index`
  (params (InputPin :type Integer))
  (returns (`Focus Index` :type Integer))
  (bind _returnvalue (+ (`self.Focus Index`) 1))
  (`|ExecutionSequence`
    (:`then_0`
      (set `self.Focus Index` (`|GetArrayItem` (`self.Focus Index Array`) InputPin))
      (bind _outrownames (`DataTableFunctionLibrary.GetDataTableRowNames` "/Game/PL/DT_PL_EquipParameters.DT_PL_EquipParameters"))
      (if (< _returnvalue (`KismetArrayLibrary.Array_Length` _outrownames))
        (set `self.Focus Index` _returnvalue)
        (else
          (set `self.Focus Index` 0)))
      (`KismetArrayLibrary.Array_Set` (`self.Focus Index Array`) InputPin (`self.Focus Index`) true))
    (:`then_1`
      (bind _outrownames_2 (`DataTableFunctionLibrary.GetDataTableRowNames` "/Game/PL/DT_Equip.DT_Equip"))
      (bind _returnvalue_2 (`|GetDataTableRow` "/Game/PL/DT_Equip.DT_Equip" (`|GetArrayItem` _outrownames_2 (`self.Focus Index`)))
        (:`then`
          (bind _returnvalue_3 (`GameplayStatics.GetActorOfClass` "/Game/Blueprint/Select/BP_SelectManager.BP_SelectManager_C"))
          (set `/Game/Blueprint/Player/BP_SelectWeaponCharacter.Weapon1` (`.武器番号_34_E6FC3BA041887FEE2711BAB2DF3332FA` (break `/Game/Blueprint/CharacterSelection/Structures/ST_Equip` _returnvalue_2)) (`/Game/Blueprint/Select/BP_SelectManager.SelectWeaponCharactor` _returnvalue_3))
          (return (`self.Focus Index`)))))))

(fn `Increment Focus Index`
  (params (Index :type Integer))
  (returns (NewParam :type Integer))
  (switch `int` Index
    (:`0`
      (bind _focus_index (`self.Increment Character Focus Index` Index))
      (return _focus_index))
    (:`1`
      (bind _focus_index_2 (`self.Increment Equip Focus Index` Index))
      (return _focus_index_2))
    (:`2`
      (bind _focus_index_3 (`self.Increment Cource Focus Index` Index))
      (return _focus_index_3))))

(fn `Increment Widget Index`
  (returns (`Widget Index` :type Integer))
  (bind _output_get (set `self.Select Index` (+ (`self.Select Index`) 1)))
  (return _output_get))

(fn `Play Couece BGM`
  (`self.Stop BGM`)
  (bind _outrownames (`DataTableFunctionLibrary.GetDataTableRowNames` "/Game/PL/DT_SelectCource.DT_SelectCource"))
  (bind _returnvalue (`|GetDataTableRow` "/Game/PL/DT_SelectCource.DT_SelectCource" (`|GetArrayItem` _outrownames (`self.Focus Index`)))
    (:`then`
      (bind _returnvalue_2 (`GameplayStatics.CreateSound2D` (`.CorceBGM_39_A97D85B84A819D916CF1BEB2540AF359` (break `/Game/PL/ST_CourceSelectParameters` _returnvalue)) 1.0 1.0 0.0 null))
      (bind _output_get (set `self.CourceBGM` _returnvalue_2))
      (`AudioComponent.Play` _output_get 0.0))))

(fn `PlaySelectionBGM`
  (`AudioComponent.Play` (`self.Slelct BGM`) 0.0))

(fn `Save Focus Index`
  (bind _focus_index_array (`self.Focus Index Array`))
  (bind _gi_default (`/Game/Blueprint/System/FL_MyLibrary.Get GI_Default`))
  (`/Game/Blueprint/Maps/GI_Defolut.Set Focus Index` _gi_default (`|GetArrayItem` _focus_index_array) (`|GetArrayItem` _focus_index_array 1)))

(fn `Stop BGM`
  (bind _slelct_bgm (`self.Slelct BGM`)
    (:`then`
      (`AudioComponent.Stop` _slelct_bgm))
    (:`else`
      (bind _courcebgm (`self.CourceBGM`)
        (:`then`
          (`AudioComponent.Stop` _courcebgm))
        (:`else`)))))

(fn `Stop Cource And Play Select BGM`
  (`AudioComponent.Stop` (`self.CourceBGM`))
  (`self.CreateSelectionBGM`)
  (`self.PlaySelectionBGM`))

(fn `UserConstructionScript`)