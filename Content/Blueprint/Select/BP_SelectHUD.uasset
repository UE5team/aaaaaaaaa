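; HUD for the selection screen, covering character, equipment and course selection.
; On BeginPlay it gets the select-mode, ready and course-select widgets from a widget creator, adds them to the viewport with only select mode left unhidden, then initializes it.
; Wrapper functions forward animations, visibility and status updates to those widgets, while WidgetArray helpers focus by BP_SelectGameMode's index.
; Course updates also push the DT_SelectCource row's type to BP_CourceManager.
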(event `self.ReceiveBeginPlay`
  (`|ExecutionSequence`
    (:`then_0`
      (bind _wbp_new_select_mode (`/Game/Blueprint/System/BP_WidgetCreater.Get WBP_New Select Mode` (`/Game/Blueprint/System/FL_MyLibrary.getWidgetCreator`)))
      (bind _output_get (set `self.WBP Select Mode` _wbp_new_select_mode))
      (`UserWidget.AddToViewport` _output_get 0)
      (bind _wbp_ready (`/Game/Blueprint/System/BP_WidgetCreater.Get WBP Ready` (`/Game/Blueprint/System/FL_MyLibrary.getWidgetCreator`)))
      (bind _output_get_2 (set `self.Ready` _wbp_ready))
      (`Widget.SetVisibility` _output_get_2 "Hidden")
      (`UserWidget.AddToViewport` _output_get_2 0)
      (bind _wbp_corceselect (`/Game/Blueprint/System/BP_WidgetCreater.Get WBP_CorceSelect` (`/Game/Blueprint/System/FL_MyLibrary.getWidgetCreator`)))
      (bind _output_get_3 (set `self.WBP Corce Select` _wbp_corceselect))
      (`Widget.SetVisibility` _output_get_3 "Hidden")
      (`UserWidget.AddToViewport` _output_get_3 0))
    (:`then_1`
      (`/Game/Blueprint/CharacterSelection/WBP/Select/WBP_newSelectMode.Init` (`self.WBP Select Mode`)))))

(event `self.ReceiveTick`
  (params (DeltaSeconds :type "Float (single-precision)")))

(fn `Cource Decrement Animation`
  (`/Game/Blueprint/CharacterSelection/WBP/Cource/WBP_SelectCourceList.Play Decrement Animation` (`/Game/Blueprint/CharacterSelection/WBP/Cource/WBP_CourceSelect.WBP_SelectCourceImage1` (`self.WBP Corce Select`))))

(fn `Cource Increment Animation`
  (`/Game/Blueprint/CharacterSelection/WBP/Cource/WBP_SelectCourceList.Play Increment Animation` (`/Game/Blueprint/CharacterSelection/WBP/Cource/WBP_CourceSelect.WBP_SelectCourceImage1` (`self.WBP Corce Select`))))

(fn `Decrement Character`)

(fn `Get Widget`
  (params (Index :type Integer))
  (returns (Widget :type "UserWidget Object Reference"))
  (return (`|GetArrayItem` (`self.Widget Array`) Index)))

(fn `Get Widget Index`
  (returns (Indexx :type Integer))
  (bind _returnvalue (`GameplayStatics.GetActorOfClass` "/Game/Blueprint/Select/BP_SelectGameMode.BP_SelectGameMode_C"))
  (bind _widget_index (`/Game/Blueprint/Select/BP_SelectGameMode.Get Widget Index` _returnvalue))
  (return _widget_index))

(fn `GetWidgetArray`
  (returns (NewParam :type "Array of UserWidget Object Reference"))
  (return (`self.Widget Array`)))

(fn `Go animation`
  (`/Game/Blueprint/CharacterSelection/WBP/Cource/WBP_CourceSelect.Play Cource Decition Animation` (`self.WBP Corce Select`))
  (`/Game/Blueprint/CharacterSelection/WBP/Select/WBP_newSelectMode.Init` (`self.WBP Select Mode`)))

(fn `Increment Character`
  (params (`Dimension 1` :type Integer))
  (bind _wbp_select_mode (`self.WBP Select Mode`)
    (:`then`
      (`/Game/Blueprint/CharacterSelection/WBP/Character/WD_CharacterParameter.Update Status` (`/Game/Blueprint/CharacterSelection/WBP/Character/WD_ChaaracterSelect.WD_CharacterParameter` (`/Game/Blueprint/CharacterSelection/WBP/Select/WBP_newSelectMode.WD_ChaaracterSelect` _wbp_select_mode)) `Dimension 1`))
    (:`else`)))

(fn `IsVisible`
  (params (Index :type Integer))
  (returns (NewParam :type Boolean))
  (bind _widget (`self.Get Widget` Index))
  (return (`|EnumEquality` (`Widget.Visibility` _widget) "Visible")))

(fn `Remove Widget Array`
  (bind _newparam (`self.GetWidgetArray`))
  (for _index (range (+ (`KismetArrayLibrary.Array_LastIndex` _newparam) 1))
    (`Widget.RemoveFromParent` (`|GetArrayItem` _newparam _index))))

(fn `Run the Back Animation`
  (bind _wbp_select_mode (`self.WBP Select Mode`)
    (:`then`
      (`/Game/Blueprint/CharacterSelection/WBP/Select/WBP_newSelectMode.Run the Back` _wbp_select_mode))
    (:`else`)))

(fn `Run the Decision Animation`
  (bind _wbp_select_mode (`self.WBP Select Mode`)
    (:`then`
      (`/Game/Blueprint/CharacterSelection/WBP/Select/WBP_newSelectMode.Run the Decision` _wbp_select_mode))
    (:`else`)))

(fn `Set Focus Widget`
  (bind _indexx (`self.Get Widget Index`))
  (bind _widget (`self.Get Widget` _indexx))
  (`Widget.SetVisibility` _widget "Visible"))

(fn `Set Visility Hidden`
  (params (`Widget Index` :type Integer))
  (bind _widget (`self.Get Widget` `Widget Index`))
  (`Widget.SetVisibility` _widget "Hidden"))

(fn `Show Select Widget`
  (params (InVisibility :type "ESlateVisibility Enum" :default "Visible"))
  (`Widget.SetVisibility` (`self.WBP Select Mode`) InVisibility))

(fn `Show WBP Corce Select`
  (params (InVisibility :type "ESlateVisibility Enum" :default "Visible"))
  (`Widget.SetVisibility` (`self.WBP Corce Select`) InVisibility))

(fn `Update Cource Slect`
  (params (`Dimension 1` :type Integer))
  (`/Game/Blueprint/CharacterSelection/WBP/Cource/WBP_CourceSelect.UpDate_CourceSelect` (`self.WBP Corce Select`) `Dimension 1`)
  (bind _outrownames (`DataTableFunctionLibrary.GetDataTableRowNames` "/Game/PL/DT_SelectCource.DT_SelectCource"))
  (bind _returnvalue (`|GetDataTableRow` "/Game/PL/DT_SelectCource.DT_SelectCource" (`|GetArrayItem` _outrownames `Dimension 1`))
    (:`then`
      (bind _returnvalue_2 (`GameplayStatics.GetActorOfClass` "/Game/Blueprint/System/BP_CourceManager.BP_CourceManager_C"))
      (`/Game/Blueprint/System/BP_CourceManager.SetCourceType` _returnvalue_2 (`.ECource_24_8A7FC85141E85845C4A7918DD29635B9` (break `/Game/PL/ST_CourceSelectParameters` _returnvalue))))))

(fn `UpDateCharacter`
  (params (InputPin :type Integer))
  (bind _wbp_select_mode (`self.WBP Select Mode`)
    (:`then`
      (`/Game/Blueprint/CharacterSelection/WBP/Character/WD_CharacterParameter.Update Status` (`/Game/Blueprint/CharacterSelection/WBP/Character/WD_ChaaracterSelect.WD_CharacterParameter` (`/Game/Blueprint/CharacterSelection/WBP/Select/WBP_newSelectMode.WD_ChaaracterSelect` _wbp_select_mode)) InputPin))
    (:`else`)))

(fn `UpdateEquipStatus`
  (params (NewVar :type Name))
  (bind _wbp_select_mode (`self.WBP Select Mode`)
    (:`then`
      (`/Game/Blueprint/CharacterSelection/WBP/Equip/WBP_EquipParameter.UpdateStatus` (`/Game/Blueprint/CharacterSelection/WBP/Equip/WD_EquipSelect.WD_Parameter_2` (`/Game/Blueprint/CharacterSelection/WBP/Select/WBP_newSelectMode.WD_EquipSelect2` _wbp_select_mode)) (`KismetTextLibrary.Conv_NameToText` NewVar)))
    (:`else`)))

(fn `UserConstructionScript`)