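; Manager actor for the character and equipment selection screens that lead into a course.
; Increment, decrement, decision and back functions update indices in BP_SelectGameMode and drive BP_SelectHUD.
; Cycling also stores equipment stats in the game instance and refreshes the preview character's weapon.
; OpenNextLevel tears down the selection actors, input and widgets once, and loads the level matching mode and course; its only call here is in disconnected legacy nodes.
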(event `self.ReceiveBeginPlay`
  (bind _newparam (`/Game/Blueprint/System/FL_MyLibrary.Get GI_Default`))
  (`/Game/Blueprint/Maps/GI_Defolut.Init Select` _newparam)
  (bind _returnvalue (`GameplayStatics.GetActorOfClass` "/Game/Blueprint/Player/BP_SelectWeaponCharacter.BP_SelectWeaponCharacter_C"))
  (set `self.SelectWeaponCharactor` _returnvalue))

(fn `Open Next Level`
  (locals (CourceTypeNum :type Integer) (BP_Level_Manager :type "/Game/Blueprint/System/BP_LevelManager Object Reference"))
  (bind _bp_level_manager (`local.BP_Level_Manager`))
  (bind _bp_level_manager_2 (`local.BP_Level_Manager`))
  (bind _bp_level_manager_3 (`local.BP_Level_Manager`))
  ;[1 1 1] コメント
  (`/Engine/EditorBlueprintResources/StandardMacros.DoOnce` false
    (:`Completed`
      (bind _newparam (`/Game/Blueprint/System/FL_MyLibrary.Get GI_Default`))
      (`/Game/Blueprint/Maps/GI_Defolut.Get magnification status` _newparam)
      ;[1 1 1] コメント
      (bind _returnvalue (`GameplayStatics.GetActorOfClass` "/Game/Blueprint/Select/BP_SelectGameMode.BP_SelectGameMode_C"))
      (`/Game/Blueprint/Select/BP_SelectGameMode.StopSelectionBGM` _returnvalue)
      (`EnhancedInputSubsystemInterface.RemoveMappingContext` (pcsubsystem `EnhancedInputLocalPlayerSubsystem` (`GameplayStatics.GetPlayerController` 0)) "/Game/Input/Title/IMC_Title.IMC_Title" (struct))
      (`WidgetLayoutLibrary.RemoveAllWidgets`)
      ;[1 1 1] 選択画面のコントロールコンテキストを削除する
      (bind _returnvalue_2 (`GameplayStatics.GetActorOfClass` "/Game/Blueprint/Select/BP_SelectPlayerController.BP_SelectPlayerController_C"))
      (`/Game/Blueprint/Select/BP_SelectPlayerController.Remove Selection Controller` _returnvalue_2)
      (bind _returnvalue_3 (`GameplayStatics.GetActorOfClass` "/Game/Blueprint/System/BP_CourceManager.BP_CourceManager_C"))
      (set `local.CourceTypeNum` (`/Game/Blueprint/System/BP_CourceManager.getCourceTypeNum` _returnvalue_3))
      (bind _returnvalue_4 (`GameplayStatics.GetActorOfClass` "/Game/Blueprint/System/BP_LevelManager.BP_LevelManager_C"))
      (bind _output_get (set `local.BP_Level_Manager` _returnvalue_4))
      (switch `int` (`/Game/Blueprint/System/BP_LevelManager.SelectModeType` _output_get)
        (:`0`
          (switch `int` (`local.CourceTypeNum`)
            (:`0`
              (`/Game/Blueprint/System/BP_LevelManager.SetupLoad` _bp_level_manager_2 "Mode_Destroy_Cource0"))
            (:`1`
              (`/Game/Blueprint/System/BP_LevelManager.SetupLoad` _bp_level_manager_2 "Mode_Destroy_Cource1"))
            (:`2`
              (`/Game/Blueprint/System/BP_LevelManager.SetupLoad` _bp_level_manager_2 "Mode_Destroy_Cource2"))))
        (:`1`
          (switch `int` (`local.CourceTypeNum`)
            (:`0`
              (`/Game/Blueprint/System/BP_LevelManager.SetupLoad` _bp_level_manager_3 "Mode_Original_Cource0"))
            (:`1`
              (`/Game/Blueprint/System/BP_LevelManager.SetupLoad` _bp_level_manager_3 "Mode_Original_Cource1"))
            (:`2`
              (`/Game/Blueprint/System/BP_LevelManager.SetupLoad` _bp_level_manager_3 "Mode_Original_Cource2"))))
        (:`2`
          (switch `int` (`local.CourceTypeNum`)
            (:`0`
              (`/Game/Blueprint/System/BP_LevelManager.SetupLoad` _bp_level_manager "Mode_TimeAttack_Cource0"))
            (:`1`
              (`/Game/Blueprint/System/BP_LevelManager.SetupLoad` _bp_level_manager "Mode_TimeAttack_Cource1"))
            (:`2`
              (`/Game/Blueprint/System/BP_LevelManager.SetupLoad` _bp_level_manager "Mode_TimeAttack_Cource2")))))
      (bind _returnvalue_5 (`GameplayStatics.GetActorOfClass` "/Game/Blueprint/Select/BP_SelectGameMode.BP_SelectGameMode_C"))
      (`self.K2_DestroyActor` _returnvalue_5)
      (bind _returnvalue_6 (`GameplayStatics.GetActorOfClass` "/Game/Blueprint/Select/BP_SelectHUD.BP_SelectHUD_C"))
      (`self.K2_DestroyActor` _returnvalue_6)
      (bind _returnvalue_7 (`GameplayStatics.GetActorOfClass` "/Game/Blueprint/Select/BP_SelectPlayerController.BP_SelectPlayerController_C"))
      (`self.K2_DestroyActor` _returnvalue_7)
      (`self.K2_DestroyActor`))))

(fn `Run the Back`
  ;[1 1 1] 今表示されている選択画面の番号を獲得する
  (bind _returnvalue (`GameplayStatics.GetActorOfClass` "/Game/Blueprint/Select/BP_SelectGameMode.BP_SelectGameMode_C"))
  (bind _widget_index (`/Game/Blueprint/Select/BP_SelectGameMode.Get Widget Index` _returnvalue))
  (bind _output_get (set `self.Select Index` _widget_index))
  (if (> _output_get 0)
    (bind _returnvalue_2 (`GameplayStatics.GetActorOfClass` "/Game/Blueprint/Select/BP_SelectHUD.BP_SelectHUD_C"))
    (if (== (`self.Select Index`) 1)
      (`/Game/Blueprint/Select/BP_SelectHUD.Run the Decrement Phase Index` _returnvalue_2))
    ;[1 1 1] 表示する選択画面の番号をデクリメントする
    (bind _returnvalue_3 (`GameplayStatics.GetActorOfClass` "/Game/Blueprint/Select/BP_SelectGameMode.BP_SelectGameMode_C"))
    (bind _output_get_2 (`/Game/Blueprint/Select/BP_SelectGameMode.Decrement Widget Index` _returnvalue_3))
    (set `self.Select Index` _output_get_2)
    (`/Game/Blueprint/Select/BP_SelectHUD.Select Equip Back` _returnvalue_2)
    (`/Game/Blueprint/Select/BP_SelectHUD.Show Ready Widget` _returnvalue_2 "Hidden")))

(fn `Run the Decision`
  (bind _select_index (`self.Select Index`))
  (if (<= (`self.Select Index`) 4)
    (bind _returnvalue (`GameplayStatics.GetActorOfClass` "/Game/Blueprint/Select/BP_SelectGameMode.BP_SelectGameMode_C"))
    (`/Game/Blueprint/Select/BP_SelectGameMode.Set Decision Index` _returnvalue _select_index (`self.Focus Index`))
    (bind _returnvalue_2 (`GameplayStatics.GetActorOfClass` "/Game/Blueprint/Select/BP_SelectHUD.BP_SelectHUD_C"))
    (if (== _select_index 0)
      (`/Game/Blueprint/Select/BP_SelectHUD.Run the Increment Phase Index` _returnvalue_2))
    ;[1 1 1] 表示する選択画面の番号をインクリメントする
    (bind _widget_index (`/Game/Blueprint/Select/BP_SelectGameMode.Increment Widget Index` _returnvalue))
    (bind _output_get (set `self.Select Index` _widget_index))
    (if (<= _output_get 3)
      (`/Game/Blueprint/Select/BP_SelectHUD.SelectEquipDecision` _returnvalue_2)
      ;[1 1 1] GameModeでフォーカスインデックスを保存する
      (`/Game/Blueprint/Select/BP_SelectGameMode.Set Decision Index` _returnvalue (`self.Select Index`) (`self.Default Focus Index`))
      ;[1 1 1] キャラクターに武器をつける
      (bind _selectweaponcharactor (`self.SelectWeaponCharactor`)
        (:`then`
          (`/Game/Blueprint/Player/BP_SelectWeaponCharacter.SetWeapon` _selectweaponcharactor))
        (:`else`))
      (elif (<= (`self.Select Index`) 4)
        (`/Game/Blueprint/Select/BP_SelectHUD.Show Ready Widget` _returnvalue_2 "Visible")
        (else
          (`/Game/Blueprint/Select/BP_SelectHUD.Go animation` _returnvalue_2))))))

(fn `Run the decrement`
  ;[1 1 1] 今表示されている選択画面の番号を獲得する
  (bind _returnvalue (`GameplayStatics.GetActorOfClass` "/Game/Blueprint/Select/BP_SelectGameMode.BP_SelectGameMode_C"))
  (bind _widget_index (`/Game/Blueprint/Select/BP_SelectGameMode.Get Widget Index` _returnvalue))
  (set `self.Select Index` _widget_index)
  ;[1 1 1] HUDで現在の選択ウィジェットのデクリメントを実行する
  (bind _returnvalue_2 (`GameplayStatics.GetActorOfClass` "/Game/Blueprint/Select/BP_SelectGameMode.BP_SelectGameMode_C"))
  (bind _newparam (`/Game/Blueprint/Select/BP_SelectGameMode.Decrement Focus index` _returnvalue_2 (`self.Select Index`)))
  (set `self.Focus Index` _newparam)
  ;[1 1 1] キャラクター選択画面でのインクリメントの処理をする
  (if (== (`self.Select Index`) 0)
    (bind _returnvalue_3 (`GameplayStatics.GetActorOfClass` "/Game/Blueprint/Select/BP_SelectHUD.BP_SelectHUD_C"))
    (`/Game/Blueprint/Select/BP_SelectHUD.Decrement Character` _returnvalue_3))
  ;[1 1 1] GameModeでフォーカスインデックスを保存する
  (bind _returnvalue_4 (`GameplayStatics.GetActorOfClass` "/Game/Blueprint/Select/BP_SelectHUD.BP_SelectHUD_C"))
  (`/Game/Blueprint/Select/BP_SelectHUD.Set Widget` _returnvalue_4 (`self.Select Index`))
  ;[1 1 1] 選択されているアイテムからステータスを読み取ってステータスを一旦保存している
  (bind _newparam_2 (`/Game/Blueprint/System/FL_MyLibrary.Get GI_Default`))
  (`/Game/Blueprint/Maps/GI_Defolut.SetEquipStatus` _newparam_2 (`self.Select Index`) (`self.Focus Index`))
  ;[1 1 1] キャラクターに武器をつける
  (bind _selectweaponcharactor (`self.SelectWeaponCharactor`)
    (:`then`
      (`/Game/Blueprint/Player/BP_SelectWeaponCharacter.SetWeapon` _selectweaponcharactor))
    (:`else`)))

(fn `Run the increment`
  ;[1 1 1] 今表示されている選択画面の番号を獲得する
  (bind _returnvalue (`GameplayStatics.GetActorOfClass` "/Game/Blueprint/Select/BP_SelectGameMode.BP_SelectGameMode_C"))
  (bind _widget_index (`/Game/Blueprint/Select/BP_SelectGameMode.Get Widget Index` _returnvalue))
  (set `self.Select Index` _widget_index)
  ;[1 1 1] HUDで現在の選択ウィジェットのインクリメントを実行する
  (bind _returnvalue_2 (`GameplayStatics.GetActorOfClass` "/Game/Blueprint/Select/BP_SelectGameMode.BP_SelectGameMode_C"))
  (bind _newparam (`/Game/Blueprint/Select/BP_SelectGameMode.Increment Focus Index` _returnvalue_2 (`self.Select Index`)))
  (set `self.Focus Index` _newparam)
  ;[1 1 1] キャラクター選択画面でのインクリメントの処理をする
  (if (== (`self.Select Index`) 0)
    (bind _returnvalue_3 (`GameplayStatics.GetActorOfClass` "/Game/Blueprint/Select/BP_SelectHUD.BP_SelectHUD_C"))
    (`/Game/Blueprint/Select/BP_SelectHUD.Increment Character` _returnvalue_3))
  ;[1 1 1] GameModeでフォーカスインデックスを保存する
  (bind _returnvalue_4 (`GameplayStatics.GetActorOfClass` "/Game/Blueprint/Select/BP_SelectHUD.BP_SelectHUD_C"))
  (`/Game/Blueprint/Select/BP_SelectHUD.Set Widget` _returnvalue_4 (`self.Select Index`))
  ;[1 1 1] 選択されているアイテムからステータスを読み取ってステータスを一旦保存している
  (bind _newparam_2 (`/Game/Blueprint/System/FL_MyLibrary.Get GI_Default`))
  (`/Game/Blueprint/Maps/GI_Defolut.SetEquipStatus` _newparam_2 (`self.Select Index`) (`self.Focus Index`))
  ;[1 1 1] キャラクターに武器をつける
  (bind _selectweaponcharactor (`self.SelectWeaponCharactor`)
    (:`then`
      (`/Game/Blueprint/Player/BP_SelectWeaponCharacter.SetWeapon` _selectweaponcharactor))
    (:`else`)))

(fn `UserConstructionScript`)