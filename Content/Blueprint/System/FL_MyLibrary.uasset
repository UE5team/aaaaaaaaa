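; Blueprint function library of shared helpers for game instance, Enhanced Input and manager lookups.
; It returns the game instance cast to GI_Defolut and finds the title and level manager actors by class.
; Mapping context helpers add or remove contexts on player 0's Enhanced Input subsystem.
; A remove-all helper clears the title, mode select, character selection, in-game, pause, result and select screen contexts.
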(fn `Get GI_Default`
  (returns (`GI Default` :type "/Game/Blueprint/Maps/GI_Defolut Object Reference"))
  (bind _asgi_defolut (cast `/Game/Blueprint/Maps/GI_Defolut` (`GameplayStatics.GetGameInstance` null)))
  (return _asgi_defolut))

(fn `getLevelManager`
  (returns (`level manager` :type "/Game/Blueprint/System/BP_LevelManager Object Reference"))
  (bind _returnvalue (`GameplayStatics.GetActorOfClass` null "/Game/Blueprint/System/BP_LevelManager.BP_LevelManager_C"))
  (return _returnvalue))

(fn `getTitleManager`
  (returns (ReturnValue :type "/Game/Blueprint/Title/BP_TitleManager Object Reference"))
  (bind _returnvalue (`GameplayStatics.GetActorOfClass` null "/Game/Blueprint/Title/BP_TitleManager.BP_TitleManager_C"))
  (return _returnvalue))

(fn `RemoveAllMappingContext`
  (`|ExecutionSequence`
    (:`then_0`
      ;[1 1 1] Tilte
      (`self.RemoveMappingContext` "/Game/Input/Title/IMC_Title.IMC_Title")
      (`self.RemoveMappingContext` "/Game/Input/Title/IMC_ModeSelect.IMC_ModeSelect"))
    (:`then_1`
      ;[1 1 1] Select
      (`self.RemoveMappingContext` "/Game/Input/CharacterSelection/IMC_CharacterSelection.IMC_CharacterSelection"))
    (:`then_2`
      ;[1 1 1] InGame
      (`self.RemoveMappingContext` "/Game/Input/Player/IMC_MyDefault.IMC_MyDefault")
      (`self.RemoveMappingContext` "/Game/Input/Player/IMC_Pause.IMC_Pause"))
    (:`then_3`
      ;[1 1 1] Result
      (`self.RemoveMappingContext` "/Game/Blueprint/UI/result/IMC_Result.IMC_Result")
      (`self.RemoveMappingContext` "/Game/Blueprint/UI/result/IMC_SelectScreen.IMC_SelectScreen"))))

(fn `RemoveMappingContext`
  (params (SetContext :type "InputMappingContext Object Reference"))
  (`EnhancedInputSubsystemInterface.RemoveMappingContext` (pcsubsystem `EnhancedInputLocalPlayerSubsystem` (`GameplayStatics.GetPlayerController` null)) SetContext (struct)))

(fn `SetMappingContext`
  (params (InputMappingContext :type "InputMappingContext Object Reference") (Priority :type Integer))
  (`EnhancedInputSubsystemInterface.AddMappingContext` (pcsubsystem `EnhancedInputLocalPlayerSubsystem` (`GameplayStatics.GetPlayerController` null)) InputMappingContext Priority (struct)))