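; Central widget factory that pre-creates the game's UI widgets once at BeginPlay and holds references to them.
; Creation is split into per-screen functions for title, select, in-game, result and others such as fade and loading, each storing its widgets in variables.
; Getter functions expose each cached widget; nothing here adds them to the viewport.
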(event `self.ReceiveBeginPlay`
  (`|ExecutionSequence`
    (:`then_0`
      (`self.CreateTitleScreenWidget`))
    (:`then_1`
      (`self.CreateSelectScreenWidget`))
    (:`then_2`
      (`self.CreateIngameScreenWidget`))
    (:`then_3`
      (`self.CreateResultScreenWidget`))
    (:`then_4`
      (`self.CreateOthersWidget`))))

(fn `CreateIngameScreenWidget`
  (`|ExecutionSequence`
    (:`then_0`
      (bind _returnvalue (`|CreateWidget` "/Game/Blueprint/Maps/goal.goal_C"))
      (set `self.Goal` _returnvalue))
    (:`then_2`
      (bind _returnvalue_2 (`|CreateWidget` "/Game/Blueprint/Maps/UI_ReverseRunning.UI_ReverseRunning_C"))
      (set `self.UI_Reverse_Run` _returnvalue_2))
    (:`then_3`
      (bind _returnvalue_3 (`|CreateWidget` "/Game/Blueprint/Maps/BP_Ingame_UI.BP_Ingame_UI_C"))
      (set `self.BP IngameUI` _returnvalue_3))))

(fn `CreateOthersWidget`
  (`|ExecutionSequence`
    (:`then_0`
      (bind _returnvalue (`|CreateWidget` "/Game/Blueprint/Title/WBP_Fade.WBP_Fade_C"))
      (set `self.WBP_Fade` _returnvalue))
    (:`then_1`
      (bind _returnvalue_2 (`|CreateWidget` "/Game/GG/UI/Roading_UI/WBP_GG_Loading.WBP_GG_Loading_C"))
      (set `self.WBP_GG_Loading` _returnvalue_2))))

(fn `CreateResultScreenWidget`
  (`|ExecutionSequence`
    (:`then_0`
      (bind _returnvalue (`|CreateWidget` "/Game/Blueprint/Player/Pause_Menu_UI.Pause_Menu_UI_C"))
      (set `self.Pause Menu UI` _returnvalue))
    (:`then_1`
      (bind _returnvalue_2 (`|CreateWidget` "/Game/Blueprint/UI/result/UI_Total_points.UI_Total_points_C"))
      (set `self.UI Total Points` _returnvalue_2))
    (:`then_2`
      (bind _returnvalue_3 (`|CreateWidget` "/Game/Blueprint/UI/result/UI_ranking.UI_ranking_C"))
      (set `self.UI ranking` _returnvalue_3))
    (:`then_3`
      (bind _returnvalue_4 (`|CreateWidget` "/Game/Blueprint/UI/result/UI_result.UI_result_C"))
      (set `self.UI_result` _returnvalue_4))))

(fn `CreateSelectScreenWidget`
  (`|ExecutionSequence`
    (:`then_0`
      (bind _returnvalue (`|CreateWidget` "/Game/Blueprint/CharacterSelection/WBP/Select/WBP_newSelectMode.WBP_newSelectMode_C"))
      (set `self.WBP_New Select Mode` _returnvalue))
    (:`then_1`
      (bind _returnvalue_2 (`|CreateWidget` "/Game/Blueprint/CharacterSelection/WBP/Decision/WBP_Ready.WBP_Ready_C"))
      (set `self.WBP_Ready` _returnvalue_2))))

(fn `CreateTitleScreenWidget`
  (`|ExecutionSequence`
    (:`then_0`
      (bind _returnvalue (`|CreateWidget` "/Game/Blueprint/Title/WBP_Title.WBP_Title_C"))
      (set `self.WBP Title` _returnvalue))
    (:`then_1`
      (bind _returnvalue_2 (`|CreateWidget` "/Game/GG/UI/Mode_Selection_UI/WBP_GG_ModeSelection.WBP_GG_ModeSelection_C"))
      (set `self.WBP GG ModeSelection` _returnvalue_2))))

(fn `Get WBP Ready`
  (returns (WBP_Ready :type "/Game/Blueprint/CharacterSelection/WBP/Decision/WBP_Ready Object Reference"))
  (return (`self.WBP_Ready`)))

(fn `Get WBP Title`
  (returns (`WBP Title` :type "/Game/Blueprint/Title/WBP_Title Object Reference"))
  (return (`self.WBP Title`)))

(fn `Get WBP_New Select Mode`
  (returns (`WBP_New Select Mode` :type "/Game/Blueprint/CharacterSelection/WBP/Select/WBP_newSelectMode Object Reference"))
  (return (`self.WBP_New Select Mode`)))

(fn `getBP Ingame UI`
  (returns (`BP IngameUI` :type "/Game/Blueprint/Maps/BP_Ingame_UI Object Reference"))
  (return (`self.BP IngameUI`)))

(fn `getGoal`
  (returns (Goal :type "/Game/Blueprint/Maps/goal Object Reference"))
  (return (`self.Goal`)))

(fn `getPauseMenuUI`
  (returns (`Pause Menu UI` :type "/Game/Blueprint/Player/Pause_Menu_UI Object Reference"))
  (return (`self.Pause Menu UI`)))

(fn `getUI ranking`
  (returns (`UI ranking` :type "/Game/Blueprint/UI/result/UI_ranking Object Reference"))
  (return (`self.UI ranking`)))

(fn `getUI result`
  (returns (UI_result :type "/Game/Blueprint/UI/result/UI_result Object Reference"))
  (return (`self.UI_result`)))

(fn `getUI Reverse Run`
  (returns (UI_Reverse_Run :type "/Game/Blueprint/Maps/UI_ReverseRunning Object Reference"))
  (return (`self.UI_Reverse_Run`)))

(fn `getUI Total Points`
  (returns (`UI Total Points` :type "/Game/Blueprint/UI/result/UI_Total_points Object Reference"))
  (return (`self.UI Total Points`)))

(fn `getWBP Fade`
  (returns (WBP_Fade :type "/Game/Blueprint/Title/WBP_Fade Object Reference"))
  (return (`self.WBP_Fade`)))

(fn `getWBP GG ModeSelection`
  (returns (`WBP GG ModeSelection` :type "/Game/GG/UI/Mode_Selection_UI/WBP_GG_ModeSelection Object Reference"))
  (return (`self.WBP GG ModeSelection`)))

(fn `getWBP_GG_Loading`
  (returns (WBP_GG_Loading :type "/Game/GG/UI/Roading_UI/WBP_GG_Loading Object Reference"))
  (return (`self.WBP_GG_Loading`)))

(fn `UserConstructionScript`)