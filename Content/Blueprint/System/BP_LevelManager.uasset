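; BP_LevelManager is a Blueprint that holds state for level loading and exposes it through simple getters and setters.
; SetupLoad stores the next level and raises LoadFlag, which can also be read or set directly.
; A separate DoSetModeScreen flag has its own accessors.
; The Blueprint performs no loading itself, and its construction script is empty.
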(fn `GetDoSetModeScreen`
  (returns (Value :type Boolean))
  (return (`self.DoSetModeScreen`)))

(fn `GetLoadFlag`
  (returns (Flag :type Boolean))
  (return (`self.LoadFlag`)))

(fn `GetNextLevel`
  (returns (NextLevel :type Name))
  (return (`self.NextLevel`)))

(fn `SetDoSetModeScreen`
  (params (SetValue :type Boolean))
  (set `self.DoSetModeScreen` SetValue))

(fn `SetLoadFlag`
  (params (Flag :type Boolean))
  (set `self.LoadFlag` Flag))

(fn `SetupLoad`
  (params (NextLevel :type Name))
  (set `self.NextLevel` NextLevel)
  (set `self.LoadFlag` true))

(fn `UserConstructionScript`)