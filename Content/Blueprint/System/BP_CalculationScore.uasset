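; BP_CalculationScore grades the player's result on enemy kills, points and time, plus an overall rank.
; BeginPlay caches GIDefault and loads threshold, rank and score columns from DT_ScoreGraph into arrays.
; While CanCalculationScore is set, Tick takes the first threshold each stat meets, averages the rank scores for the overall grade, and refreshes rank texts.
; CheckRank can also return the individual and total scores.
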(event `self.ReceiveBeginPlay`
  (bind _gi_default (`/Game/Blueprint/System/FL_MyLibrary.Get GI_Default`))
  (set `self.GI Default` _gi_default)
  (bind _outrownames (`DataTableFunctionLibrary.GetDataTableRowNames` "/Game/PL/DT_ScoreGraph.DT_ScoreGraph"))
  (`self.SetCheckScoreGraph` _outrownames))

(event `self.ReceiveTick`
  (params (DeltaSeconds :type "Float (single-precision)"))
  (if (`self.CanCalculationScore`)
    (`self.CheckRank` false)
    (`self.SetOutputRankText`)))

(fn `CheckRank`
  (params (`Is GetScore` :type Boolean))
  (returns (RankScoreArray :type "Array of Integer"))
  (locals (NowCheckItemNum :type Integer) (EnemyDeathCountScoreBuf :type Integer) (PointScoreBuf :type Integer) (TimeScoreBuf :type Integer) (TotalScoreBuf :type Integer) (MAX_CHECK_ITEM :type Integer :default 3))
  (for _index (range (+ (`local.MAX_CHECK_ITEM`) 1))
    (bind _output_get (set `local.NowCheckItemNum` _index))
    (switch `int` _output_get
      (:`0`
        ;[1 1 1] 撃破した敵の数に対する評価をだす
        (for (_array_element _array_index) (`self.EnemyDeathCountCheckGraph`)
          (if (<= _array_element (`/Game/Blueprint/Maps/GI_Defolut.EnemyDeathCount` (`self.GI Default`)))
            (`KismetArrayLibrary.Array_Set` (`self.OutputRankNum`) (`local.NowCheckItemNum`) _array_index)
            (break))))
      (:`1`
        ;[1 1 1] ポイントに対する評価をだす
        (for (_array_element_2 _array_index_2) (`self.PointCheckGraph`)
          (if (<= _array_element_2 (`/Game/Blueprint/Maps/GI_Defolut.ViewPoint` (`self.GI Default`)))
            (`KismetArrayLibrary.Array_Set` (`self.OutputRankNum`) (`local.NowCheckItemNum`) _array_index_2)
            (break))))
      (:`2`
        ;[1 1 1] タイムに対する評価を出す
        (for (_array_element_3 _array_index_3) (`self.TimeCheckGraph`)
          (if (>= _array_element_3 (`/Game/Blueprint/Maps/GI_Defolut.Gi_msec` (`self.GI Default`)))
            (`KismetArrayLibrary.Array_Set` (`self.OutputRankNum`) (`local.NowCheckItemNum`) _array_index_3)
            (break)
            (else
              ;;[1 1 1] Eの時
              (if (== (`KismetArrayLibrary.Array_LastIndex` (`self.TimeCheckGraph`)) _array_index_3)
                (`KismetArrayLibrary.Array_Set` (`self.OutputRankNum`) (`local.NowCheckItemNum`) _array_index_3))))))
      (:`3`
        ;[1 1 1] 各チェック項目のランクに対する点数を保存
        (for _index_2 (range (`local.MAX_CHECK_ITEM`))
          (switch `int` _index_2
            (:`0`
              (bind _output (`|GetArrayItem` (`self.RankScoreGraph`) (`|GetArrayItem` (`self.OutputRankNum`) _index_2)))
              (set `local.EnemyDeathCountScoreBuf` _output))
            (:`1`
              (set `local.PointScoreBuf` _output))
            (:`2`
              (set `local.TimeScoreBuf` _output))))
        ;[1 1 1] 各項目のスコアの合計/項目数をRankScoreGraphを見て評価を出す
        (bind _output_get_2 (set `local.TotalScoreBuf` (+ (`local.EnemyDeathCountScoreBuf`) (`local.PointScoreBuf`) (`local.TimeScoreBuf`))))
        (for (_array_element_4 _array_index_4) (`self.RankScoreGraph`)
          (if (<= _array_element_4 (/ _output_get_2 (`local.MAX_CHECK_ITEM`)))
            (`KismetArrayLibrary.Array_Set` (`self.OutputRankNum`) (`local.NowCheckItemNum`) _array_index_4)
            (break))))
      (:`4`
        (if `Is GetScore`
          (return (`|MakeArray` (`local.EnemyDeathCountScoreBuf`) (`local.PointScoreBuf`) (`local.TimeScoreBuf`) (`local.TotalScoreBuf`))))))))

(fn `GetOutputRankText`
  (params (index :type Integer))
  (returns (Rank :type String))
  (return (`|GetArrayItem` (`self.OutputRankText`) index)))

(fn `SetCheckScoreGraph`
  (params (RowNames :type "Array of Name"))
  (for (_array_element _array_index) RowNames
    (bind _returnvalue (`|GetDataTableRow` "/Game/PL/DT_ScoreGraph.DT_ScoreGraph" _array_element)
      (:`then`
        (`KismetArrayLibrary.Array_Set` (`self.EnemyDeathCountCheckGraph`) _array_index (break `/Game/PL/ST_ScoreGraph` _returnvalue))
        (`KismetArrayLibrary.Array_Set` (`self.PointCheckGraph`) _array_index (`.ポイント_10_5E3AF5F5478CA80F13958E95547DDCAA` (break `/Game/PL/ST_ScoreGraph` _returnvalue)))
        (`KismetArrayLibrary.Array_Set` (`self.TimeCheckGraph`) _array_index (`.タイム_11_A963A74641D893458D8AD39B9235B28B` (break `/Game/PL/ST_ScoreGraph` _returnvalue)))
        (`KismetArrayLibrary.Array_Set` (`self.RankGraph`) _array_index (`.評価_8_B645F027422C544F05FB338BB47FBF3C` (break `/Game/PL/ST_ScoreGraph` _returnvalue)))
        (`KismetArrayLibrary.Array_Set` (`self.RankScoreGraph`) _array_index (`.点数_14_2C9B45A247DCB40EE6892489A9A1C0FF` (break `/Game/PL/ST_ScoreGraph` _returnvalue)))))))

(fn `SetOutputRankText`
  (for (_array_element _array_index) (`self.OutputRankNum`)
    (`KismetArrayLibrary.Array_Set` (`self.OutputRankText`) _array_index (`|GetArrayItem` (`self.RankGraph`) _array_element))))

(fn `UserConstructionScript`)