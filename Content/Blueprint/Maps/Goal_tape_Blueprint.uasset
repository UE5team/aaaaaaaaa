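; Goal tape actor that handles lap completion and the race finish.
; BeginPlay caches the game instance and polls each tick until the in-game UI's Timer is valid.
; The Goal event, also fired by a debug key, records lap times in the game instance, respawns enemies and road points, or finishes on the last lap.
; Box overlap only checks the player tag; checkpoint-based lap validation is disconnected.
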(event OnComponentBeginOverlap(Box)
  (params (OverlappedComponent :type Primitive%20Component%20Object%20Reference) (OtherActor :type Actor%20Object%20Reference) (OtherComp :type Primitive%20Component%20Object%20Reference) (OtherBodyIndex :type Integer) (bFromSweep :type Boolean) (SweepResult :type Hit%20Result%20Structure%20%28by%20ref%29))
  ;[1 1 1] Playerかどうか
  (if (Components|ComponentHasTag OtherComp "PlayerCollision")
    _))

(event Custom|Goal
  (params (lap%20input :type Integer))
  (bind _gi (Variables|Default|GetGi))
  (bind _gi_2 (Variables|Default|GetGi))
  (switch int (Variables|time|GetLap%20digit)
    (:1
      (Variables|time|SetIndex 0))
    (:2
      (Variables|time|SetIndex 1))
    (:3
      (Variables|time|SetIndex 2)))
  (if (>= lap%20input (Variables|time|GetLap%20digit))
    (bind _output_get (Variables|time|Setlap%20time (- (Variables|/Game/Blueprint/Maps/timer.timer_C|Getmsec (Variables|time|Gettimer)) (Variables|time|Getbefore%20time))))
    (Variables|time|Setbefore%20time (+ _output_get (Variables|time|Getbefore%20time)))
    ;[1 1 1] ゴールしていないか
    (if (< (Variables|time|GetLap%20digit) (.コースの周回数 (Utilities|Struct|BreakST_InGameParameters (Utilities|Struct|MakeST_InGameParameters 6.0))))
      ;[1 1 1] Lap可算
      (Variables|time|SetLap%20digit (+ (Variables|time|GetLap%20digit) 1))
      ;[1 1 1] タイム
      (Default|タイム計算 (Variables|Default|GetGi) (Variables|time|Getlap%20time))
      (Utilities|Array|SetArrayElem (Variables|/Game/Blueprint/Maps/GI_Defolut.GI_Defolut_C|GetGi_goal%20time _gi_2) (Variables|time|GetIndex) (Variables|/Game/Blueprint/Maps/GI_Defolut.GI_Defolut_C|GetGi_Saved%20time _gi_2))
      ;[1 1 1] 敵のデスポーンとスポーン
      (Default|ResetEnemy _gi)
      ;[1 1 1] ポイントのデスポーンとスポーン
      (Default|SpawnRoadPoint _gi)
      (else
        (Default|Goal (Variables|Default|GetGi))))))

(event EventBeginPlay
  (Input|EnableInput (Game|GetPlayerController 0)) ; デバッグ用
  (bind _asgi_defolut (Utilities|Casting|CastToGI_Defolut (Game|GetGameInstance)))
  (Variables|Default|SetGi _asgi_defolut)
  (bind _foundwidgets (Widget|GetAllWidgetsOfClass "/Game/Blueprint/Maps/BP_Ingame_UI.BP_Ingame_UI_C" true :!label _label))
  (Utilities|IsValid (Variables|/Game/Blueprint/Maps/BP_Ingame_UI.BP_Ingame_UI_C|Gettimer (Utilities|Array|Get(acopy) _foundwidgets))
    (:Is%20Valid
      (Variables|time|Settimer (Variables|/Game/Blueprint/Maps/BP_Ingame_UI.BP_Ingame_UI_C|Gettimer (Utilities|Array|Get(acopy) _foundwidgets))))
    (:Is%20Not%20Valid
      (Utilities|FlowControl|DelayUntilNextTick)
      (goto _label))))

(event Input|KeyboardEvents|DebugKey1
  (params (Key :type Key%20Structure :default "None") (ActionValue :type Input%20Action%20Value%20Structure))
  (:Pressed
    (CallFunction|Goal 10)))

(fn ConstructionScript)

(fn CheckGoalCondition
  (Utilities|FlowControl|Sequence
    (:then_0
      (for _index (range 0 (Variables|Default|GetLapCountPointLastIndex))
        (LocalVariables|SetNewLocalVar (Utilities|Array|Get(acopy) (Variables|Default|GetLapCountPoint) _index))
        (bind _newlocalvar (LocalVariables|GetNewLocalVar)
          (:then
            (if (Variables|/Game/Blueprint/Maps/BP_LapCountPoint.BP_LapCountPoint_C|GetIsLapFlag _newlocalvar)
              (Math|Integer|IncrementInt (LocalVariables|GetCount))))
          (:else))))
    (:then_1
      (return (== (Variables|Default|GetLapCountPointLength) (LocalVariables|GetCount))))))