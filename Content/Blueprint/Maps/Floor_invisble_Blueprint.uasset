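; Invisible floor actor that marks off-course areas and penalizes the player while they overlap its OverLapMesh.
; Overlap begin and end switch the player's walk speed (deferring to ACBoost while boosting) and toggle a Japanese course-out warning with a looping-style siren sound.
; Tick reports off-course points to the game mode until the Timer reaches goal.
; BeginPlay retries each tick until the player and both HUD widgets exist.
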(event `self.OverLapMesh.OnComponentBeginOverlap`
  (params (OverlappedComponent :type "PrimitiveComponent Object Reference") (OtherActor :type "Actor Object Reference") (OtherComp :type "PrimitiveComponent Object Reference") (OtherBodyIndex :type Integer) (bFromSweep :type Boolean) (SweepResult :type "HitResult Structure (by ref)"))
  (bind _ac_boost (`/Game/Blueprint/Player/BP_Player.AC_Boost` (`self.BP Player`)))
  (if (`self.ActorHasTag` OtherActor "player")
    (set `self.isOffCource` true)
    (if (`/Game/Blueprint/Player/AC_Boost.IsBoost` _ac_boost)
      (`/Game/Blueprint/Player/AC_Boost.Set_Boost_Speed` _ac_boost)
      (else
        (`self.SetCourceOutWalkSpeed`)))
    (bind _courseoutwarning (`self.CourseOutWarning`)
      (:`then`
        (set `/Game/Blueprint/Maps/Course_out_warning.warning text` "コースの外に出ています" _courseoutwarning)
        (bind _returnvalue (`GameplayStatics.CreateSound2D` "/Game/Sound/OtoLogic/Warning-Siren05-08_Slow-Single__Edited_Cue.Warning-Siren05-08_Slow-Single__Edited_Cue" 1.0 1.0 0.0 null))
        (`AudioComponent.Play` _returnvalue 0.0))
      (:`else`))))

(event `self.OverLapMesh.OnComponentEndOverlap`
  (params (OverlappedComponent :type "PrimitiveComponent Object Reference") (OtherActor :type "Actor Object Reference") (OtherComp :type "PrimitiveComponent Object Reference") (OtherBodyIndex :type Integer))
  (bind _ac_boost (`/Game/Blueprint/Player/BP_Player.AC_Boost` (`self.BP Player`)))
  (if (`self.ActorHasTag` OtherActor "player")
    (set `self.isOffCource` false)
    (if (`/Game/Blueprint/Player/AC_Boost.IsBoost` _ac_boost)
      (`/Game/Blueprint/Player/AC_Boost.Set_Boost_Speed` _ac_boost)
      (else
        (`self.SetDefultWalkSpeed`)))
    (bind _courseoutwarning (`self.CourseOutWarning`)
      (:`then`
        (set `/Game/Blueprint/Maps/Course_out_warning.warning text` "  " _courseoutwarning)
        (`/Engine/EditorBlueprintResources/StandardMacros.IsValid` (stale `self.OverLapMesh.OnComponentBeginOverlap` _returnvalue)
          (:`Is Valid`
            (`AudioComponent.Stop` (stale `self.OverLapMesh.OnComponentBeginOverlap` _returnvalue)))))
      (:`else`))))

(event `self.ReceiveBeginPlay`
  (bind _returnvalue (`GameplayStatics.GetActorOfClass` "/Game/Blueprint/Maps/BP_InGame_GameMode.BP_InGame_GameMode_C"))
  (set `self.BP_Ingame_GameMode` _returnvalue)
  (bind _returnvalue_2 (`GameplayStatics.GetActorOfClass` "/Game/Blueprint/Player/BP_Player.BP_Player_C" :!label _label))
  (bind _output_get (set `self.BP Player` _returnvalue_2))
  (`/Engine/EditorBlueprintResources/StandardMacros.IsValid` _output_get
    (:`Is Valid`
      (bind _foundwidgets (`WidgetBlueprintLibrary.GetAllWidgetsOfClass` "/Game/Blueprint/Maps/timer.timer_C" :!label _label_2))
      (bind _output_get_2 (set `self.Timer` (`|GetArrayItem` _foundwidgets)))
      (`/Engine/EditorBlueprintResources/StandardMacros.IsValid` _output_get_2
        (:`Is Valid`
          (bind _foundwidgets_2 (`WidgetBlueprintLibrary.GetAllWidgetsOfClass` "/Game/Blueprint/Maps/Course_out_warning.Course_out_warning_C" :!label _label_3))
          (bind _output_get_3 (set `self.CourseOutWarning` (`|GetArrayItem` _foundwidgets_2)))
          (`/Engine/EditorBlueprintResources/StandardMacros.IsValid` _output_get_3
            (:`Is Not Valid`
              (`KismetSystemLibrary.DelayUntilNextTick`)
              (goto _label_3))))
        (:`Is Not Valid`
          (`KismetSystemLibrary.DelayUntilNextTick`)
          (goto _label_2))))
    (:`Is Not Valid`
      (`KismetSystemLibrary.DelayUntilNextTick`)
      (goto _label))))

(event `self.ReceiveTick`
  (params (DeltaSeconds :type "Float (single-precision)"))
  (`/Engine/EditorBlueprintResources/StandardMacros.IsValid` (`self.Timer`)
    (:`Is Valid`
      (if (`self.isOffCource`)
        (if (not (`/Game/Blueprint/Maps/timer.is goal` (`self.Timer`)))
          (`/Game/Blueprint/Maps/BP_InGame_GameMode.PointsGoingOutside` (`self.BP_Ingame_GameMode`) (`self.Course out point`)))))))

(fn `SetCourceOutWalkSpeed`
  (set `CharacterMovementComponent.MaxWalkSpeed` (`self.OffCourceMaxWalkSpeed`) (`Character.CharacterMovement` (`self.BP Player`))))

(fn `SetDefultWalkSpeed`
  (bind _bp_player (`self.BP Player`))
  (set `CharacterMovementComponent.MaxWalkSpeed` (`/Game/Blueprint/Player/BP_Player.DefaultMax Walk Speed` _bp_player) (`Character.CharacterMovement` _bp_player)))

(fn `UserConstructionScript`)