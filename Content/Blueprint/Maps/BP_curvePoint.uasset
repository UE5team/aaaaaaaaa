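; Map trigger actor that shows and hides a left or right curve icon on the WB_curve HUD widget as the player passes.
; BeginPlay caches the first top-level WB_curve found.
; When a PlayerCollision component leaves either Second volume, it shows the hidden icon using IsRight; leaving either First volume hides the visible icon.
; An older DoOnce-based BP_Player overlap chain remains unconnected.
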(event `self.ReceiveBeginPlay`
  ;[1 1 1] BP_GameStateを参照する変数を作成
  (bind _foundwidgets (`WidgetBlueprintLibrary.GetAllWidgetsOfClass` "/Game/Blueprint/Maps/WB_curve.WB_curve_C"))
  (set `self.WB_Carb` (`|GetArrayItem` _foundwidgets)))

(event `self.FirstOverlap_In.OnComponentEndOverlap`
  (params (OverlappedComponent :type "PrimitiveComponent Object Reference") (OtherActor :type "Actor Object Reference") (OtherComp :type "PrimitiveComponent Object Reference") (OtherBodyIndex :type Integer))
  (bind _wb_carb (`self.WB_Carb` :!label _label)
    (:`then`
      (bind _newparam (`/Game/Blueprint/Maps/WB_curve.Get Is Visible` _wb_carb))
      (if (and _newparam (`ActorComponent.ComponentHasTag` OtherComp "PlayerCollision"))
        (`/Game/Blueprint/Maps/WB_curve.Hidden Icon` _wb_carb)))
    (:`else`)))

(event `self.FirstOverlap_Out.OnComponentEndOverlap`
  (params (OverlappedComponent :type "PrimitiveComponent Object Reference") (OtherActor :type "Actor Object Reference") (OtherComp :type "PrimitiveComponent Object Reference") (OtherBodyIndex :type Integer))
  (goto _label))

(event `self.SecondOverlap_In.OnComponentEndOverlap`
  (params (OverlappedComponent :type "PrimitiveComponent Object Reference") (OtherActor :type "Actor Object Reference") (OtherComp :type "PrimitiveComponent Object Reference") (OtherBodyIndex :type Integer))
  (bind _wb_carb (`self.WB_Carb` :!label _label_2)
    (:`then`
      (bind _newparam (`/Game/Blueprint/Maps/WB_curve.Get Is Visible` _wb_carb))
      (if (and (!= _newparam true) (`ActorComponent.ComponentHasTag` OtherComp "PlayerCollision"))
        (`/Game/Blueprint/Maps/WB_curve.Show Icon` _wb_carb (`self.Is Right`))))
    (:`else`)))

(event `self.SecondOverlap_Out.OnComponentEndOverlap`
  (params (OverlappedComponent :type "PrimitiveComponent Object Reference") (OtherActor :type "Actor Object Reference") (OtherComp :type "PrimitiveComponent Object Reference") (OtherBodyIndex :type Integer))
  (goto _label_2))

(fn `UserConstructionScript`)