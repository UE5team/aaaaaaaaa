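; BP_Wall is a wall actor that bounces and damages a fast-moving player on impact, then turns them along the wall's spline.
; OnWallHit acts above a speed threshold, classifying the yaw against the closest spline rotation as front, intermediate or back.
; It also launches the player along a damped, clamped reflected velocity.
; While IsTouchWall is set, Tick interpolates player rotation along or against the spline, skipping intermediate hits.
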(event `self.ReceiveTick`
  (params (DeltaSeconds :type "Float (single-precision)"))
  (bind _bp_player (`self.BP Player`))
  (bind _bp_player_2 (`self.BP Player`)
    (:`then`
      (if (`/Game/Blueprint/Player/BP_Player.is Touch Wall` _bp_player_2)
        (switch `/Game/Blueprint/Enum/E_Angle` (`self.Hit Angle`)
          (:`NewEnumerator0`
            (`SceneComponent.K2_SetWorldRotation` (`Actor.RootComponent` _bp_player) (`KismetMathLibrary.MakeRotator` 0.0 (.pitch (`KismetMathLibrary.RInterpTo` (`self.K2_GetActorRotation` _bp_player) (`SplineComponent.FindRotationClosestToWorldLocation` (`self.BP Spline`) (`self.K2_GetActorLocation` (`self.BP Player`)) "World") DeltaSeconds 10.0)) (.yaw (`KismetMathLibrary.RInterpTo` (`self.K2_GetActorRotation` _bp_player) (`SplineComponent.FindRotationClosestToWorldLocation` (`self.BP Spline`) (`self.K2_GetActorLocation` (`self.BP Player`)) "World") DeltaSeconds 10.0))) false false))
          (:`NewEnumerator2`
            (`SceneComponent.K2_SetWorldRotation` (`Actor.RootComponent` (`self.BP Player`)) (`KismetMathLibrary.MakeRotator` 0.0 (.pitch (`KismetMathLibrary.RInterpTo` (`self.K2_GetActorRotation` (`self.BP Player`)) (`KismetMathLibrary.MakeRotator` (.roll (`SplineComponent.FindRotationClosestToWorldLocation` (`self.BP Spline`) (`self.K2_GetActorLocation` (`self.BP Player`)) "World")) (.pitch (`SplineComponent.FindRotationClosestToWorldLocation` (`self.BP Spline`) (`self.K2_GetActorLocation` (`self.BP Player`)) "World")) (- (.yaw (`SplineComponent.FindRotationClosestToWorldLocation` (`self.BP Spline`) (`self.K2_GetActorLocation` (`self.BP Player`)) "World")) 180.0)) DeltaSeconds 10.0)) (.yaw (`KismetMathLibrary.RInterpTo` (`self.K2_GetActorRotation` (`self.BP Player`)) (`KismetMathLibrary.MakeRotator` (.roll (`SplineComponent.FindRotationClosestToWorldLocation` (`self.BP Spline`) (`self.K2_GetActorLocation` (`self.BP Player`)) "World")) (.pitch (`SplineComponent.FindRotationClosestToWorldLocation` (`self.BP Spline`) (`self.K2_GetActorLocation` (`self.BP Player`)) "World")) (- (.yaw (`SplineComponent.FindRotationClosestToWorldLocation` (`self.BP Spline`) (`self.K2_GetActorLocation` (`self.BP Player`)) "World")) 180.0)) DeltaSeconds 10.0))) false false)))))
    (:`else`)))

(fn `Leave Wall`
  (set `self.isHit` false))

(fn `OnWallHit`
  (params (BP_Player :type "/Game/Blueprint/Player/BP_Player Object Reference") (BP_Spline :type "SplineComponent Object Reference") (hit :type "HitResult Structure"))
  (bind _returnvalue (`self.GetVelocity` BP_Player))
  (bind (_returnvalue_roll _returnvalue_pitch _returnvalue_yaw) (`KismetMathLibrary.BreakRotator` (`self.K2_GetActorRotation` (`self.BP Player`))))
  (bind _returnvalue_2 (`KismetMathLibrary.Abs` (`KismetMathLibrary.NormalizeAxis` (- (.yaw (.rotation (`SplineComponent.FindTransformClosestToWorldLocation` (`self.BP Spline`) (`self.K2_GetActorLocation` (`self.BP Player`)) "World" false))) _returnvalue_yaw))))
  (set `self.BP Player` BP_Player)
  (set `self.BP Spline` BP_Spline)
  (if (> (`KismetMathLibrary.VSize` _returnvalue) 3000.0)
    (set `/Game/Blueprint/Player/BP_Player.is Touch Wall` true BP_Player)
    (`|ExecutionSequence`
      (:`then_0`
        (if (< _returnvalue_2 80.0)
          (set `self.Hit Angle` "NewEnumerator0")
          (elif (< _returnvalue_2 100.0)
            (set `self.Hit Angle` "NewEnumerator1")
            (else
              (set `self.Hit Angle` "NewEnumerator2")))))
      (:`then_1`
        (`Character.LaunchCharacter` BP_Player (`KismetMathLibrary.ClampVectorSize` (* (- _returnvalue (* (* hit_Normal (`KismetMathLibrary.Dot_VectorVector` _returnvalue hit_Normal)) 2.0)) 0.8) 0.0 3000.0) true false)
        (`GameplayStatics.ApplyDamage` (`self.BP Player`) (`self.Damage Value`))
        (`KismetSystemLibrary.PrintString` "hit")
        (`/Game/Blueprint/Player/BP_Player.Reflect damage animation` (`self.BP Player`))))))

(fn `UserConstructionScript`)