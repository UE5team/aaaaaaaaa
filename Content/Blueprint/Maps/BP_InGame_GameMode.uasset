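; In-game GameMode that tracks score, player damage and game over, keeping the values in the GI_Defolut game instance.
; Functions add enemy, road and course-out points, and Tick calls the instance's GetViewPoint.
; TakeDamage lowers durability and, at zero or below, calls KillPlayer, which pauses the game and shows the HUD_InGame result screen.
; RespawnPlayer spawns and possesses a new BP_Player at the start transform saved on BeginPlay; ResultGame triggers the HUD's retry event.
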(event `self.ReceiveBeginPlay`
  ;[1 1 1] PlayerStartを初期位置として値を保持する
  (set `self.SpawnTransform` (`self.GetTransform` (`GameplayStatics.GetPlayerCharacter` 0)))
  (`KismetSystemLibrary.Delay` 0.2)
  (bind _foundwidgets (`WidgetBlueprintLibrary.GetAllWidgetsOfClass` "/Game/Blueprint/point/BP_UI_point_num_2.BP_UI_point_num_2_C"))
  (set `self.UI Point Num2` (`|GetArrayItem` _foundwidgets)))

(event `self.ReceiveTick`
  (params (DeltaSeconds :type "Float (single-precision)"))
  (bind _asgi_defolut (cast `/Game/Blueprint/Maps/GI_Defolut` (`GameplayStatics.GetGameInstance`)))
  (`/Game/Blueprint/Maps/GI_Defolut.GetViewPoint` _asgi_defolut))

(event `RespawnPlayer`
  ;[1 1 1] Destroy後にRespawnを実行する
  (bind _returnvalue (`|SpawnActorFromClass` :`Class` "/Game/Blueprint/Player/BP_Player.BP_Player_C" :`SpawnTransform` (`self.SpawnTransform`) :`CollisionHandlingOverride` "Undefined" :`TransformScaleMethod` "OverrideRootScale" :`Owner` (`GameplayStatics.GetPlayerPawn` 0) :`Instigator` null))
  (`Controller.Possess` (`GameplayStatics.GetPlayerController` 0) _returnvalue))

(event `ResultGame`
  ;[1 1 1] GameOver画面を表示する
  (bind _ashud_in_game (cast `/Game/Blueprint/point/HUD_InGame` (`PlayerController.GetHUD` (`GameplayStatics.GetPlayerController` 0))))
  (`/Game/Blueprint/point/HUD_InGame.ReTry_Event` _ashud_in_game))

(fn `AddEnemyPoint`
  (returns (NewPointNumber :type Integer))
  ;[1 1 1] ポイントのトータルを加算する
  (bind _asgi_defolut (cast `/Game/Blueprint/Maps/GI_Defolut` (`GameplayStatics.GetGameInstance`)))
  (bind _output_get (set `/Game/Blueprint/Maps/GI_Defolut.EnemyPoints` (+ (`/Game/Blueprint/Maps/GI_Defolut.EnemyPoints` _asgi_defolut) (`/Game/Blueprint/Maps/GI_Defolut.ConstantEnemyPoint` _asgi_defolut)) _asgi_defolut))
  (return _output_get))

(fn `AddRoadPoint`
  (returns (NewPointNumber :type Integer))
  ;[1 1 1] ポイントのトータルを加算する
  (bind _asgi_defolut (cast `/Game/Blueprint/Maps/GI_Defolut` (`GameplayStatics.GetGameInstance`)))
  (bind _output_get (set `/Game/Blueprint/Maps/GI_Defolut.RoadPoints` (+ (`/Game/Blueprint/Maps/GI_Defolut.RoadPoints` _asgi_defolut) (`/Game/Blueprint/Maps/GI_Defolut.ConstantRoadPoints` _asgi_defolut)) _asgi_defolut))
  (return _output_get))

(fn `KillPlayer`
  (params (BP_Player :type "/Game/Blueprint/Player/BP_Player Object Reference"))
  ;[1 1 1] プレイヤーを操作できないようにする
  (`GameplayStatics.SetGamePaused` true)
  ;[1 1 1] ゲームオーバー画面を表示する
  (bind _ashud_in_game (cast `/Game/Blueprint/point/HUD_InGame` (`PlayerController.GetHUD` (`GameplayStatics.GetPlayerController` 0))))
  (`/Game/Blueprint/point/HUD_InGame.DispResult_Event` _ashud_in_game))

(fn `PointsGoingOutside`
  (params (NewParam :type Integer))
  ;[1 1 1] コースアウトした分のポイントを加算
  (bind _asgi_defolut (cast `/Game/Blueprint/Maps/GI_Defolut` (`GameplayStatics.GetGameInstance`)))
  (if (> (`/Game/Blueprint/Maps/GI_Defolut.ViewPoint` _asgi_defolut) 0)
    (set `/Game/Blueprint/Maps/GI_Defolut.CourceOutPoints` (+ (`/Game/Blueprint/Maps/GI_Defolut.CourceOutPoints` _asgi_defolut) NewParam) _asgi_defolut)))

(fn `TakeDamage`
  (params (Damage :type "Float (double-precision)"))
  (returns (Returnvalue :type "Float (double-precision)"))
  (bind _asgi_defolut (cast `/Game/Blueprint/Maps/GI_Defolut` (`GameplayStatics.GetGameInstance`)))
  ;[1 1 1] DurableにDamageを与える
  (bind _output_get (set `/Game/Blueprint/Maps/GI_Defolut.Durable value` (- (`/Game/Blueprint/Maps/GI_Defolut.Durable value` _asgi_defolut) Damage) _asgi_defolut))
  (if (<= _output_get 0.0)
    ;[1 1 1] 0以下：PlayerをKillする
    (bind _asbp_player (cast `/Game/Blueprint/Player/BP_Player` (`GameplayStatics.GetPlayerPawn` 0)))
    (`self.KillPlayer` _asbp_player))
  (return 0.0))

(fn `UserConstructionScript`)