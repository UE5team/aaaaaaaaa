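; BP_TheWorld_Trigger_3 is an overlap trigger that sends the player into a "TheWorld" transition on a specific lap.
; When its static mesh is overlapped, it checks that the level's Goal_tape_Blueprint reports LapDigit 1 and the overlapping component is tagged PlayerCollision.
; It then calls TransitionToTheWorld on BP_Player, using the MoveTarget and FrontTarget components' world locations as destination and look direction.
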(event `self.StaticMesh.OnComponentBeginOverlap`
  (params (OverlappedComponent :type "PrimitiveComponent Object Reference") (OtherActor :type "Actor Object Reference") (OtherComp :type "PrimitiveComponent Object Reference") (OtherBodyIndex :type Integer) (bFromSweep :type Boolean) (SweepResult :type "HitResult Structure (by ref)"))
  (if (== (`/Game/Blueprint/Maps/Goal_tape_Blueprint.Lap digit` (`self.Get Goal Tape`)) 1)
    (if (`ActorComponent.ComponentHasTag` OtherComp "PlayerCollision")
      (`/Game/Blueprint/Player/BP_Player.transitionToTheWorld` (cast `/Game/Blueprint/Player/BP_Player` OtherActor :!pure true) (`SceneComponent.K2_GetComponentLocation` (`self.MoveTarget`)) (`SceneComponent.K2_GetComponentLocation` (`self.FrontTarget`))))))

(fn `Get Goal Tape`
  (returns (`Goal Tape` :type "/Game/Blueprint/Maps/Goal_tape_Blueprint Object Reference"))
  (bind _returnvalue (`GameplayStatics.GetActorOfClass` "/Game/Blueprint/Maps/Goal_tape_Blueprint.Goal_tape_Blueprint_C"))
  (return _returnvalue))

(fn `UserConstructionScript`)