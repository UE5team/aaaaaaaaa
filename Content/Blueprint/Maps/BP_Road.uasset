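; BP_Road is a spline-based road actor that lays street meshes along an editable path.
; The construction script re-syncs the spline to the root's location with a fixed -90 degree rotation and 100x the root's scale.
; It then adds a Y-forward SM_Street spline mesh per segment, bent by the endpoint positions and tangents, with query and physics collision.
; The event graph holds no runtime logic.
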(fn `UserConstructionScript`
  (bind _spline (`self.Spline`))
  (bind (_returnvalue_location _returnvalue_rotation _returnvalue_scale) (`KismetMathLibrary.BreakTransform` (`SceneComponent.K2_GetComponentToWorld` (`self.DefaultSceneRoot`))))
  ;[1 1 1] Transformの同期
  (`SceneComponent.K2_SetWorldTransform` (`self.Spline`) (`KismetMathLibrary.MakeTransform` _returnvalue_location (struct :`Roll` -90.0) (* _returnvalue_scale 100.0)) false false)
  ;[1 1 1] セグメントの数だけ処理を実行
  (for _index (range (`SplineComponent.GetNumberOfSplineSegments` (`self.Spline`)))
    ;;[1 1 1] スプラインメッシュコンポーネントの作成
    (bind _returnvalue (`AddComponent|NODE_AddSplineMeshComponent-0`))
    ;;[1 1 1] 作成したスプラインメッシュをスプラインにつける
    (`SceneComponent.K2_AttachToComponent` _returnvalue (`self.Spline`) "None" "KeepRelative" "KeepRelative" "KeepRelative" true)
    (`SplineMeshComponent.SetForwardAxis` _returnvalue "Y" true)
    ;;[1 1 1] 道メッシュの割り当て
    (`StaticMeshComponent.SetStaticMesh` _returnvalue "/Game/ExampleContent/Landscapes/Meshes/SM_Street.SM_Street")
    (bind (_location _tangent) (`SplineComponent.GetLocationAndTangentAtSplinePoint` _spline _index "Local"))
    (bind (_location_2 _tangent_2) (`SplineComponent.GetLocationAndTangentAtSplinePoint` _spline (+ _index 1) "Local"))
    ;;[1 1 1] 道メッシュの変形
    (`SplineMeshComponent.SetStartAndEnd` _returnvalue _location _tangent _location_2 _tangent_2 true)
    ;;[1 1 1] コリジョン設定
    (`PrimitiveComponent.SetCollisionEnabled` _returnvalue "QueryAndPhysics")))