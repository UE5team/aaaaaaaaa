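; BP_Dashboard is a dash pad that boosts the player along the direction they are facing.
; Mesh component hit, actor hit and overlap events all feed one branch that checks for the "Player" tag.
; It then finds BP_Player by class, scales its normalized forward vector horizontally, and adds that through LaunchCharacter without overriding velocity, followed by a 2D sound.
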(event `self.StaticMeshComponent.OnComponentHit` :!enabledstate Disabled
  (params (HitComponent :type "PrimitiveComponent Object Reference") (OtherActor :type "Actor Object Reference") (OtherComp :type "PrimitiveComponent Object Reference") (NormalImpulse :type "Vector Structure") (Hit :type "HitResult Structure (by ref)"))
  (if (`self.ActorHasTag` (stale `self.ReceiveHit` Other) "Player") :!label _label
    (bind _returnvalue (`GameplayStatics.GetActorOfClass` "/Game/Blueprint/Player/BP_Player.BP_Player_C"))
    (bind _output_get (set `self.dash speed` (* (`KismetMathLibrary.Normal` (`self.GetActorForwardVector` _returnvalue)) (1200.0 1200.0 0.0))))
    (`Character.LaunchCharacter` _returnvalue _output_get false false)
    (`GameplayStatics.PlaySound2D` "/Game/Sound/シーン切り替え2.シーン切り替え2" 1.0 1.0 0.0 null null)))

(event `self.ReceiveActorBeginOverlap` :!enabledstate Disabled
  (params (OtherActor :type "Actor Object Reference"))
  (goto _label))

(event `self.ReceiveHit`
  (params (MyComp :type "PrimitiveComponent Object Reference") (Other :type "Actor Object Reference") (OtherComp :type "PrimitiveComponent Object Reference") (bSelfMoved :type Boolean) (HitLocation :type "Vector Structure") (HitNormal :type "Vector Structure") (NormalImpulse :type "Vector Structure") (Hit :type "HitResult Structure (by ref)"))
  (goto _label))

(fn `UserConstructionScript`)