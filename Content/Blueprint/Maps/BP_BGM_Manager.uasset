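; BP_BGM_Manager is an actor that manages the background music for the course being played.
; On BeginPlay it finds BP_CourceManager, reads the course type number, and adds one of three audio components accordingly.
; It stores that component as BGM, which the stopBGM event later stops.
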(event `self.ReceiveBeginPlay`
  (bind _returnvalue (`GameplayStatics.GetActorOfClass` "/Game/Blueprint/System/BP_CourceManager.BP_CourceManager_C"))
  (switch `/Game/Blueprint/System/E_Cource` (`/Game/Blueprint/System/BP_CourceManager.getCourceTypeNum` _returnvalue)
    (:`NewEnumerator0`
      (bind _returnvalue_2 (`AddComponent|NODE_AddAudioComponent-0`))
      (set `self.BGM` _returnvalue_2))
    (:`NewEnumerator1`
      (bind _returnvalue_3 (`AddComponent|NODE_AddAudioComponent-1`))
      (set `self.BGM` _returnvalue_3))
    (:`NewEnumerator2`
      (bind _returnvalue_4 (`AddComponent|NODE_AddAudioComponent-2`))
      (set `self.BGM` _returnvalue_4))))

(event `stopBGM`
  (`AudioComponent.Stop` (`self.BGM`)))

(fn `UserConstructionScript`)