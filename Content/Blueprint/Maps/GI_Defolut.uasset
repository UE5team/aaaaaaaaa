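; Game instance for a lap-based race game, holding points, formatted lap time, loading state and player selection data across levels.
; Goal runs once until Init resets it: it plays finish UI and audio, clears enemies and energy, then loads results via BP_LevelManager.
; GoaltapeOverlap resets lap checkpoints and energy between laps; ResetEnemy's destroy call is disconnected.
; GetViewPoint totals the score; タイム計算 formats time through Timer.
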(event `Goal`
  (`/Engine/EditorBlueprintResources/StandardMacros.DoOnce` false :!label _label
    (:`Completed`
      (set `self.BP Player` (cast `/Game/Blueprint/Player/BP_Player` (`GameplayStatics.GetPlayerCharacter` 0) :!pure true))
      ;[1 1 1] ゴールしたことを示す変数をtrueに
      (bind _foundwidgets (`WidgetBlueprintLibrary.GetAllWidgetsOfClass` "/Game/Blueprint/Maps/WBP_Ingame_UI.WBP_Ingame_UI_C"))
      (bind _output_get (set `self.Timer_0` (`/Game/Blueprint/Maps/WBP_Ingame_UI.timer` (`|GetArrayItem` _foundwidgets))))
      (set `/Game/Blueprint/Maps/timer.is goal` true _output_get)
      ;[1 1 1] プレイヤーを無敵状態にする
      (set `/Game/Blueprint/Player/BP_Player.IsHitCoolTime` true (`self.BP Player`))
      (`UserWidget.AddToViewport` (`/Game/Blueprint/System/BP_WidgetCreater.getGoal` (`/Game/Blueprint/System/FL_MyLibrary.getWidgetCreator`)) 0)
      ;[1 1 1] ゴール時効果音再生
      (`GameplayStatics.PlaySoundAtLocation` "/Game/Sound/効果音ラボ/エアーホーン.エアーホーン" (0.0 0.0 0.0) (struct) 1.0 1.0 0.0 null null null null)
      ;[1 1 1] BGMを止める
      (bind _returnvalue (`GameplayStatics.GetActorOfClass` "/Game/Blueprint/Maps/BP_BGM_Manager.BP_BGM_Manager_C"))
      (`/Game/Blueprint/Maps/BP_BGM_Manager.stopBGM` _returnvalue)
      (`KismetSystemLibrary.Delay` 0.7)
      (bind _returnvalue_2 (`GameplayStatics.SpawnSound2D` "/Game/Sound/Pulsewave_Pinnacle.Pulsewave_Pinnacle" 1.0 1.0 0.0 null))
      (set `self.Pulsewave_Pinnacle` _returnvalue_2)
      (`KismetSystemLibrary.Delay` 5.0)
      (bind _foundwidgets_2 (`WidgetBlueprintLibrary.GetAllWidgetsOfClass` "/Game/Blueprint/Maps/WBP_Ingame_UI.WBP_Ingame_UI_C" false))
      (bind _outactors (`GameplayStatics.GetAllActorsOfClass` "/Game/Blueprint/Enemy/BP_NEO_Enemy.BP_NEO_Enemy_C"))
      (`Actor.K2_DestroyActor` _outactors)
      (`WidgetLayoutLibrary.RemoveAllWidgets`)
      (`/Game/Blueprint/System/FL_MyLibrary.RemoveAllMappingContext`)
      (bind _returnvalue_3 (`GameplayStatics.GetActorOfClass` "/Game/Blueprint/System/BP_LevelManager.BP_LevelManager_C"))
      (`/Game/Blueprint/System/BP_LevelManager.SetupLoad` _returnvalue_3 "result")
      (bind _outactors_2 (`GameplayStatics.GetAllActorsOfClass` "/Game/Blueprint/point/BP_energy.BP_energy_C"))
      (for _array_element _outactors_2
        (`/Game/Blueprint/point/BP_energy.DestroyPoint` _array_element _array_element))
      (bind _outactors_3 (`GameplayStatics.GetAllActorsOfClass` "/Game/Blueprint/Enemy/BP_NEO_Enemy.BP_NEO_Enemy_C"))
      (for _array_element_2 _outactors_3
        (`/Game/Blueprint/Enemy/EnemyManager.DestroyEnemy` (`self.Get BP_EnemyMamager`) _array_element_2)))))

(event `ResetGoalEvent`
  (goto _label :!via `Reset`))

(event `Goal tape Over lap`
  (params (`Goal tape` :type "/Game/Blueprint/Maps/Goal_tape_Blueprint Object Reference") (BGM :type "AudioComponent Object Reference") (timer :type "/Game/Blueprint/Maps/timer Object Reference") (BP_Player :type "/Game/Blueprint/Player/BP_Player Object Reference") (Gi_Final_Lap :type Integer))
  (bind _goal_tape (`self.Goal Tape`))
  (bind _goal_tape_2 (`self.Goal Tape`))
  (set `self.Goal Tape` `Goal tape`)
  (set `self.BGM` BGM)
  (set `self.Timer_0` timer)
  (set `self.BP Player` BP_Player)
  (set `self.Gi_Final_Lap` Gi_Final_Lap)
  (`/Game/Blueprint/Maps/Goal_tape_Blueprint.CheckGoalCondition` _goal_tape)
  (if (and (== (`/Game/Blueprint/Maps/Goal_tape_Blueprint.Lap digit` _goal_tape) (`self.Gi_Final_Lap`)) (== (`/Game/Blueprint/Maps/Goal_tape_Blueprint.LapCountPointLength` _goal_tape) (`/Game/Blueprint/Maps/Goal_tape_Blueprint.LapCOuntPointPassedNum` _goal_tape)))
    (set `/Game/Blueprint/Maps/Goal_tape_Blueprint.LapCountPointPassedNum` 0 _goal_tape_2)
    (else
      (set `/Game/Blueprint/Maps/Goal_tape_Blueprint.LapCountPointPassedNum` 0 _goal_tape_2)
      (if (> (`/Game/Blueprint/Maps/Goal_tape_Blueprint.Lap digit` (`self.Goal Tape`)) 1)
        (`self.Reset Enemy`)
        (`self.Reset RoadPoint`)
        (for _index (range (+ (`/Game/Blueprint/Maps/Goal_tape_Blueprint.LapCountPointLastIndex` (`self.Goal Tape`)) 1))
          (set `/Game/Blueprint/Maps/BP_LapCountPoint.IsLapFlag` false (`|GetArrayItem` (`/Game/Blueprint/Maps/Goal_tape_Blueprint.LapCountPoint` (`self.Goal Tape`)) _index)))))))

(event `タイム計算`
  (params (msec :type "Float (double-precision)"))
  ;[1 1 1] タイム計算
  (bind _output_get (set `self.Lap Time` msec))
  (if (< _output_get 9.99)
    (set `self.lap digit count` 2)
    (bind _output_get_2 (set `self.lap msec string` (`KismetStringLibrary.RightChop` (`KismetTextLibrary.Conv_TextToString` (`KismetTextLibrary.Conv_DoubleToText` (`self.Lap Time`) "HalfToEven" false true 1 324 2 2)) (`self.lap digit count`)) :!label _label_2))
    (bind _time_string (`self.timer` (`self.Lap Time`) _output_get_2))
    (set `self.Gi_Saved time` _time_string)
    (elif (< _output_get 99.99)
      (set `self.lap digit count` 3)
      (goto _label_2)
      (elif (< _output_get 999.99)
        (set `self.lap digit count` 4)
        (goto _label_2)
        (elif (< _output_get 9999.99)
          (set `self.lap digit count` 5)
          (goto _label_2))))))

(fn `Get BP_EnemyMamager`
  (returns (BP_NEO_Enemy :type "/Game/Blueprint/Enemy/EnemyManager Object Reference"))
  (bind _returnvalue (`GameplayStatics.GetActorOfClass` "/Game/Blueprint/Enemy/EnemyManager.EnemyManager_C"))
  (return _returnvalue))

(fn `GetLoadingNow`
  (returns (value :type Boolean))
  (return (`self.loadingnow`)))

(fn `GetViewPoint`
  (returns (NewParam :type Integer))
  (bind _asgi_defolut (cast `/Game/Blueprint/Maps/GI_Defolut` (`GameplayStatics.GetGameInstance`)))
  (bind _output_get (set `self.ViewPoint` (+ (+ (* (`/Game/Blueprint/Maps/GI_Defolut.EnemyPoints` _asgi_defolut) (`self.EnemyDeathCount`)) (`/Game/Blueprint/Maps/GI_Defolut.RoadPoints` _asgi_defolut)) (+ (`/Game/Blueprint/Maps/GI_Defolut.CourceOutPoints` _asgi_defolut) (`/Game/Blueprint/Maps/GI_Defolut.WeaponPoints` _asgi_defolut)) (`self.Initial Point`) (`self.DeadPoint`))))
  (return _output_get))

(fn `init`
  (bind (_gi_goal_time _gi_msec _gi_saved_time _gi_pointnum _max_durable _gi_name _enemypoints _roadpoints _courceoutpoints _weaponpoints _mesc_m _msec_string_m _timer_m _time_string_m _lap_time _lap_digit_count _lap_msec_string _loadingnow _durabilityscoce _constantenemypoint _constantcourepoint _totalspeed _totalacceleration _level _constantroadpoints _initial_point _viewpoint _totalturbo _totalarmor _equipindex _target_array _loading_process_task _equipstatus _equip_focus_index_array _target_index _gi_final_lap _enemycount _goal_tape _bp_player _enemydeathcount) (defaults `/Game/Blueprint/Maps/GI_Defolut` "GI_Defolut_C"))
  ;[1 1 1] DefaultValueを設定する
  (set `self.Gi_goal time` _gi_goal_time)
  (set `self.Gi_msec` _gi_msec)
  (set `self.Gi_Saved time` _gi_saved_time)
  (set `self.Gi_PointNum` _gi_pointnum)
  (set `self.Gi_name` _gi_name)
  (set `self.EnemyPoints` _enemypoints)
  (set `self.RoadPoints` _roadpoints)
  (set `self.CourceOutPoints` _courceoutpoints)
  (set `self.WeaponPoints` _weaponpoints)
  (set `self.EnemyDeathCount` _enemydeathcount)
  (`self.ResetGoalEvent`))

(fn `Reset Enemy`
  (bind _outactors (`GameplayStatics.GetAllActorsOfClass` "/Game/Blueprint/Enemy/BP_NEO_Enemy.BP_NEO_Enemy_C"))
  (for _array_element _outactors
    _))

(fn `Reset RoadPoint`
  (bind _outactors (`GameplayStatics.GetAllActorsOfClass` "/Game/Blueprint/point/BP_energy.BP_energy_C"))
  (for _array_element _outactors
    (`Actor.K2_DestroyActor` _array_element)))

(fn `Set Focus Index`
  (params (CharacterFocusIndex :type Integer) (EquipFocusIndex :type Integer))
  (set `self.CharacterFocusIndex` CharacterFocusIndex)
  (set `self.EquipFocusIndex` EquipFocusIndex))

(fn `Set PG_Player Parameter`
  (params (`PG_Player Parameter` :type "/Game/Blueprint/CharacterSelection/Structures/ST_PG_PlayerParameters Structure"))
  (set `self.PG Player Parameter` `PG_Player Parameter`))

(fn `Spawn RoadPoint`
  (bind _outactors (`GameplayStatics.GetAllActorsOfClass` "/Game/Blueprint/point/BP_EnergySpawn.BP_EnergySpawn_C"))
  (for _array_element _outactors
    (`/Game/Blueprint/point/BP_EnergySpawn.SpawnEnergy` _array_element)))

(fn `Stop Pulsewave Pinnacle`
  (bind _pulsewave_pinnacle (`self.Pulsewave_Pinnacle`)
    (:`then`
      (`AudioComponent.Stop` _pulsewave_pinnacle)
      (return))
    (:`else`)))

(fn `timer`
  (params (mesc :type "Float (double-precision)") (`msec stinrg` :type String))
  (returns (`time string` :type String))
  (bind _timer_m (`self.Timer_M`))
  (bind _timer_m_2 (`self.Timer_M`))
  (bind _timer_m_3 (`self.Timer_M`))
  (bind _output_get (set `self.Mesc M` mesc))
  (set `self.Msec String_M` `msec stinrg`)
  (set `self.Timer_M` (`KismetMathLibrary.FTrunc` _output_get))
  (if (> (`self.Timer_M`) 59)
    (if (>= (`self.Timer_M`) 600)
      ;[1 1 1] 10分以上の場合の処理
      (set `self.time string_M` (`KismetStringLibrary.Concat_StrStr` (`KismetStringLibrary.Concat_StrStr` (`KismetStringLibrary.Conv_IntToString` (/ _timer_m_3 60)) ":") (`KismetStringLibrary.Conv_IntToString` (mod _timer_m_3 60)) ":" (`self.Msec String_M`)))
      (elif (>= (mod (`self.Timer_M`) 60) 10)
        ;[1 1 1] 一分10秒以上の場合の処理
        (set `self.time string_M` (`KismetStringLibrary.Concat_StrStr` (`KismetStringLibrary.Concat_StrStr` "0" (`KismetStringLibrary.Conv_IntToString` (/ _timer_m 60)) ":") (`KismetStringLibrary.Conv_IntToString` (mod _timer_m 60)) ":" (`self.Msec String_M`)))
        (else
          ;[1 1 1] 一分9秒以下の場合の処理
          (set `self.time string_M` (`KismetStringLibrary.Concat_StrStr` (`KismetStringLibrary.Concat_StrStr` "0" (`KismetStringLibrary.Conv_IntToString` (/ _timer_m_2 60)) ":") (`KismetStringLibrary.Concat_StrStr` "0" (`KismetStringLibrary.Conv_IntToString` (mod _timer_m_2 60)) ":" (`self.Msec String_M`)))))))
    (else
      ;[1 1 1] 59秒以下の場合の処理
      (if (> (`self.Timer_M`) 9)
        (set `self.time string_M` (`KismetStringLibrary.Concat_StrStr` "00:" (`KismetStringLibrary.Conv_IntToString` (`self.Timer_M`)) ":" (`self.Msec String_M`)))
        (elif (> (`self.Mesc M`) 0.99)
          (set `self.time string_M` (`KismetStringLibrary.Concat_StrStr` "00:0" (`KismetStringLibrary.Conv_IntToString` (`self.Timer_M`)) ":" (`self.Msec String_M`)))
          (else
            ;[1 1 1] 1秒未満
            (set `self.time string_M` (`KismetStringLibrary.Concat_StrStr` "00:00:" (`self.Msec String_M`))))))))
  (return (`self.time string_M`)))