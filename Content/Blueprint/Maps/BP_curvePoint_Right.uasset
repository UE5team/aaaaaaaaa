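; BP_curvePoint_Right is a map trigger that shows the right-curve icon on the WB_curve widget as BP_Player passes through.
; BeginPlay caches the first top-level WB_curve found.
; The FirstOverlap volume sets a flag and re-arms SecondOverlap, which shows the icon only if that flag is set.
; Two cross-resetting DoOnce nodes enforce the first-then-second order, although the flag is never cleared.
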(event `self.ReceiveBeginPlay`
  ;[1 1 1] BP_GameStateを参照する変数を作成
  (bind _foundwidgets (`WidgetBlueprintLibrary.GetAllWidgetsOfClass` "/Game/Blueprint/Maps/WB_curve.WB_curve_C"))
  (set `self.WB_Carb` (`|GetArrayItem` _foundwidgets)))

(event `self.FirstOverlap.OnComponentBeginOverlap`
  (params (OverlappedComponent :type "PrimitiveComponent Object Reference") (OtherActor :type "Actor Object Reference") (OtherComp :type "PrimitiveComponent Object Reference") (OtherBodyIndex :type Integer) (bFromSweep :type Boolean) (SweepResult :type "HitResult Structure (by ref)"))
  (cast `/Game/Blueprint/Player/BP_Player` OtherActor)
  (`/Engine/EditorBlueprintResources/StandardMacros.DoOnce` false :!label _label
    (:`Completed`
      (set `self.FirstObjectOverlap` true)
      (goto _label_2 :!via `Reset`))))

(event `self.SecondOverlap.OnComponentBeginOverlap`
  (params (OverlappedComponent :type "PrimitiveComponent Object Reference") (OtherActor :type "Actor Object Reference") (OtherComp :type "PrimitiveComponent Object Reference") (OtherBodyIndex :type Integer) (bFromSweep :type Boolean) (SweepResult :type "HitResult Structure (by ref)"))
  (cast `/Game/Blueprint/Player/BP_Player` OtherActor)
  (`/Engine/EditorBlueprintResources/StandardMacros.DoOnce` false :!label _label_2
    (:`Completed`
      (if (`self.FirstObjectOverlap`)
        (bind _wb_carb (`self.WB_Carb`)
          (:`then`
            (`/Game/Blueprint/Maps/WB_curve.Show Right Icon` _wb_carb)
            (goto _label :!via `Reset`))
          (:`else`))))))

(fn `UserConstructionScript`)