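; Game instance that retains race state such as times, points, durability and name, with Init restoring it to class defaults.
; The lap-time event slices the decimal digits from a seconds value and passes them to Timer, which builds a colon-separated minutes, seconds and fraction string for the saved time.
; Openlevel stream-loads and opens the target level, bracketed by a loading-screen process task that it registers and then unregisters.
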(event `タイム計算`
  (params (msec :type "Float (double-precision)"))
  ;[1 1 1] タイム計算
  (bind _output_get (set `self.Lap Time` msec))
  (set `self.convert to time` (`KismetMathLibrary.FTrunc` (`self.Lap Time`)))
  (if (< _output_get 9.99)
    (set `self.lap digit count` 2)
    (bind _output_get_2 (set `self.lap msec string` (`KismetStringLibrary.RightChop` (`KismetTextLibrary.Conv_TextToString` (`KismetTextLibrary.Conv_DoubleToText` (`self.Lap Time`) "HalfToEven" false true 1 324 2)) (`self.lap digit count`)) :!label _label))
    (bind _time_string (`self.timer` (`self.Lap Time`) _output_get_2))
    (set `self.Gi_Saved time` _time_string)
    (elif (< _output_get 99.99)
      (set `self.lap digit count` 3)
      (goto _label)
      (elif (< _output_get 999.99)
        (set `self.lap digit count` 4)
        (goto _label)
        (elif (< _output_get 9999.99)
          (set `self.lap digit count` 5)
          (goto _label))))))

(event `Openlevel`
  (bind _level (`self.Level`))
  (`self.BeginLoadingScreen`) ; ローディング画面表示
  ;[1 1 1] levelをロードして開く
  (`GameplayStatics.LoadStreamLevelBySoftObjectPtr` _level true true)
  (`GameplayStatics.OpenLevelBySoftObjectPtr` _level)
  (`self.EndLoadingScreen`) ; ローディング画面を閉じる
)

(event `BeginLoadingScreen`
  (`/Engine/EditorBlueprintResources/StandardMacros.IsValid` (`self.LodingProcessTask`)
    (:`Is Not Valid`
      (bind _returnvalue (`LoadingProcessTask.CreateLoadingScreenProcessTask` "LoadingScreen"))
      (set `self.LodingProcessTask` _returnvalue))))

(event `EndLoadingScreen`
  (bind _lodingprocesstask (`self.LodingProcessTask`)
    (:`then`
      (`LoadingProcessTask.Unregister` _lodingprocesstask)
      (set `self.LodingProcessTask` null))
    (:`else`)))

(fn `init`
  (bind (_gi_goal_time _gi_msec _gi_saved_time _gi_pointnum _gi_lap_time _durable_value _max_durable _gi_name _enemypoints _roadpoints _courceoutpoints _weaponpoints) (defaults `/Game/Blueprint/Maps/GI_VariableRetention` "GI_VariableRetention_C"))
  ;[1 1 1] DefaultValueを設定する
  (set `self.Gi_goal time` _gi_goal_time)
  (set `self.Gi_msec` _gi_msec)
  (set `self.Gi_Saved time` _gi_saved_time)
  (set `self.Gi_PointNum` _gi_pointnum)
  (set `self.Gi_lap time` _gi_lap_time)
  (set `self.Durable value` _durable_value)
  (set `self.Gi_name` _gi_name)
  (set `self.EnemyPoints` _enemypoints)
  (set `self.RoadPoints` _roadpoints)
  (set `self.CourceOutPoints` _courceoutpoints)
  (set `self.WeaponPoints` _weaponpoints))

(fn `timer`
  (params (mesc :type "Float (double-precision)") (`msec stinrg` :type String))
  (returns (`time string` :type String))
  (bind _timer_m (`self.Timer_M`))
  (bind _timer_m_2 (`self.Timer_M`))
  (bind _timer_m_3 (`self.Timer_M`))
  (bind _output_get (set `self.Mesc M` mesc))
  (set `self.Msec String_M` `msec stinrg`)
  (set `self.Timer_M` (`KismetMathLibrary.FTrunc` _output_get))
  (if (> (`self.Timer_M`) 59)
    (if (>= (`self.Timer_M`) 600)
      ;[1 1 1] 10分以上の場合の処理
      (set `self.time string_M` (`KismetStringLibrary.Concat_StrStr` (`KismetStringLibrary.Concat_StrStr` (`KismetStringLibrary.Conv_IntToString` (/ _timer_m_3 60)) ":") (`KismetStringLibrary.Conv_IntToString` (mod _timer_m_3 60)) ":" (`self.Msec String_M`)))
      (elif (>= (mod (`self.Timer_M`) 60) 10)
        ;[1 1 1] 一分10秒以上の場合の処理
        (set `self.time string_M` (`KismetStringLibrary.Concat_StrStr` (`KismetStringLibrary.Concat_StrStr` "0" (`KismetStringLibrary.Conv_IntToString` (/ _timer_m 60)) ":") (`KismetStringLibrary.Conv_IntToString` (mod _timer_m 60)) ":" (`self.Msec String_M`)))
        (else
          ;[1 1 1] 一分9秒以下の場合の処理
          (set `self.time string_M` (`KismetStringLibrary.Concat_StrStr` (`KismetStringLibrary.Concat_StrStr` "0" (`KismetStringLibrary.Conv_IntToString` (/ _timer_m_2 60)) ":") (`KismetStringLibrary.Concat_StrStr` "0" (`KismetStringLibrary.Conv_IntToString` (mod _timer_m_2 60)) ":" (`self.Msec String_M`)))))))
    (else
      ;[1 1 1] 59秒以下の場合の処理
      (if (> (`self.Timer_M`) 9)
        (set `self.time string_M` (`KismetStringLibrary.Concat_StrStr` "00:" (`KismetStringLibrary.Conv_IntToString` (`self.Timer_M`)) ":" (`self.Msec String_M`)))
        (elif (> (`self.Mesc M`) 0.99)
          (set `self.time string_M` (`KismetStringLibrary.Concat_StrStr` "00:0" (`KismetStringLibrary.Conv_IntToString` (`self.Timer_M`)) ":" (`self.Msec String_M`)))
          (else
            ;[1 1 1] 1秒未満
            (set `self.time string_M` (`KismetStringLibrary.Concat_StrStr` "00:00:" (`self.Msec String_M`))))))))
  (return (`self.time string_M`)))