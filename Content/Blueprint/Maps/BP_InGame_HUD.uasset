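; In-game HUD actor that adds the gameplay UI and manages the result screen and its menu actions.
; BeginPlay creates the result widget collapsed, plus an unused BP_UI_Result; DispResult_Event reveals it in UI-only input mode.
; W and S cycle a wrapping index that highlights one of four buttons.
; Separate events open a level, quit, or retry by re-initializing GI_Defolut, unpausing and reloading the current level.
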(event `self.ReceiveBeginPlay`
  (`|ExecutionSequence`
    (:`then_0`
      (`|CreateWidget` "/Game/Blueprint/UI/GameOver/BP_UI_Result.BP_UI_Result_C")
      (bind _returnvalue (`|CreateWidget` "/Game/Blueprint/Maps/BP_Ingame_UI.BP_Ingame_UI_C"))
      (`UserWidget.AddToViewport` _returnvalue 0))
    (:`then_1`
      ;[1 1 1] Result画面を非表示で生成する
      (bind _returnvalue_2 (`|CreateWidget` "/Game/Blueprint/point/BPW_Result.BPW_Result_C" (`GameplayStatics.GetPlayerController` 0)))
      (bind _output_get (set `self.ResultWidget` _returnvalue_2))
      (`Widget.SetVisibility` _output_get "Collapsed")
      (`UserWidget.AddToViewport` _output_get 0))))

(event `OpenLevel_Event`
  (params (LevelName :type Name))
  ;[1 1 1] Levelに遷移する
  (`WidgetBlueprintLibrary.SetInputMode_GameOnly` (`GameplayStatics.GetPlayerController` 0))
  (`GameplayStatics.OpenLevel` LevelName))

(event `DispResult_Event`
  (bind _resultwidget (`self.ResultWidget`))
  (bind _button_charactor (`/Game/Blueprint/point/BPW_Result.Button_Charactor` _resultwidget))
  (`|ExecutionSequence`
    (:`then_0`
      ;[1 1 1] Result画面をUIモードで表示する
      (bind _resultwidget_2 (`self.ResultWidget`)
        (:`then`
          (`Widget.SetVisibility` _resultwidget_2 "Visible")
          (`WidgetBlueprintLibrary.SetInputMode_UIOnlyEx` (`GameplayStatics.GetPlayerController` 0) _resultwidget_2))
        (:`else`)))
    (:`then_1`
      (`Button.SetBackgroundColor` _button_charactor (struct :`R` 1.0 :`G` 1.0 :`B` 1.0 :`A` 1.0) :!label _label)
      (`Button.SetBackgroundColor` (`/Game/Blueprint/point/BPW_Result.Button_Continue` _resultwidget) (struct :`R` 1.0 :`G` 1.0 :`B` 1.0 :`A` 1.0))
      (`Button.SetBackgroundColor` (`/Game/Blueprint/point/BPW_Result.Button_Quit` _resultwidget) (struct :`R` 1.0 :`G` 1.0 :`B` 1.0 :`A` 1.0))
      (`Button.SetBackgroundColor` (`/Game/Blueprint/point/BPW_Result.Button_Title` _resultwidget) (struct :`R` 1.0 :`G` 1.0 :`B` 1.0 :`A` 1.0))
      (switch `int` (`self.Number`)
        (:`1`
          (`Button.SetBackgroundColor` (`/Game/Blueprint/point/BPW_Result.Button_Continue` _resultwidget) (struct :`R` 1.0 :`G` 0.400952 :`B` 0.117099 :`A` 1.0)))
        (:`2`
          (`Button.SetBackgroundColor` _button_charactor (struct :`R` 1.0 :`G` 0.4 :`B` 0.117647 :`A` 1.0)))
        (:`3`
          (`Button.SetBackgroundColor` (`/Game/Blueprint/point/BPW_Result.Button_Title` _resultwidget) (struct :`R` 1.0 :`G` 0.4 :`B` 0.117647 :`A` 1.0)))
        (:`4`
          (`Button.SetBackgroundColor` (`/Game/Blueprint/point/BPW_Result.Button_Quit` _resultwidget) (struct :`R` 1.0 :`G` 0.4 :`B` 0.117647 :`A` 1.0)))))))

(event `QuitGame_Event`
  ;[1 1 1] ゲームを終了する
  (`KismetSystemLibrary.QuitGame` (`GameplayStatics.GetPlayerController` 0) "Quit"))

(event `Key|W`
  (params (Key :type "Key Structure"))
  (bind _number (`self.Number`))
  (:`Pressed`
    (set `self.Number` (- _number 1))
    (if (<= _number 0)
      (set `self.Number` 4)
      (goto _label)
      (else
        (goto _label)))))

(event `Key|S`
  (params (Key :type "Key Structure"))
  (bind _number (`self.Number`))
  (:`Pressed`
    (set `self.Number` (+ _number 1))
    (if (>= _number 5)
      (set `self.Number` 1)
      (goto _label)
      (else
        (goto _label)))))

(event `ReTry_Event`
  (`|ExecutionSequence`
    (:`then_0`
      ;[1 1 1] 初期化する
      (bind _asgi_defolut (cast `/Game/Blueprint/Maps/GI_Defolut` (`GameplayStatics.GetGameInstance`)))
      (`/Game/Blueprint/Maps/GI_Defolut.init` _asgi_defolut)
      (`GameplayStatics.SetGamePaused` false)
      (`WidgetBlueprintLibrary.SetInputMode_GameOnly` (`GameplayStatics.GetPlayerController` 0)))
    (:`then_1`
      ;[1 1 1] 現在のレベルをオープンする
      (bind _returnvalue (`GameplayStatics.GetCurrentLevelName` true))
      (`GameplayStatics.OpenLevel` (`KismetStringLibrary.Conv_StringToName` _returnvalue)))))

(event `self.ReceiveTick`
  (params (DeltaSeconds :type "Float (single-precision)")))

(fn `UserConstructionScript`)