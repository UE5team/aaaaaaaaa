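; BP_TheWorld_Point is a map trigger that gradually slows game time to a near stop once the player touches it.
; Overlapping its Cube with a Player-tagged actor sets StartTheWorld.
; Tick then drives the TheWorld event, which lowers WorldAccel by a fixed per-frame step and applies it as global time dilation until it reaches about 0.01.
; Nothing here resets the flag or restores normal speed.
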(event `self.ReceiveTick`
  (params (DeltaSeconds :type "Float (single-precision)"))
  (`self.The World!!`))

(event `The World!!`
  (if (and (> (`self.world Accel`) 0.01) (`self.Start The World`))
    (bind _output_get (set `self.world Accel` (- (`self.world Accel`) (`self.DecreseAccel`))))
    (`GameplayStatics.SetGlobalTimeDilation` _output_get)))

(event `self.Cube.OnComponentBeginOverlap`
  (params (OverlappedComponent :type "PrimitiveComponent Object Reference") (OtherActor :type "Actor Object Reference") (OtherComp :type "PrimitiveComponent Object Reference") (OtherBodyIndex :type Integer) (bFromSweep :type Boolean) (SweepResult :type "HitResult Structure (by ref)"))
  (if (`self.ActorHasTag` OtherActor "Player")
    (set `self.Start The World` true)))

(fn `UserConstructionScript`)