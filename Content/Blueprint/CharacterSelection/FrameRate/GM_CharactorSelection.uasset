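; Game mode for the character selection screen, tracking the current selection step and opening test_Stage2 when advanced past the last one.
; Confirming a step reads the HUD's focus index and stores it as the character, minigun, missile, SMG or SR choice.
; It also accumulates Speed, acceleration, Turbo and Weight from equipment DataTable lookups.
; Only minigun rows supply real stats; missiles return zeros and other steps have no lookup.
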(event `Increment Widget Index`
  (bind _returnvalue (+ (`self.Widget Index`) 1))
  (if (> (`self.Max Widget Index`) _returnvalue)
    (set `self.Widget Index` _returnvalue)
    (else
      (`GameplayStatics.OpenLevel` "test_Stage2"))))

(event `Decrement Widget Index`
  (bind _returnvalue (- (`self.Widget Index`) 1))
  (if (>= _returnvalue 0)
    (set `self.Widget Index` _returnvalue)))

(event `Set Decision Index`
  (bind _widget_index (`self.Widget Index`))
  (bind _ashud_choaractor_selecsion (cast `/Game/Blueprint/CharacterSelection/FrameRate/HUD_ChoaractorSelecsion` (`PlayerController.GetHUD` (`GameplayStatics.GetPlayerController` 0))))
  (bind _newparam1 (`/Game/Blueprint/CharacterSelection/FrameRate/HUD_ChoaractorSelecsion.Get Focus Index` _ashud_choaractor_selecsion _widget_index))
  (`self.Set Focus Index` _widget_index _newparam1)
  (bind (_newparam2 _newparam3 _newparam4 _newparam5 _newparam6) (`self.NewFunction` _widget_index _newparam1))
  (set `self.Speed` (+ _newparam3 (`self.Speed`)))
  (set `self.Axxeletation` (+ _newparam4 (`self.Axxeletation`)))
  (set `self.Turbo` (+ _newparam5 (`self.Turbo`)))
  (set `self.Weight` (+ _newparam6 (`self.Weight`))))

(fn `get Focus Index`
  (params (NewParam :type Integer))
  (returns (NewParam1 :type Integer))
  (switch `int` NewParam
    (:`0`
      (return (`self.Character Index`)))
    (:`1`
      (return (`self.MiniGun Index`)))
    (:`2`
      (return (`self.Missile Index`)))
    (:`3`
      (return (`self.SMG Index`)))
    (:`4`
      (return (`self.SR Index`)))))

(fn `NewFunction`
  (params (NewParam :type Integer) (NewParam1 :type Integer))
  (returns (NewParam2 :type "Texture2D Object Reference") (NewParam3 :type "Float (double-precision)") (NewParam4 :type "Float (double-precision)") (NewParam5 :type "Float (double-precision)") (NewParam6 :type "Float (double-precision)"))
  (switch `int` NewParam
    (:`1`
      (bind _outrownames (`DataTableFunctionLibrary.GetDataTableRowNames` "/Game/Blueprint/CharacterSelection/DataTables/DT_Equip_MiniGum.DT_Equip_MiniGum"))
      (bind _returnvalue (`|GetDataTableRow` "/Game/Blueprint/CharacterSelection/DataTables/DT_Equip_MiniGum.DT_Equip_MiniGum" (`|GetArrayItem` _outrownames NewParam1))
        (:`then`
          (bind (_texture _speed _acceleration _turbo _weight) (break `/Game/Blueprint/CharacterSelection/Structures/Struct_Equip` _returnvalue))
          (return _texture _speed _acceleration _turbo _weight))))
    (:`2`
      (bind _outrownames_2 (`DataTableFunctionLibrary.GetDataTableRowNames` "/Game/Blueprint/CharacterSelection/DataTables/DT_Equip_Missile.DT_Equip_Missile"))
      (`|GetDataTableRow` "/Game/Blueprint/CharacterSelection/DataTables/DT_Equip_Missile.DT_Equip_Missile" (`|GetArrayItem` _outrownames_2 NewParam1)
        (:`then`
          (return null 0.0 0.0 0.0 0.0))))))

(fn `Set Focus Index`
  (params (`Widget Index` :type Integer) (`Focus Index` :type Integer))
  (switch `int` `Widget Index`
    (:`0`
      (set `self.Character Index` `Focus Index`))
    (:`1`
      (set `self.MiniGun Index` `Focus Index`))
    (:`2`
      (set `self.Missile Index` `Focus Index`))
    (:`3`
      (set `self.SMG Index` `Focus Index`))
    (:`4`
      (set `self.SR Index` `Focus Index`))))

(fn `UserConstructionScript`)