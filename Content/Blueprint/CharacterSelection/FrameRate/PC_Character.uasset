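; Player controller for the character selection screen that turns Enhanced Input actions into menu navigation, confirm and back.
; Increment and decrement step the selection on HUD_ChoaractorSelecsion after a short delay, then update the decision index in GM_CharactorSelection.
; Decide and Back hide the current widget, move the game mode's widget index forward or back, and refocus.
; Decide also calls SetWeapon on the BP_SelectWeaponCharacter actor cached at BeginPlay.
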(event `self.ReceiveBeginPlay`
  (`WidgetBlueprintLibrary.SetInputMode_GameAndUIEx` self null)
  (set `self.bShowMouseCursor` false)
  (bind _outactors (`GameplayStatics.GetAllActorsOfClass` "/Game/Blueprint/Player/BP_SelectWeaponCharacter.BP_SelectWeaponCharacter_C"))
  (set `self.SelectWeaponCharactor` (`|GetArrayItem` _outactors)))

(event `EnhancedInput|/Game/Input/CharacterSelection/IA_Charactor_Decrement`
  (params (ActionValue :type Boolean) (ElapsedSeconds :type "Float (double-precision)") (TriggeredSeconds :type "Float (double-precision)") (InputAction :type "InputAction Object Reference" :default "/Game/Input/CharacterSelection/IA_Charactor_Decrement.IA_Charactor_Decrement"))
  (:`Triggered`
    ;[1 1 1] デクリメントを実行する
    (`KismetSystemLibrary.Delay` 0.3)
    (bind _ashud_choaractor_selecsion (cast `/Game/Blueprint/CharacterSelection/FrameRate/HUD_ChoaractorSelecsion` (`self.GetHUD` (`GameplayStatics.GetPlayerController` 0))))
    (`/Game/Blueprint/CharacterSelection/FrameRate/HUD_ChoaractorSelecsion.Decrement` _ashud_choaractor_selecsion)
    (bind _asgm_charactor_selection (cast `/Game/Blueprint/CharacterSelection/FrameRate/GM_CharactorSelection` (`GameplayStatics.GetGameMode`)))
    (`/Game/Blueprint/CharacterSelection/FrameRate/GM_CharactorSelection.Set Decision Index` _asgm_charactor_selection)))

(event `EnhancedInput|/Game/Input/CharacterSelection/IA_Charactor_Increment`
  (params (ActionValue :type Boolean) (ElapsedSeconds :type "Float (double-precision)") (TriggeredSeconds :type "Float (double-precision)") (InputAction :type "InputAction Object Reference" :default "/Game/Input/CharacterSelection/IA_Charactor_Increment.IA_Charactor_Increment"))
  (:`Triggered`
    ;[1 1 1] インクリメントを実行する
    (`KismetSystemLibrary.Delay` 0.3)
    (bind _ashud_choaractor_selecsion (cast `/Game/Blueprint/CharacterSelection/FrameRate/HUD_ChoaractorSelecsion` (`self.GetHUD` (`GameplayStatics.GetPlayerController` 0))))
    (`/Game/Blueprint/CharacterSelection/FrameRate/HUD_ChoaractorSelecsion.Increment` _ashud_choaractor_selecsion)
    (bind _asgm_charactor_selection (cast `/Game/Blueprint/CharacterSelection/FrameRate/GM_CharactorSelection` (`GameplayStatics.GetGameMode`)))
    (`/Game/Blueprint/CharacterSelection/FrameRate/GM_CharactorSelection.Set Decision Index` _asgm_charactor_selection)))

(event `EnhancedInput|/Game/Input/CharacterSelection/IA_Decide`
  (params (ActionValue :type Boolean) (ElapsedSeconds :type "Float (double-precision)") (TriggeredSeconds :type "Float (double-precision)") (InputAction :type "InputAction Object Reference" :default "/Game/Input/CharacterSelection/IA_Decide.IA_Decide"))
  (:`Started`
    ;[1 1 1] 決定を実行する
    (bind _ashud_choaractor_selecsion (cast `/Game/Blueprint/CharacterSelection/FrameRate/HUD_ChoaractorSelecsion` (`self.GetHUD`)))
    (`/Game/Blueprint/CharacterSelection/FrameRate/HUD_ChoaractorSelecsion.Set Visility Hidden` _ashud_choaractor_selecsion)
    (bind _asgm_charactor_selection (cast `/Game/Blueprint/CharacterSelection/FrameRate/GM_CharactorSelection` (`GameplayStatics.GetGameMode`)))
    (`/Game/Blueprint/CharacterSelection/FrameRate/GM_CharactorSelection.Set Decision Index` _asgm_charactor_selection)
    (`/Game/Blueprint/CharacterSelection/FrameRate/GM_CharactorSelection.Increment Widget Index` _asgm_charactor_selection)
    (`/Game/Blueprint/CharacterSelection/FrameRate/HUD_ChoaractorSelecsion.Set Focus Widget` _ashud_choaractor_selecsion)
    (`/Game/Blueprint/Player/BP_SelectWeaponCharacter.SetWeapon` (`self.SelectWeaponCharactor`))
    (bind _asgm_charactor_selection_2 (cast `/Game/Blueprint/CharacterSelection/FrameRate/GM_CharactorSelection` (`GameplayStatics.GetGameMode`)))
    (`/Game/Blueprint/CharacterSelection/FrameRate/GM_CharactorSelection.Set Decision Index` _asgm_charactor_selection_2)))

(event `EnhancedInput|/Game/Input/CharacterSelection/IA_Back`
  (params (ActionValue :type Boolean) (ElapsedSeconds :type "Float (double-precision)") (TriggeredSeconds :type "Float (double-precision)") (InputAction :type "InputAction Object Reference" :default "/Game/Input/CharacterSelection/IA_Back.IA_Back"))
  (:`Started`
    ;[1 1 1] ウィジェットインデックスを減らす
    (bind _ashud_choaractor_selecsion (cast `/Game/Blueprint/CharacterSelection/FrameRate/HUD_ChoaractorSelecsion` (`self.GetHUD`)))
    (`/Game/Blueprint/CharacterSelection/FrameRate/HUD_ChoaractorSelecsion.Set Visility Hidden` _ashud_choaractor_selecsion)
    (bind _asgm_charactor_selection (cast `/Game/Blueprint/CharacterSelection/FrameRate/GM_CharactorSelection` (`GameplayStatics.GetGameMode`)))
    (`/Game/Blueprint/CharacterSelection/FrameRate/GM_CharactorSelection.Decrement Widget Index` _asgm_charactor_selection)
    (`/Game/Blueprint/CharacterSelection/FrameRate/HUD_ChoaractorSelecsion.Set Focus Widget` _ashud_choaractor_selecsion)))

(fn `UserConstructionScript`)