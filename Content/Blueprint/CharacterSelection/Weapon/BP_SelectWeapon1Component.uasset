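; Weapon mesh component for the character selection feature, displaying a selectable weapon on the owning BP_SelectWeaponCharacter.
; On BeginPlay it attaches itself to the character mesh at socket Weapon4, keeping relative transforms.
; SwitchingWeapon swaps the static mesh from WeaponArray by index.
; SetWeaponSocket re-attaches it to the indexed WeaponSocket entry, snapping location, rotation and scale to the socket.
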(event `self.ReceiveBeginPlay`
  (bind _asbp_select_weapon_character (cast `/Game/Blueprint/Player/BP_SelectWeaponCharacter` (`self.GetOwner`)))
  (`self.K2_AttachToComponent` (`/Game/Blueprint/Player/BP_SelectWeaponCharacter.CharactorMesh` _asbp_select_weapon_character) "Weapon4" "KeepRelative" "KeepRelative" "KeepRelative"))

(fn `SetWeaponSocket`
  (params (Weapon_Index :type Integer))
  (bind _asbp_select_weapon_character (cast `/Game/Blueprint/Player/BP_SelectWeaponCharacter` (`self.GetOwner`)))
  (`self.K2_AttachToComponent` (`/Game/Blueprint/Player/BP_SelectWeaponCharacter.CharactorMesh` _asbp_select_weapon_character) (`|GetArrayItem` (`self.WeaponSocket`) Weapon_Index) "SnapToTarget" "SnapToTarget" "SnapToTarget"))

(fn `switchingWeapon`
  (params (WeaponNum :type Integer))
  (`self.SetStaticMesh` (`|GetArrayItem` (`self.WeaponArray`) WeaponNum)))