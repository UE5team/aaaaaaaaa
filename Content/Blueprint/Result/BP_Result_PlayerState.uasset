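; BP_Result_PlayerState is a player state Blueprint holding game-over logic for a crashed player, though that logic is currently inactive.
; A disconnected graph chain would check IsCrashed once, wait briefly, then call SetGameOver, which flags the first game-over widget.
; IsCrashed is commented as a player durability check but only casts the pawn to BP_Player and returns false, and Tick is empty.
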(event `self.ReceiveTick`
  (params (DeltaSeconds :type "Float (single-precision)")))

(fn `IsCrashed`
  (returns (crashed :type Boolean))
  ;[1 1 1] PlayerのDurableが０以下であるか
  (cast `/Game/Blueprint/Player/BP_Player` (`GameplayStatics.GetPlayerPawn` 0))
  (return false))

(fn `SetGameOver`
  (bind _foundwidgets (`WidgetBlueprintLibrary.GetAllWidgetsOfClass` "/Game/Blueprint/point/BP_UI_ganeover.BP_UI_ganeover_C"))
  (set `/Game/Blueprint/point/BP_UI_ganeover.IsGameOver` true (`|GetArrayItem` _foundwidgets)))

(fn `UserConstructionScript`)