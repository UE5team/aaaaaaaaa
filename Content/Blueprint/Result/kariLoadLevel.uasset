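; Level-loading actor in the Result folder that drives transitions through the "loadlevel" streaming level.
; On BeginPlay it caches BP_LevelManager, streams in "loadlevel", sends it a begin message for "Title" and records "result" as the current level.
; Tick polls the manager's load flag, then, guarded by a DoOnce, sends next and current level names to the loading level, updates the current name and clears the flag.
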(event `self.ReceiveBeginPlay`
  (bind _returnvalue (`GameplayStatics.GetActorOfClass` "/Game/Blueprint/Mode/BP_LevelManager.BP_LevelManager_C"))
  (set `self.LevelManager` _returnvalue)
  (`GameplayStatics.LoadStreamLevel` "loadlevel" true)
  (message `/Game/Blueprint/Maps/IF_Load.Loading_Begin` (`GameplayStatics.GetStreamingLevel` "loadlevel") "Title")
  (set `self.Current level` "result"))

(event `self.ReceiveTick`
  (params (DeltaSeconds :type "Float (single-precision)"))
  (if (`/Game/Blueprint/Mode/BP_LevelManager.GetLoadFlag` (`self.LevelManager`))
    (`/Engine/EditorBlueprintResources/StandardMacros.DoOnce` false :!label _label
      (:`Completed`
        (`GameplayStatics.LoadStreamLevel` "loadlevel" true)
        (message `/Game/Blueprint/Maps/IF_Load.Loading_Widget` (`GameplayStatics.GetStreamingLevel` "loadlevel") (`/Game/Blueprint/Mode/BP_LevelManager.GetNextLevel` (`self.LevelManager`)) (`KismetStringLibrary.Conv_StringToName` (`self.Current level`)))
        (set `self.Current level` (`KismetStringLibrary.Conv_NameToString` (`/Game/Blueprint/Mode/BP_LevelManager.GetNextLevel` (`self.LevelManager`))))
        (`/Game/Blueprint/Mode/BP_LevelManager.SetLoadFlag` (`self.LevelManager`) false)
        (goto _label :!via `Reset`)))))

(fn `UserConstructionScript`)