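; Player controller for the result screen, stepping through total points, result, ranking and next-destination selection widgets.
; WidgetNum tracks the current page for confirm and return input, with fades, visibility toggles and an on-screen keyboard on the result page.
; The selection page swaps Input Mapping Contexts and auto-repeats scrolling on held input.
; Decision clears the UI and loads the in-game level, character selection or Title through BP_LevelManager, optionally opening mode select.
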(event `self.ReceiveBeginPlay`
  (`self.EnableInput` (`GameplayStatics.GetPlayerController` 0)))

(event `EnhancedInput|/Game/Blueprint/UI/result/IA_ConfirmButton`
  (params (ActionValue :type Boolean) (ElapsedSeconds :type "Float (double-precision)") (TriggeredSeconds :type "Float (double-precision)") (InputAction :type "InputAction Object Reference" :default "/Game/Blueprint/UI/result/IA_ConfirmButton.IA_ConfirmButton"))
  (:`Completed`
    (if (`self.CanChangeUI`)
      (set `self.CanChangeUI` false)
      (switch `int` (`self.WidgetNum`)
        (:`0`
          (`self.PlayFade`)
          (`KismetSystemLibrary.Delay` 1.0)
          (bind _foundwidgets (`WidgetBlueprintLibrary.GetAllWidgetsOfClass` "/Game/Blueprint/UI/result/UI_Total_points.UI_Total_points_C"))
          (bind (_newparam _ui_result) (`/Game/Blueprint/UI/result/UI_Total_points.Total_point_next` (`|GetArrayItem` _foundwidgets) (`self.UI Result`)))
          (set `self.UI Result` _ui_result)
          (set `self.WidgetNum` _newparam)
          (set `self.CanChangeUI` true))
        (:`1`
          (`self.KeyBoard visibility`
            (:`true`
              _)
            (:`KeyBoardは有効でない`
              _))
          (bind _foundwidgets_2 (`WidgetBlueprintLibrary.GetAllWidgetsOfClass` "/Game/Blueprint/UI/result/UI_result.UI_result_C"))
          (bind (_newparam_2 _ranking _save_) (`/Game/Blueprint/UI/result/UI_result.result_next` (`|GetArrayItem` _foundwidgets_2)))
          (set `self.WidgetNum` _newparam_2)
          (`/Engine/EditorBlueprintResources/StandardMacros.IsValid` _ranking
            (:`Is Valid`
              (set `self.UI Ranking` _ranking)
              (set `self.Save Data` _save_))
            (:`Is Not Valid`
              _))
          (set `self.CanChangeUI` true))
        (:`2`
          (set `self.WidgetNum` 3)
          (`/Engine/EditorBlueprintResources/StandardMacros.IsValid` (`self.UI SelectScreen`)
            (:`Is Valid`
              (`Widget.SetVisibility` (`self.UI SelectScreen`) "Visible"))
            (:`Is Not Valid`
              (bind _returnvalue (`|CreateWidget` "/Game/Blueprint/UI/result/UI_SelectScreen.UI_SelectScreen_C"))
              (bind _output_get (set `self.UI SelectScreen` _returnvalue))
              (`UserWidget.AddToViewport` _output_get 0)))
          (`/Game/Blueprint/System/FL_MyLibrary.RemoveMappingContext` "/Game/Blueprint/UI/result/IMC_Result.IMC_Result")
          (`/Game/Blueprint/System/FL_MyLibrary.SetMappingContext` "/Game/Blueprint/UI/result/IMC_SelectScreen.IMC_SelectScreen")
          (`Widget.SetVisibility` (`self.UI Ranking`) "Hidden")
          (set `self.CanChangeUI` true))))))

(event `EnhancedInput|/Game/Blueprint/UI/result/IA_return`
  (params (ActionValue :type Boolean) (ElapsedSeconds :type "Float (double-precision)") (TriggeredSeconds :type "Float (double-precision)") (InputAction :type "InputAction Object Reference" :default "/Game/Blueprint/UI/result/IA_return.IA_return"))
  (:`Completed`
    (switch `int` (`self.WidgetNum`)
      (:`0`
        (set `self.WidgetNum` 0))
      (:`1`
        (set `self.WidgetNum` 0)
        (bind _keyboard (`self.Keyboard`)
          (:`then`
            _)
          (:`else`
            _))
        (`Widget.SetVisibility` (`self.UI Result`) "Hidden")
        (`Widget.SetVisibility` (`self.WBP Fade`) "Hidden")
        (`Widget.SetVisibility` _keyboard "Hidden"))
      (:`2`
        (set `self.WidgetNum` 1)
        (`Widget.SetVisibility` (`self.UI Ranking`) "Hidden")
        (`Widget.SetVisibility` (`self.UI Result`) "Visible")
        (`Widget.SetVisibility` (`self.WBP Fade`) "Visible"))
      (:`3`
        (set `self.WidgetNum` 2)
        (`/Game/Blueprint/System/FL_MyLibrary.RemoveMappingContext` "/Game/Blueprint/UI/result/IMC_SelectScreen.IMC_SelectScreen")
        (`/Game/Blueprint/System/FL_MyLibrary.SetMappingContext` "/Game/Blueprint/UI/result/IMC_Result.IMC_Result")
        (`Widget.SetVisibility` (`self.UI Ranking`) "Visible")
        (`Widget.SetVisibility` (`self.UI SelectScreen`) "Hidden")))))

(event `EnhancedInput|/Game/Blueprint/UI/result/IA_KeyBoard`
  (params (ActionValue :type Boolean) (ElapsedSeconds :type "Float (double-precision)") (TriggeredSeconds :type "Float (double-precision)") (InputAction :type "InputAction Object Reference" :default "/Game/Blueprint/UI/result/IA_KeyBoard.IA_KeyBoard"))
  (:`Completed`
    (if (== (`self.WidgetNum`) 1)
      (`/Engine/EditorBlueprintResources/StandardMacros.IsValid` (`self.Save Data`)
        (:`Is Not Valid`
          (bind _foundwidgets (`WidgetBlueprintLibrary.GetAllWidgetsOfClass` "/Game/Blueprint/UI/result/UI_result.UI_result_C"))
          (bind _keyboard (`/Game/Blueprint/UI/result/UI_result.KeyBorad` (`|GetArrayItem` _foundwidgets)))
          (set `self.Keyboard` _keyboard))))))

(event `PlayFade`
  (bind _wbp_fade (`self.WBP Fade`))
  (`/Engine/EditorBlueprintResources/StandardMacros.IsValid` (`self.WBP Fade`)
    (:`Is Valid`
      (`Widget.SetVisibility` (`self.WBP Fade`) "Visible"))
    (:`Is Not Valid`
      (bind _returnvalue (`|CreateWidget` "/Game/Blueprint/Title/WBP_Fade.WBP_Fade_C"))
      (bind _output_get (set `self.WBP Fade` _returnvalue))
      (`UserWidget.AddToViewport` _output_get 0)))
  (`|PlayAnimation` _wbp_fade (`/Game/Blueprint/Title/WBP_Fade.LightFade` _wbp_fade)))

(event `EnhancedInput|/Game/Blueprint/UI/result/IA_SelectButton`
  (params (ActionValue :type "Float (double-precision)") (ElapsedSeconds :type "Float (double-precision)") (TriggeredSeconds :type "Float (double-precision)") (InputAction :type "InputAction Object Reference" :default "/Game/Blueprint/UI/result/IA_SelectButton.IA_SelectButton"))
  (bind _ui_selectscreen (`self.UI SelectScreen`))
  ;[1 1 1] IMC_SelectScreen
  (:`Triggered`
    (bind _result (`/Engine/EditorBlueprintResources/StandardMacros.IncrementInt` (`self.CountFrame`))
      (:`  `
        (set `self.ElapsedTime` (+ (`self.ElapsedTime`) (`GameplayStatics.GetWorldDeltaSeconds`)))
        (if (and (> (`self.ElapsedTime`) 0.7) (== (mod _result 4) 0))
          (`/Game/Blueprint/UI/result/UI_SelectScreen.ResetTexture` _ui_selectscreen :!label _label)
          (if (> ActionValue 0.0)
            (`/Game/Blueprint/UI/result/UI_SelectScreen.AddButtonNum` _ui_selectscreen)
            (else
              (`/Game/Blueprint/UI/result/UI_SelectScreen.SubtractButtonNum` _ui_selectscreen)))))))
  (:`Started`
    (set `self.ElapsedTime` 0.0)
    (set `self.CountFrame` 0)
    (goto _label)))

(event `EnhancedInput|/Game/Blueprint/UI/result/IA_Decision`
  (params (ActionValue :type Boolean) (ElapsedSeconds :type "Float (double-precision)") (TriggeredSeconds :type "Float (double-precision)") (InputAction :type "InputAction Object Reference" :default "/Game/Blueprint/UI/result/IA_Decision.IA_Decision"))
  ;[1 1 1] IMC_SelectScreen
  (:`Started`
    (`/Game/Blueprint/System/FL_MyLibrary.RemoveAllMappingContext`)
    (`WidgetLayoutLibrary.RemoveAllWidgets`)
    (switch `int` (`/Game/Blueprint/UI/result/UI_SelectScreen.PickButtonNum` (`self.UI SelectScreen`))
      (:`0`
        (bind _returnvalue (`GameplayStatics.GetActorOfClass` "/Game/Blueprint/System/BP_LevelManager.BP_LevelManager_C"))
        ;;[1 1 1] SetupLoadでレベル遷移
        (set `self.NextLevel` (`/Game/Blueprint/System/BP_LevelManager.GetInGameLevel` _returnvalue))
        (bind _returnvalue_2 (`GameplayStatics.GetActorOfClass` "/Game/Blueprint/System/BP_LevelManager.BP_LevelManager_C" :!label _label_2))
        (`/Game/Blueprint/System/BP_LevelManager.SetupLoad` _returnvalue_2 (`self.NextLevel`)))
      (:`1`
        (set `self.NextLevel` "Test_CharacterSelection")
        (goto _label_2))
      (:`2`
        (set `self.NextLevel` "Title")
        ;;;[1 1 1] モード選択画面を開くように設定
        (bind _returnvalue_3 (`GameplayStatics.GetActorOfClass` "/Game/Blueprint/System/BP_LevelManager.BP_LevelManager_C"))
        (`/Game/Blueprint/System/BP_LevelManager.SetDoSetModeScreen` _returnvalue_3 true)
        (`/Game/Blueprint/System/BP_LevelManager.SetupLoad` _returnvalue_3 (`self.NextLevel`)))
      (:`3`
        (set `self.NextLevel` "Title")
        (goto _label_2)))
    (bind _returnvalue_4 (`GameplayStatics.GetActorOfClass` "/Game/Blueprint/UI/result/ResultPawn.ResultPawn_C"))
    (`self.K2_DestroyActor` _returnvalue_4)))

(fn `UserConstructionScript`)