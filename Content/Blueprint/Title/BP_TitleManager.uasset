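; Title-screen manager that runs the title movie and switches between the title and mode-select widgets.
; BeginPlay picks the starting screen from a LevelManager flag, setting widgets and input mapping context.
; ChangeScreen swaps widgets and mapping contexts behind a fade played forward, then reversed.
; When the sound media player ends, it replays the title sequence or mode-select media, with timed input locks and a DoOnce-guarded title state change.
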(event `ReplayTitleAnimation`
  (bind _playback_speed (`self.Playback Speed`))
  (bind _wbp_title (`/Game/Blueprint/System/BP_WidgetCreater.Get WBP Title` (`/Game/Blueprint/System/FL_MyLibrary.getWidgetCreator`)))
  ;[1 1 1] タイトル開始時アニメーション
  (`/Game/Blueprint/Title/WBP_Title.ReplayAnimationFade` (`/Game/Blueprint/System/BP_WidgetCreater.Get WBP Title` (`/Game/Blueprint/System/FL_MyLibrary.getWidgetCreator`)) _playback_speed)
  (`KismetSystemLibrary.Delay` (/ 1.0 _playback_speed))
  ;;[1 1 1] アニメーションで使うものの初期化
  (`/Game/Blueprint/Title/WBP_Title.init` _wbp_title :!label _label)
  (bind _asbp_title_pc (`self.getTitlePC`))
  (set `/Game/Blueprint/Title/BP_Title_PC.IsInputInMovie` false _asbp_title_pc)
  (`self.ResetChangeStateEvent`)
  (`/Game/Blueprint/Title/WBP_Title.PlayMovieAndSound` _wbp_title)
  (`KismetSystemLibrary.Delay` (`self.Can\`tInputTime`))
  (set `self.is_play_sound` true)
  (`/Game/Blueprint/Title/BP_Title_PC.setCan\`tInput` _asbp_title_pc false)
  (`KismetSystemLibrary.K2_SetTimerDelegate` (delegate `changeState`) 10.0))

(event `self.ReceiveBeginPlay`
  (`self.Initialize variables`)
  (bind _asbp_title_pc (`self.getTitlePC`))
  (`/Game/Blueprint/Title/BP_Title_PC.setCan\`tInput` _asbp_title_pc true)
  (bind _level_manager (`/Game/Blueprint/System/FL_MyLibrary.getLevelManager`))
  (if (`/Game/Blueprint/System/BP_LevelManager.GetDoSetModeScreen` _level_manager)
    ;[1 1 1] モードセレクトスタート
    (set `self.CurrentDisplay` "ModeSelect")
    (bind _output_get (set `self.CurrentDisplayWidget` (`/Game/Blueprint/System/BP_WidgetCreater.getWBP GG ModeSelection` (`/Game/Blueprint/System/FL_MyLibrary.getWidgetCreator`))))
    (`UserWidget.AddToViewport` _output_get 0)
    (bind _output_get_2 (set `self.NextDisplayWidget` (`/Game/Blueprint/System/BP_WidgetCreater.Get WBP Title` (`/Game/Blueprint/System/FL_MyLibrary.getWidgetCreator`))))
    (`UserWidget.AddToViewport` _output_get_2 0)
    (`Widget.SetVisibility` _output_get_2 "Hidden")
    (set `self.CurrentMappingContext` "/Game/Input/Title/IMC_ModeSelect.IMC_ModeSelect")
    (`/Game/Blueprint/System/BP_LevelManager.SetDoSetModeScreen` _level_manager false)
    (set `self.NowAnimationWidget` (`/Game/Blueprint/System/BP_WidgetCreater.Get WBP Title` (`/Game/Blueprint/System/FL_MyLibrary.getWidgetCreator`)))
    (bind _returnvalue (`GameplayStatics.GetActorOfClass` "/Game/Blueprint/Title/BP_Title_PC.BP_Title_PC_C"))
    (`/Game/Blueprint/Title/BP_Title_PC.SetInputMappingContext` _returnvalue (`self.CurrentMappingContext`))
    ;[1 1 1] タイトルロゴを出す
    (`/Game/Blueprint/Title/WBP_Title.State1Setup` (`/Game/Blueprint/System/BP_WidgetCreater.Get WBP Title` (`/Game/Blueprint/System/FL_MyLibrary.getWidgetCreator`)))
    (bind _asbp_title_pc_2 (`self.getTitlePC`))
    (`/Game/Blueprint/Title/BP_Title_PC.setCan\`tInput` _asbp_title_pc_2 false)
    (else
      ;[1 1 1] タイトルスタート
      (set `self.CurrentDisplay` "Title")
      (bind _output_get_3 (set `self.CurrentDisplayWidget` (`/Game/Blueprint/System/BP_WidgetCreater.Get WBP Title` (`/Game/Blueprint/System/FL_MyLibrary.getWidgetCreator`))))
      (`UserWidget.AddToViewport` _output_get_3 0)
      (bind _output_get_4 (set `self.NextDisplayWidget` (`/Game/Blueprint/System/BP_WidgetCreater.getWBP GG ModeSelection` (`/Game/Blueprint/System/FL_MyLibrary.getWidgetCreator`))))
      (`UserWidget.AddToViewport` _output_get_4 0)
      (`Widget.SetVisibility` _output_get_4 "Hidden")
      (set `self.CurrentMappingContext` "/Game/Input/Title/IMC_Title.IMC_Title")
      (bind _returnvalue_2 (`GameplayStatics.GetActorOfClass` "/Game/Blueprint/Title/BP_Title_PC.BP_Title_PC_C"))
      (`/Game/Blueprint/Title/BP_Title_PC.SetInputMappingContext` _returnvalue_2 (`self.CurrentMappingContext`))
      (goto _label))))

(event `changeState`
  (bind _playback_speed (`self.Playback Speed`))
  (`/Engine/EditorBlueprintResources/StandardMacros.DoOnce` false :!label _label_2
    (:`Completed`
      (bind _asbp_title_pc (`self.getTitlePC`))
      (`/Game/Blueprint/Title/BP_Title_PC.setCan\`tInput` _asbp_title_pc true)
      (`/Game/Blueprint/Title/WBP_Title.changeState` (`/Game/Blueprint/System/BP_WidgetCreater.Get WBP Title` (`/Game/Blueprint/System/FL_MyLibrary.getWidgetCreator`)) _playback_speed (`self.FadeSpan`))
      (`KismetSystemLibrary.Delay` (/ 1.0 _playback_speed))
      (`/Game/Blueprint/Title/BP_Title_PC.setCan\`tInput` _asbp_title_pc false))))

(event `ResetChangeStateEvent`
  (goto _label_2 :!via `Reset`))

(event `ChangeScreen`
  (bind _currentmappingcontext (`self.CurrentMappingContext`))
  (bind _wbp_fade (`/Game/Blueprint/System/BP_WidgetCreater.getWBP Fade` (`/Game/Blueprint/System/FL_MyLibrary.getWidgetCreator`)))
  (set `self.IsEventChangeScreen` true)
  (`UserWidget.AddToViewport` _wbp_fade 5)
  ;[1 1 1] フェードアウト
  (`|PlayAnimation` _wbp_fade (`/Game/Blueprint/Title/WBP_Fade.Fade` _wbp_fade) 0.0 1 "Forward" (`self.FadeTime`)
    (:`Finished`
      (`Widget.SetVisibility` (`self.CurrentDisplayWidget`) "Hidden")
      ;[1 1 1] フェードイン後に表示されているウィジェットを表示
      (`Widget.SetVisibility` (`self.NextDisplayWidget`) "Visible")
      (`self.ExchangeDisplayWidget`)
      (bind _returnvalue (`GameplayStatics.GetActorOfClass` "/Game/Blueprint/Title/BP_Title_PC.BP_Title_PC_C"))
      (switch `name` (`self.CurrentDisplay`)
        (:`Title`
          (bind _setcurrentmappingcontext (`/Game/Blueprint/Title/BP_Title_PC.ChangeMappingContext` _returnvalue "/Game/Input/Title/IMC_ModeSelect.IMC_ModeSelect" _currentmappingcontext))
          (set `self.CurrentDisplay` "ModeSelect")
          (set `self.CurrentMappingContext` _setcurrentmappingcontext))
        (:`ModeSelect`
          (bind _setcurrentmappingcontext_2 (`/Game/Blueprint/Title/BP_Title_PC.ChangeMappingContext` _returnvalue "/Game/Input/Title/IMC_Title.IMC_Title" _currentmappingcontext))
          (set `self.CurrentDisplay` "Title")
          (set `self.CurrentMappingContext` _setcurrentmappingcontext_2)))
      ;[1 1 1] フェードイン
      (`|PlayAnimation` _wbp_fade (`/Game/Blueprint/Title/WBP_Fade.Fade` _wbp_fade) 0.0 1 "Reverse" (`self.FadeTime`)
        (:`Finished`
          (`Widget.RemoveFromParent` _wbp_fade)
          (set `self.IsEventChangeScreen` false))))))

(event `RemoveWidget`
  (`Widget.RemoveFromParent` (`self.CurrentDisplayWidget`))
  (`Widget.RemoveFromParent` (`self.NextDisplayWidget`)))

(event `MyStopAnimation`
  (params (UserWidget :type "UserWidget Object Reference") (WidgetAnimation :type "WidgetAnimation Object Reference"))
  (`UserWidget.StopAnimation` UserWidget WidgetAnimation))

(event `self.ReceiveTick`
  (params (DeltaSeconds :type "Float (single-precision)"))
  (add `MediaPlayer.OnEndReached` (`self.SoundMediaPlayer`) (delegate `replayMediaPlayer`)))

(event `replayMediaPlayer`
  (if (`self.is_play_sound`)
    (set `self.is_play_sound` false)
    (switch `name` (`self.CurrentDisplay`)
      (:`Title`
        (`self.ReplayTitleAnimation`))
      (:`ModeSelect`
        (`MediaPlayer.Play` (`self.SoundMediaPlayer`))
        (`MediaPlayer.Rewind` (`self.SoundMediaPlayer`))
        (set `self.is_play_sound` true)))))

(fn `ExchangeDisplayWidget`
  (locals (save :type "UserWidget Object Reference"))
  (set `local.save` (`self.CurrentDisplayWidget`))
  (set `self.CurrentDisplayWidget` (`self.NextDisplayWidget`))
  (set `self.NextDisplayWidget` (`local.save`)))

(fn `GetIsEventChangeScreen`
  (returns (value :type Boolean))
  (return (`self.IsEventChangeScreen`)))

(fn `getTitlePC`
  (returns (`AsBP Title PC` :type "/Game/Blueprint/Title/BP_Title_PC Object Reference"))
  (bind _returnvalue (`GameplayStatics.GetActorOfClass` "/Game/Blueprint/Title/BP_Title_PC.BP_Title_PC_C"))
  (return _returnvalue))

(fn `Initialize variables`
  (bind (`_st_titleparameters_フェードインアウトのアニメーション再生速度倍率例1_15倍1_05秒` `_st_titleparameters_ムービー終了_フェードイン後からフェードアウトまでの間の時間_秒_` `_st_titleparameters_ムービー中の入力が可能いなるまでの時間`) (break `/Game/PL/ST_TitleParameters` (make `/Game/PL/ST_TitleParameters`)))
  (`|ExecutionSequence`
    (:`then_0`
      (set `self.Playback Speed` `_st_titleparameters_フェードインアウトのアニメーション再生速度倍率例1_15倍1_05秒`))
    (:`then_1`
      (set `self.FadeSpan` `_st_titleparameters_ムービー終了_フェードイン後からフェードアウトまでの間の時間_秒_`))
    (:`then_2`
      (set `self.Can\`tInputTime` `_st_titleparameters_ムービー中の入力が可能いなるまでの時間`))))

(fn `UserConstructionScript`)