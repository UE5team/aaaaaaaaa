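; Title-screen player controller that handles Enhanced Input for the title and mode-select menus.
; Input actions skip title animations, change screens, quit or drive WBP_ModeSelect, gated by IsOperatingAuthority against screen changes, loading and CantInput.
; DoOnce nodes and CanEntry block repeated selection or confirmation until reset events fire.
; Helper functions add or swap mapping contexts, and debug number keys load levels through BP_LevelManager.
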(event `self.ReceiveBeginPlay`
  (bind _asgi_defolut (cast `/Game/Blueprint/Maps/GI_Defolut` (`GameplayStatics.GetGameInstance`)))
  (set `self.GI Default` _asgi_defolut)
  (`self.Reset`))

(event `self.ReceiveTick`
  (params (DeltaSeconds :type "Float (single-precision)"))
  (set `self.CoolTime` (+ DeltaSeconds (`self.CoolTime`))))

(event `EnhancedInput|/Game/Input/CharacterSelection/IA_Decide`
  (params (ActionValue :type Boolean) (ElapsedSeconds :type "Float (double-precision)") (TriggeredSeconds :type "Float (double-precision)") (InputAction :type "InputAction Object Reference" :default "/Game/Input/CharacterSelection/IA_Decide.IA_Decide"))
  ;[1 1 1] IMC_Titleのインプットアクション
  (:`Started`
    (bind _value (`self.IsOperatingAuthority`))
    (if _value
      (bind _foundwidgets (`WidgetBlueprintLibrary.GetAllWidgetsOfClass` "/Game/Blueprint/Title/WBP_TitleManager.WBP_TitleManager_C"))
      (bind _output (`|GetArrayItem` _foundwidgets))
      (if (`/Game/Blueprint/Title/WBP_TitleManager.IsTitleAnimation` _output)
        (bind _nowanimationwidget (`/Game/Blueprint/Title/WBP_TitleManager.NowAnimationWidget` _output))
        (`/Engine/EditorBlueprintResources/StandardMacros.IsValid` _nowanimationwidget
          (:`Is Valid`
            (set `/Game/Blueprint/Title/WBP_TitleManager.IsInputInAnimation` true _output)
            (`/Game/Blueprint/Title/WBP_TitleManager.MyStopAnimation` _output _nowanimationwidget (`/Game/Blueprint/Title/WBP_TitleManager.NowAnimation` _output))))
        (else
          (`/Game/Blueprint/Title/WBP_TitleManager.ChangeScreen` _output))))))

(event `EnhancedInput|/Game/Input/Title/IA_Quit`
  (params (ActionValue :type Boolean) (ElapsedSeconds :type "Float (double-precision)") (TriggeredSeconds :type "Float (double-precision)") (InputAction :type "InputAction Object Reference" :default "/Game/Input/Title/IA_Quit.IA_Quit"))
  ;[1 1 1] IMC_Titleのインプットアクション
  (:`Started`
    (bind _value (`self.IsOperatingAuthority`))
    (if _value
      (`KismetSystemLibrary.QuitGame` null "Quit"))))

(event `EnhancedInput|/Game/Input/Title/IA_ModeSelectDecision`
  (params (ActionValue :type Boolean) (ElapsedSeconds :type "Float (double-precision)") (TriggeredSeconds :type "Float (double-precision)") (InputAction :type "InputAction Object Reference" :default "/Game/Input/Title/IA_ModeSelectDecision.IA_ModeSelectDecision"))
  ;[1 1 1] IMC_ModeSelect
  (:`Started`
    (bind _value (`self.IsOperatingAuthority`))
    (if _value
      (`/Engine/EditorBlueprintResources/StandardMacros.DoOnce` false :!label _label
        (:`Completed`
          (bind _foundwidgets (`WidgetBlueprintLibrary.GetAllWidgetsOfClass` "/Game/Blueprint/Title/WBP_ModeSelect.WBP_ModeSelect_C"))
          (`/Game/Blueprint/Title/WBP_ModeSelect.ShiftMode` (`|GetArrayItem` _foundwidgets))
          (`self.DisableInput` (`GameplayStatics.GetPlayerController` 0)))))))

(event `Reset`
  ;[1 1 1] IMC_ModeSelect
  (goto _label :!via `Reset`))

(event `EnhancedInput|/Game/Input/Title/IA_ModeSelectReturn`
  (params (ActionValue :type Boolean) (ElapsedSeconds :type "Float (double-precision)") (TriggeredSeconds :type "Float (double-precision)") (InputAction :type "InputAction Object Reference" :default "/Game/Input/Title/IA_ModeSelectReturn.IA_ModeSelectReturn"))
  ;[1 1 1] IMC_ModeSelect
  (:`Started`
    (bind _value (`self.IsOperatingAuthority`))
    (if _value
      (bind _foundwidgets (`WidgetBlueprintLibrary.GetAllWidgetsOfClass` "/Game/Blueprint/Title/WBP_TitleManager.WBP_TitleManager_C"))
      (`/Game/Blueprint/Title/WBP_TitleManager.ChangeScreen` (`|GetArrayItem` _foundwidgets)))))

(event `EnhancedInput|/Game/Input/Title/IA_ModeSelectLeft`
  (params (ActionValue :type Boolean) (ElapsedSeconds :type "Float (double-precision)") (TriggeredSeconds :type "Float (double-precision)") (InputAction :type "InputAction Object Reference" :default "/Game/Input/Title/IA_ModeSelectLeft.IA_ModeSelectLeft"))
  ;[1 1 1] IMC_ModeSelect
  (:`Started`
    (bind _value (`self.IsOperatingAuthority`))
    (if _value
      (if (`self.CanEntry`)
        (set `self.CanEntry` false)
        (`/Engine/EditorBlueprintResources/StandardMacros.DoOnce` false :!label _label_2
          (:`Completed`
            (bind _foundwidgets (`WidgetBlueprintLibrary.GetAllWidgetsOfClass` "/Game/Blueprint/Title/WBP_ModeSelect.WBP_ModeSelect_C"))
            (`/Game/Blueprint/Title/WBP_ModeSelect.SelectionTargetToTheLeft` (`|GetArrayItem` _foundwidgets))))))))

(event `ResetLeftDoOnce`
  ;[1 1 1] IMC_ModeSelect
  (set `self.CanEntry` true)
  (goto _label_2 :!via `Reset`))

(event `EnhancedInput|/Game/Input/Title/IA_ModeSelectRight`
  (params (ActionValue :type Boolean) (ElapsedSeconds :type "Float (double-precision)") (TriggeredSeconds :type "Float (double-precision)") (InputAction :type "InputAction Object Reference" :default "/Game/Input/Title/IA_ModeSelectRight.IA_ModeSelectRight"))
  ;[1 1 1] IMC_ModeSelect
  (:`Started`
    (bind _value (`self.IsOperatingAuthority`))
    (if _value
      (if (`self.CanEntry`)
        (set `self.CanEntry` false)
        (`/Engine/EditorBlueprintResources/StandardMacros.DoOnce` false :!label _label_3
          (:`Completed`
            (bind _foundwidgets (`WidgetBlueprintLibrary.GetAllWidgetsOfClass` "/Game/Blueprint/Title/WBP_ModeSelect.WBP_ModeSelect_C"))
            (`/Game/Blueprint/Title/WBP_ModeSelect.SelectionTargetToTheRight` (`|GetArrayItem` _foundwidgets))))))))

(event `ResetRightDoOnce`
  ;[1 1 1] IMC_ModeSelect
  (set `self.CanEntry` true)
  (goto _label_3 :!via `Reset`))

(event `Key|One`
  (params (Key :type "Key Structure"))
  ;[1 1 1] デバッグ用
  (:`Pressed`
    (set `self.ChangeLevel` "Test_CharacterSelection")
    (`WidgetLayoutLibrary.RemoveAllWidgets` :!label _label_4)
    (`/Game/Blueprint/System/FL_MyLibrary.RemoveAllMappingContext`)
    (bind _returnvalue (`GameplayStatics.GetActorOfClass` "/Game/Blueprint/System/BP_LevelManager.BP_LevelManager_C"))
    (`/Game/Blueprint/System/BP_LevelManager.SetupLoad` _returnvalue (`self.ChangeLevel`))))

(event `Key|Two`
  (params (Key :type "Key Structure"))
  ;[1 1 1] デバッグ用
  (:`Pressed`
    (set `self.ChangeLevel` "test_Stage2")
    (goto _label_4)))

(event `Key|Three`
  (params (Key :type "Key Structure"))
  ;[1 1 1] デバッグ用
  (:`Pressed`
    (set `self.ChangeLevel` "result")
    (goto _label_4)))

(event `Key|Four`
  (params (Key :type "Key Structure"))
  ;[1 1 1] デバッグ用
  (:`Pressed`
    (set `self.ChangeLevel` "TimeAttack")
    (goto _label_4)))

(fn `ChangeMappingContext`
  (params (Add :type "InputMappingContext Object Reference") (CurrentMappingContext :type "InputMappingContext Object Reference"))
  (returns (SetCurrentMappingContext :type "InputMappingContext Object Reference"))
  (bind _returnvalue (pcsubsystem `EnhancedInputLocalPlayerSubsystem` (`GameplayStatics.GetPlayerController` 0)))
  (`EnhancedInputSubsystemInterface.RemoveMappingContext` _returnvalue CurrentMappingContext (struct))
  (`EnhancedInputSubsystemInterface.AddMappingContext` _returnvalue Add 0 (struct))
  (return Add))

(fn `IsOperatingAuthority`
  (returns (value :type Boolean))
  (bind _foundwidgets (`WidgetBlueprintLibrary.GetAllWidgetsOfClass` "/Game/Blueprint/Title/WBP_TitleManager.WBP_TitleManager_C"))
  (return (not (or (`/Game/Blueprint/Title/WBP_TitleManager.GetIsEventChangeScreen` (`|GetArrayItem` _foundwidgets)) (`/Game/Blueprint/Maps/GI_Defolut.GetLoadingNow` (`self.GI Default`)) (`self.Can'tInput`)))))

(fn `SetCanEntry`
  (params (value :type Boolean))
  (set `self.CanEntry` value))

(fn `SetInputMappingContext`
  (params (CurrentMappingContext :type "InputMappingContext Object Reference"))
  (bind _returnvalue (`GameplayStatics.GetPlayerController` 0))
  ;[1 1 1] コメント
  (`EnhancedInputSubsystemInterface.AddMappingContext` (pcsubsystem `EnhancedInputLocalPlayerSubsystem` _returnvalue) CurrentMappingContext 0 (struct))
  (`self.EnableInput` _returnvalue))

(fn `UserConstructionScript`)